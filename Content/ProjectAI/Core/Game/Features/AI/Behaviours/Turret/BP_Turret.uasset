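; AI turret that switches between alert and passive as targets enter and leave, and fires through a laser component.
; AI controller target events drive the state changes, with target loss also disabling the laser.
; Shoot starts the laser's cycle and is marked as a TODO to change.
; Helper functions smoothly rotate the pivot toward the target or back to relative zero, using shortest-path lerps scaled by delta time and look speed.
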(event `self.ReceiveBeginPlay`
  (`parent.ReceiveBeginPlay`)
  (`|ExecutionSequence`
    (:`then_0`
      (`self.Init`))
    (:`then_1`
      ;[1 0 0] Events
      (add `/Game/ProjectAI/Core/Game/Features/AI/Behaviours/Base/Behaviour/AC_EntityController_Base.OnTargetEnter` (`self.AIController`) (delegate `OnTargetEnter_Event`))
      (add `/Game/ProjectAI/Core/Game/Features/AI/Behaviours/Base/Behaviour/AC_EntityController_Base.OnTargetExit` (`self.AIController`) (delegate `OnTargetLost_Event`)))))

(event `Init`
  ;[1 0 0] Initialization
  (`/Game/ProjectAI/Core/Game/Features/Gameplay/WeaponSystem/Laser/Components/AC_Laser.Init` (`self.AC_Laser`) (`self.TurretMesh`)))

(event `OnTargetEnter_Event`
  (params (TargetEntity :type "/Game/ProjectAI/Core/Game/Features/Player/Base/BP_EntityBase Object Reference"))
  ;[1 0 0] Events
  (`self.ChangeToAlert`))

(event `OnTargetLost_Event`
  (params (TargetEntity :type "/Game/ProjectAI/Core/Game/Features/Player/Base/BP_EntityBase Object Reference"))
  ;[1 0 0] Events
  (`self.ChangeToPassive`)
  (`/Game/ProjectAI/Core/Game/Features/Gameplay/WeaponSystem/Laser/Components/AC_Laser.DisableLaser` (`self.AC_Laser`)))

(event `Shoot`
  ;[1 1 1] TODO: Change this
  (`/Game/ProjectAI/Core/Game/Features/Gameplay/WeaponSystem/Laser/Components/AC_Laser.StartCycle` (`self.AC_Laser`)))

(fn `LookAtTarget`
  (bind _targetactor (`self.GetTargetActor`))
  (`self.LerpRotate` (`KismetMathLibrary.FindLookAtRotation` (`SceneComponent.K2_GetComponentLocation` (`self.Pivot`)) (`self.K2_GetActorLocation` _targetactor))))

(fn `ResetLookRotation`
  (`self.LerpRotate` (struct) true))

(fn `UserConstructionScript`
  (`parent.UserConstructionScript`))