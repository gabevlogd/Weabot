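; Health manager component that handles damage, death, health regeneration and revival for its owner.
; TakeDamage uses a DoOnce gate as a hit cooldown, then starts a looping, delayed timer that regenerates health up to max.
; At zero health it marks death, waits, then regenerates; reaching max triggers BackToLife, which reopens the damage gate.
; Call functions broadcast each change, and helpers add, restore or query health and death state.
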(event `self.ReceiveBeginPlay`
  ;[0 0 0] Initialize
  (set `self.Health` (`self.MaxHealth`)))

(event `RegainHealth`
  ;[0 0 0] Regain Health Event
  (bind _output_get (set `self.Health` (+ (`self.Health`) (* (`self.RegainedHpPerSecond`) (`self.RegainHpEventTick`)))))
  (`self.OnRegainingHealth` _output_get)
  (if (>= (`self.Health`) (`self.MaxHealth`))
    (set `self.Health` (`self.MaxHealth`))
    (`self.StopHpRegaining`)
    (if (`self.IsDead`)
      (set `self.IsDead` false)
      (`self.BackToLife`))))

(event `Death`
  ;[0 0 0] Death Event
  (set `self.IsDead` true)
  (`self.OnDeath`)
  (`KismetSystemLibrary.Delay` (`self.RegainingHPAfterDeathDealy`))
  (`self.StartHpRegaining`))

(event `TakeDamage`
  (params (Damage :type "Float (double-precision)"))
  ;[0 0 0] Take Damage Event
  (`/Engine/EditorBlueprintResources/StandardMacros.DoOnce` false :!label _label
    (:`Completed`
      (bind _output_get (set `self.Health` (- (`self.Health`) Damage)))
      (`self.OnTakeDamage` _output_get Damage)
      (if (<= (`self.Health`) 0.0)
        (`self.StopHpRegaining`)
        (`self.Death`)
        (else
          (`self.StartHpRegaining`)
          (`KismetSystemLibrary.Delay` (`self.TakeDamageCooldown`))
          (goto _label :!via `Reset`))))))

(event `BackToLife`
  ;[0 0 0] Take Damage Event
  (`self.OnBackToLife`)
  (goto _label :!via `Reset`))

(fn `AddHealth`
  (params (GainedHealth :type "Float (double-precision)"))
  (bind _output_get (set `self.Health` (`KismetMathLibrary.FClamp` (+ GainedHealth (`self.Health`)) 0.0 (`self.MaxHealth`))))
  (`self.OnRegainingHealth` _output_get))

(fn `GetCurrentHealth`
  (returns (Health :type "Float (double-precision)"))
  (return (`self.Health`)))

(fn `GetDeathState`
  (returns (IsDead :type Boolean))
  (return (`self.IsDead`)))

(fn `GetMaxHealth`
  (returns (MaxHealth :type "Float (double-precision)"))
  (return (`self.MaxHealth`)))

(fn `ResetHpRegaining`
  (if (`KismetSystemLibrary.K2_IsTimerActiveHandle` (`self.RegainHpTimer`))
    (`self.StartHpRegaining`)))

(fn `RestoreHealth`
  (returns (Health :type "Float (double-precision)"))
  (set `self.IsDead` false)
  (bind _output_get (set `self.Health` (`self.MaxHealth`)))
  (`self.OnRegainingHealth` _output_get)
  (return _output_get))

(fn `StartHpRegaining`
  (bind _returnvalue (`KismetSystemLibrary.K2_SetTimerDelegate` (`|CreateDelegate` :!event `RegainHealth`) (`self.RegainHpEventTick`) true (`self.RegainHpCooldown`)))
  (set `self.RegainHpTimer` _returnvalue))

(fn `StopHpRegaining`
  (`KismetSystemLibrary.K2_PauseTimerHandle` (`self.RegainHpTimer`)))