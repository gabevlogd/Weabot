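; Base Blueprint for a grabbable physics object that can be placed in sockets as part of the activable socket system.
; Grab and Ungrab toggle whether it can be placed and notify via socketable events, while placing or removing it switches mesh physics simulation off or on.
; On release, it briefly cycles physics and collision to refresh overlaps, and a key comparison checks whether it matches a given socket.
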(event `/Game/ProjectAI/Core/Game/Features/Gameplay/HookSystem/Interfaces/BPI_Grabbable.Grab`
  (set `self.bCanBePlaced` false)
  (`self.OnSocketableGrabbed`))

(event `/Game/ProjectAI/Core/Game/Features/Gameplay/HookSystem/Interfaces/BPI_Grabbable.Ungrab`
  (set `self.bCanBePlaced` true)
  (`self.UpdateOverlap`)
  (`self.OnSocketableUngrabbed`))

(event `/Game/ProjectAI/Core/Game/Features/Gameplay/ActivableSocketSystem/Interfaces/BPI_Socketable.PlaceSocket`
  (`PrimitiveComponent.SetSimulatePhysics` (`self.Mesh`) false))

(event `/Game/ProjectAI/Core/Game/Features/Gameplay/ActivableSocketSystem/Interfaces/BPI_Socketable.RemoveSocket`
  (`PrimitiveComponent.SetSimulatePhysics` (`self.Mesh`) true))

(fn `CanBePlaced`
  (returns (bCanBePlaced :type Boolean))
  (return (`self.bCanBePlaced`)))

(fn `GetCanBeGrabbed`
  (returns (bCanBeGrabbed :type Boolean))
  (return true))

(fn `UpdateOverlap`
  (`PrimitiveComponent.SetSimulatePhysics` (`self.Mesh`) false)
  (`PrimitiveComponent.SetCollisionEnabled` (`self.Mesh`) "NoCollision")
  (`PrimitiveComponent.SetSimulatePhysics` (`self.Mesh`) true)
  (`PrimitiveComponent.SetCollisionEnabled` (`self.Mesh`) "QueryAndPhysics"))

(fn `UserConstructionScript`)