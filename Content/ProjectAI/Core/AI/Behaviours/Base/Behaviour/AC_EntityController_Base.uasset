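; Base AI controller that runs a supplied behaviour tree and tracks a perceived player as its target.
; AI perception sets the first sensed BPI_Player actor as target, clears it when that actor is lost, and fires found and lost calls.
; State and disabled setters write to the blackboard using key names looked up in DT_BBKeys.
; A helper looks up an actor's last stimulus for sight, hearing or damage.
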(event `Init`
  (params (Behaviour :type "BehaviorTree Object Reference"))
  (`self.RunBehaviour` Behaviour))

(event `self.AIPerception.OnTargetPerceptionUpdated`
  (params (Actor :type "Actor Object Reference") (Stimulus :type "AIStimulus Structure"))
  (cast `/Game/ProjectAI/Core/Characters/Interfaces/BPI_Player` Actor)
  (if Stimulus_bSuccessfullySensed
    (`self.TargetActor`
      (:`then`)
      (:`else`
        (`self.SetTarget` Actor)
        (`self.OnTargetFound` Actor)))
    (elif (== Actor (`self.TargetActor`))
      (`self.SetTarget` null)
      (`self.OnTargetLost` Actor))))

(fn `Can Sense Actor`
  (params (Actor :type "Actor Object Reference") (Interface :type "Interface Class Reference") (Sense :type "/Game/ProjectAI/Core/AI/_Debug/Utility/Enums/E_Sense Enum" :default "NewEnumerator0"))
  (returns (Stimulus :type "AIStimulus Structure") (bIsSensed :type Boolean))
  (bind _info (`AIPerceptionComponent.GetActorsPerception` (`self.AIPerception`) null))
  (for _array_element (`.LastSensedStimuli` (break `ActorPerceptionBlueprintInfo` _info))
    (bind _returnvalue (`AIPerceptionSystem.GetSenseClassForStimulus` _array_element))
    (if (== _returnvalue (select `/Game/ProjectAI/Core/AI/_Debug/Utility/Enums/E_Sense` Sense :`NewEnumerator1` "/Script/AIModule.AISense_Sight" :`NewEnumerator2` "/Script/AIModule.AISense_Hearing" :`NewEnumerator3` "/Script/AIModule.AISense_Damage" :!type "Object Class Reference"))
      (return _array_element (`.bSuccessfullySensed` (break `AIStimulus` _array_element))))))

(fn `GetState`
  (returns (CurrentState :type "/Game/ProjectAI/Core/AI/Data/Enums/E_EntityState Enum"))
  (return (`self.CurrentState`)))

(fn `IsState`
  (params (State :type "/Game/ProjectAI/Core/AI/Data/Enums/E_EntityState Enum" :default "NewEnumerator0"))
  (returns (bIsState :type Boolean))
  (return (`|EnumEquality` State (`self.CurrentState`))))

(fn `RunBehaviour`
  (params (Behaviour :type "BehaviorTree Object Reference"))
  (bind _returnvalue (`self.RunBehaviorTree` Behaviour))
  (if (not _returnvalue)
    (`self.PrintBehaviourError`)))

(fn `SetIsDisabled`
  (params (bIsDisabled :type Boolean))
  (bind _returnvalue (`|GetDataTableRow` "/Game/ProjectAI/Core/AI/Data/Tables/DT_BBKeys.DT_BBKeys" "IsDisabled")
    (:`then`
      (`BlackboardComponent.SetValueAsBool` (`self.Blackboard`) (break `/Game/ProjectAI/Core/AI/Data/Structs/S_BBKey` _returnvalue) bIsDisabled)
      (set `self.bIsDisabled` bIsDisabled))))

(fn `SetState`
  (params (State :type "/Game/ProjectAI/Core/AI/Data/Enums/E_EntityState Enum" :default "NewEnumerator0"))
  (bind _returnvalue (`|GetDataTableRow` "/Game/ProjectAI/Core/AI/Data/Tables/DT_BBKeys.DT_BBKeys" "State")
    (:`then`
      (bind _output_get (set `self.CurrentState` State))
      (`BlackboardComponent.SetValueAsEnum` (`self.Blackboard`) (break `/Game/ProjectAI/Core/AI/Data/Structs/S_BBKey` _returnvalue) _output_get))))

(fn `SetTarget`
  (params (TargetActor :type "Actor Object Reference"))
  (set `self.TargetActor` TargetActor))

(fn `UserConstructionScript`)