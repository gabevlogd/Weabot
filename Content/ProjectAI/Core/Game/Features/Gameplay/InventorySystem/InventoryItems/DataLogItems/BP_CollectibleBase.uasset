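; Base collectible actor for inventory data log items, providing a timed spawn animation and optional delayed destruction.
; BeginPlay starts the animation alongside empty sound and VFX hooks, using self-recursive next-tick delays and a shared elapsed-time counter instead of Timelines.
; Animation updates lerp the mesh's location, rotation and scale in world or relative space.
; Animation end can schedule destruction, whose sequence fires update and end dispatchers before destroying the actor.
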(event `self.ReceiveBeginPlay`
  (add `self.OnAnimationUpdate` (`|CreateDelegate` :!event `OnUpdateAnimation`))
  (add `self.OnAnimationEnded` (`|CreateDelegate` :!event `OnEndedAnimation`))
  (`self.OnPerformSpwanAnimation`)
  (`self.OnPerformSpawnSound`)
  (`self.OnPerformSpawnVFX`))

(event `OnPerformSpwanAnimation`
  (`self.SequenceCompleted` (`self.AnimSpeed`) (`self.AnimDuration`)
    (:`True`
      (`self.OnAnimationEnded`))
    (:`False`
      (`self.OnAnimationUpdate`)
      (`KismetSystemLibrary.DelayUntilNextTick`)
      (`self.OnPerformSpwanAnimation`))))

(event `OnPerformSpawnSound`)

(event `OnPerformSpawnVFX`)

(event `OnPerformDestruction`
  (`self.SequenceCompleted` (`self.DestructionSpeed`) (`self.DestructionDuration`)
    (:`True`
      (`self.OnDestructionEnded`)
      (`self.K2_DestroyActor`))
    (:`False`
      (`self.OnDestructionUpdate`)
      (`KismetSystemLibrary.DelayUntilNextTick`)
      (`self.OnPerformDestruction`))))

(fn `GetElapsedTime`
  (returns (ElapsedTime :type "Float (double-precision)"))
  (return (`self.ElapsedTime`)))

(fn `OnEndedAnimation`
  (if (`self.DestroyOnAnimationEnd`)
    (set `self.ElapsedTime` 0.0)
    (`KismetSystemLibrary.K2_SetTimerDelegate` (`|CreateDelegate` :!event `OnPerformDestruction`) (`self.DestructionDelay`))))

(fn `OnUpdateAnimation`
  (bind _returnvalue (`KismetMathLibrary.RLerp` (`self.Rotation A`) (`self.Rotation B`) (/ (`self.ElapsedTime`) (`self.AnimDuration`)) (`self.RotationShortest Path`)))
  (bind _returnvalue_2 (`KismetMathLibrary.VLerp` (`self.Scale A`) (`self.Scale B`) (/ (`self.ElapsedTime`) (`self.AnimDuration`))))
  (bind _returnvalue_3 (`KismetMathLibrary.VLerp` (`self.Location A`) (`self.Location B`) (/ (`self.ElapsedTime`) (`self.AnimDuration`))))
  (`|ExecutionSequence`
    (:`then_0`
      ;[1 0.7742 0] Location
      (if (`self.UseWorldLocation`)
        (`SceneComponent.K2_SetWorldLocation` (`self.StaticMesh`) _returnvalue_3 (`self.SweepLocation`) (`self.TeleportLocation`))
        (else
          (`SceneComponent.K2_SetRelativeLocation` (`self.StaticMesh`) _returnvalue_3 (`self.SweepLocation`) (`self.TeleportLocation`)))))
    (:`then_1`
      ;[0.2834 0.3136 1] Rotation
      (if (`self.UseWorldRotation`)
        (`SceneComponent.K2_SetWorldRotation` (`self.StaticMesh`) _returnvalue false false)
        (else
          (`SceneComponent.K2_SetRelativeRotation` (`self.StaticMesh`) _returnvalue false false))))
    (:`then_2`
      ;[0 1 0.1382] Scale
      (if (`self.UseWorldScale`)
        (`SceneComponent.SetWorldScale3D` (`self.StaticMesh`) _returnvalue_2)
        (else
          (`SceneComponent.SetRelativeScale3D` (`self.StaticMesh`) _returnvalue_2))))))

(fn `UserConstructionScript`)