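; Gameplay HUD that creates and manages the player's on-screen widgets: health bar, selected item, interaction prompt, pickup notifications, saving icon, popups and loading screen.
; Widgets react to inventory, data log, save manager, game event and player controller menu delegates.
; Pickups are queued and shown one at a time with a short delay, with data log items getting a separate collectible widget.
; Popups pause the game and block menus until closed.
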(event `self.ReceiveBeginPlay`
  (bind _asbp_gameplay_player_controller (cast `/Game/ProjectAI/Core/Game/UGameFramework/Controllers/BP_GameplayPlayerController` (`GameplayStatics.GetPlayerController` 0)))
  (set `self.PlayerController` _asbp_gameplay_player_controller)
  (bind _playerinventory (`/Game/ProjectAI/Core/Game/Utility/BFL_PAIComponentsUtility.TryGetPlayerInventory`))
  (set `self.PlayerInventory` _playerinventory)
  (bind _datalog (`/Game/ProjectAI/Core/Game/Utility/BFL_PAIComponentsUtility.TryGetPlayerDataLog`))
  (set `self.PlayerDataLog` _datalog)
  (`self.InitPlayerHUD`)
  (`self.InitSavingIcon`)
  (`self.InitInteractionWidget`)
  (`self.InitItemsList`)
  (`self.InitPopup`))

(event `OnPreGameModeInit`
  (`self.InitLoadingGraph`))

(event `InitInteractionWidget`
  (bind _returnvalue (`|SpawnActorFromClass` "/Game/ProjectAI/Core/Game/Features/Gameplay/InteractSystem/BP_InteractionOverlay.BP_InteractionOverlay_C" (`KismetMathLibrary.MakeTransform` (0.0 0.0 0.0)) "AlwaysSpawn" "MultiplyWithRoot" null null))
  (bind _output_get (set `self.InteractionOverlay` _returnvalue))
  (`/Game/ProjectAI/Core/Game/Features/Gameplay/InteractSystem/BP_InteractionOverlay.Disable` _output_get))

(event `ShowInteraction`
  (params (WorldPosition :type "Vector Structure") (InteractionText :type Text) (InputAction :type "InputAction Object Reference"))
  (`self.K2_SetActorLocation` (`self.InteractionOverlay`) WorldPosition false false)
  (`/Game/ProjectAI/Core/Game/Features/Gameplay/InteractSystem/BP_InteractionOverlay.SetTextAndGlyph` (`self.InteractionOverlay`) InputAction InteractionText)
  (`/Game/ProjectAI/Core/Game/Features/Gameplay/InteractSystem/BP_InteractionOverlay.Enable` (`self.InteractionOverlay`)))

(event `HideInteraction`
  (if (not (`Actor.bHidden` (`self.InteractionOverlay`)))
    (`/Game/ProjectAI/Core/Game/Features/Gameplay/InteractSystem/BP_InteractionOverlay.Disable` (`self.InteractionOverlay`))))

(event `InitItemsList`
  (bind _returnvalue (`|CreateWidget` "/Game/ProjectAI/Core/Game/Features/Gameplay/ChestSystem/UI/WBP_NewItemsList.WBP_NewItemsList_C"))
  (bind _output_get (set `self.ItemsListWidget` _returnvalue))
  (`UserWidget.AddToViewport` _output_get 0)
  (add `InventorySystem.OnAnyItemAdded` (`self.PlayerInventory`) (delegate `OnItemAdded_Event`))
  (add `InventorySystem.OnAnyItemAdded` (`self.PlayerDataLog`) (delegate `OnItemAdded_Event`)))

(event `OnItemAdded_Event`
  (params (Item :type "ItemBase Object Reference"))
  (`self.QueueNewItem` (`ItemBase.GetItemData` Item)))

(event `QueueNewItem`
  (params (ItemData :type "ItemData Object Reference"))
  (`KismetArrayLibrary.Array_Add` (`self.NewItems`) ItemData)
  (`KismetSystemLibrary.DelayUntilNextTick`)
  (`/Engine/EditorBlueprintResources/StandardMacros.DoOnce` false :!label _label
    (:`Completed`
      (`self.ShowItems`))))

(event `ShowItems`
  (bind _output (`|GetArrayItem` (`self.NewItems`)))
  (bind (_drawas _tiling _mirroring _imagesize _margin _tintcolor _outlinesettings _resourceobject) (break `SlateBrush` (`ItemData.ItemIcon` _output)))
  (bind _returnvalue (`KismetTextLibrary.Conv_StringToText` (`ItemData.ItemName` _output)))
  (`/Engine/EditorBlueprintResources/StandardMacros.IsValid` _output
    (:`Is Valid`
      (cast `/Game/ProjectAI/Core/Game/Features/Gameplay/InventorySystem/InventoryItems/Base/BP_PAIDataLogItemData` _output
        (:`then`
          (bind _returnvalue_2 (`|CreateWidget` "/Game/ProjectAI/Core/Game/Features/Gameplay/ChestSystem/UI/WBP_NewCollectible.WBP_NewCollectible_C" null _resourceobject _returnvalue))
          (`UserWidget.AddToViewport` _returnvalue_2 0))
        (:`CastFailed`
          (bind _returnvalue_3 (`|CreateWidget` "/Game/ProjectAI/Core/Game/Features/Gameplay/ChestSystem/UI/WBP_NewItemSlot.WBP_NewItemSlot_C" null _resourceobject _returnvalue))
          (`/Game/ProjectAI/Core/Game/Features/Gameplay/ChestSystem/UI/WBP_NewItemsList.AddItem` (`self.ItemsListWidget`) _returnvalue_3)))
      (`GameplayStatics.PlaySound2D` (`self.ItemCollectedSound`) 1.0 1.0 0.0 null null))
    (:`Is Not Valid`
      _))
  (`KismetArrayLibrary.Array_Remove` (`self.NewItems`))
  (if (`KismetArrayLibrary.Array_IsNotEmpty` (`self.NewItems`))
    (`KismetSystemLibrary.Delay` 0.1)
    (`self.ShowItems`)
    (else
      (goto _label :!via `Reset`))))

(event `InitSavingIcon`
  (bind _returnvalue (`|GenericCreateObject` "/Game/ProjectAI/Core/Game/Features/UI/Widgets/Menus/LoadingScreens/WBP_IsSavingIcon.WBP_IsSavingIcon_C"))
  (set `self.IsSavingIconWidget` _returnvalue)
  (add `SaveManager.OnPrepareSave` (`SSUtility.GetSaveManager`) (`|CreateDelegate` :!event `OnPrepareSave_Event`))
  (add `SaveManager.OnSaveGame` (`SSUtility.GetSaveManager`) (`|CreateDelegate` :!event `OnSaveGame_Event`)))

(event `OnPrepareSave_Event`
  (params (SaveGameData :type "DefaultSaveGame Object Reference") (SlotInfoItem :type "SlotInfoItem Object Reference") (Instigator :type "Object Object Reference"))
  (`UserWidget.AddToViewport` (`self.IsSavingIconWidget`) 1))

(event `OnSaveGame_Event`
  (params (SlotName :type String) (UserIndex :type Integer) (bSuccess :type Boolean) (SaveGameData :type "DefaultSaveGame Object Reference") (Instigator :type "Object Object Reference"))
  (bind _returnvalue (`|GetDataTableRow` "/Game/ProjectAI/Core/Game/ProjectConfig/DT_ProjectConfigs.DT_ProjectConfigs" "IsSavingMinDuration")
    (:`then`
      (`KismetSystemLibrary.Delay` (`.FloatValue_6_D6B628494000F149351A3B8B736089B6` (break `/Game/ProjectAI/Core/Game/ProjectConfig/Structs/S_ConfigValue` _returnvalue)))
      (`Widget.RemoveFromParent` (`self.IsSavingIconWidget`)))))

(event `InitPopup`
  (bind _asgm_paigameplay (cast `/Game/ProjectAI/Core/Game/UGameFramework/GameModes/GM_PAIGameplay` (`GameplayStatics.GetGameMode`)))
  (bind _ac_gameevents (`/Game/ProjectAI/Core/Game/UGameFramework/GameModes/GM_PAIGameplay.AC_GameEvents` _asgm_paigameplay))
  (add `/Game/ProjectAI/Core/Game/Managers/Events/Components/AC_GameEvents.OnOpenPopup` _ac_gameevents (`|CreateDelegate` :!event `OnOpenPopup_Event`))
  (add `/Game/ProjectAI/Core/Game/Managers/Events/Components/AC_GameEvents.OnClosePopup` _ac_gameevents (`|CreateDelegate` :!event `OnClosePopup_Event`)))

(event `OnOpenPopup_Event`
  (params (PopupData :type "/Game/ProjectAI/Core/Game/Features/Gameplay/PopupSystem/Data/BP_PopupData Object Reference"))
  (bind _returnvalue (`|GenericCreateObject` "/Game/ProjectAI/Core/Game/Features/UI/Widgets/Systems/PopupSystem/WBP_PopupWidget.WBP_PopupWidget_C" PopupData))
  (bind _output_get (set `self.PopupWidget` _returnvalue))
  (`UserWidget.AddToViewport` _returnvalue 11)
  (`WidgetBlueprintLibrary.SetInputMode_GameAndUIEx` (`GameplayStatics.GetPlayerController` 0) _output_get "LockInFullscreen" true true)
  (set `PlayerController.bShowMouseCursor` true (`GameplayStatics.GetPlayerController` 0))
  (`GameplayStatics.SetGamePaused` true)
  (`/Game/ProjectAI/Core/Game/UGameFramework/Controllers/BP_GameplayPlayerController.SetCanOpenMenus` (`self.PlayerController`) false))

(event `OnClosePopup_Event`
  (set `PlayerController.bShowMouseCursor` false (`GameplayStatics.GetPlayerController` 0))
  (`GameplayStatics.SetGamePaused` false)
  (`WidgetBlueprintLibrary.SetInputMode_GameOnly` (`GameplayStatics.GetPlayerController` 0) true)
  (`/Game/ProjectAI/Core/Game/UGameFramework/Controllers/BP_GameplayPlayerController.SetCanOpenMenus` (`self.PlayerController`) true))

(event `CloseCurrentPopup`
  (bind _popupwidget (`self.PopupWidget`)
    (:`then`
      (`/Game/ProjectAI/Core/Game/Features/UI/Widgets/Systems/PopupSystem/WBP_PopupWidget.ClosePopup` _popupwidget))
    (:`else`)))

(event `InitLoadingGraph`
  (bind _returnvalue (`|GenericCreateObject` "/Game/ProjectAI/Core/Game/Features/UI/Widgets/Menus/LoadingScreens/WBP_LoadingScreen.WBP_LoadingScreen_C"))
  ;[1 0 0] Making sure is above everything
  (`UserWidget.AddToViewport` _returnvalue 100)
  (bind _output_get (set `self.LoadingScreenWidget` _returnvalue))
  (`Widget.SetVisibility` _output_get "Collapsed")
  (bind (_bsuccess _gameevents) (`/Game/ProjectAI/Core/Game/Managers/Events/Utility/BFL_GameEventsUtility.TryGetGameEvents`))
  (add `/Game/ProjectAI/Core/Game/Managers/Events/Components/AC_GameEvents.OnStartLoadingLevel` _gameevents (`|CreateDelegate` :!event `OnStartLoadingLevel_Event`))
  (add `/Game/ProjectAI/Core/Game/Managers/Events/Components/AC_GameEvents.OnCompletedLoadingLevel` _gameevents (`|CreateDelegate` :!event `OnCompletedLoadingLevel_Event`)))

(event `OnStartLoadingLevel_Event`
  (params (LevelName :type Name))
  (`Widget.SetVisibility` (`self.LoadingScreenWidget`) "Visible"))

(event `OnCompletedLoadingLevel_Event`
  (params (LevelName :type Name))
  (`Widget.SetVisibility` (`self.LoadingScreenWidget`) "Collapsed"))

(event `InitPlayerHUD`
  (add `/Game/ProjectAI/Core/Game/UGameFramework/Controllers/BP_GameplayPlayerController.OnOpenUIMenu` (`self.PlayerController`) (`|CreateDelegate` :!event `OnOpenUIMenu_Event`))
  (add `/Game/ProjectAI/Core/Game/UGameFramework/Controllers/BP_GameplayPlayerController.OnCloseUIMenu` (`self.PlayerController`) (`|CreateDelegate` :!event `OnCloseUIMenu_Event`))
  (`self.AddSelectedItemWidgetToViewport`)
  (`self.AddHealthBarWidgetToViewport`))

(event `OnOpenUIMenu_Event`
  (params (Menu :type "Widget Object Reference"))
  (`Widget.SetVisibility` (`self.HealthBarWidget`) "Collapsed")
  (`Widget.SetVisibility` (`self.SelectedItemWidget`) "Collapsed"))

(event `OnCloseUIMenu_Event`
  (params (Menu :type "Widget Object Reference"))
  (`Widget.SetVisibility` (`self.HealthBarWidget`) "Visible")
  (`Widget.SetVisibility` (`self.SelectedItemWidget`) "Visible"))

(fn `AddHealthBarWidgetToViewport`
  (bind _asbp_entity_catcher (cast `/Game/ProjectAI/Core/Game/Features/Player/CaptureSystem/BP_EntityCatcher` (`GameplayStatics.GetPlayerPawn` 0)))
  (bind _returnvalue (`|CreateWidget` "/Game/ProjectAI/Core/Game/Features/UI/Widgets/Systems/HealthBarSystem/WBP_HealthBar.WBP_HealthBar_C" null (`/Game/ProjectAI/Core/Game/Features/Gameplay/HealthSystem/Components/AC_HealthManager.GetMaxHealth` (`/Game/ProjectAI/Core/Game/Features/Player/Base/BP_EntityBase.AC_HealthManager` _asbp_entity_catcher))))
  (`UserWidget.AddToViewport` _returnvalue 0)
  (set `self.HealthBarWidget` _returnvalue))

(fn `AddSelectedItemWidgetToViewport`
  (bind _returnvalue (`|GenericCreateObject` "/Game/ProjectAI/Core/Game/Features/UI/Widgets/Systems/InventorySystem/WBP_SelectedItem.WBP_SelectedItem_C"))
  (`UserWidget.AddToViewport` _returnvalue 0)
  (set `self.SelectedItemWidget` _returnvalue))

(fn `UserConstructionScript`)