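; Base Blueprint for AI entities that switch between passive and alert states.
; On BeginPlay it casts its AI controller to AC_EntityController_Base, caches it and initializes it with its Behaviour.
; ChangeToAlert and ChangeToPassive set the controller's state only when it differs, then fire OnAlertState or OnPassiveState, which are empty hooks here.
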(event `self.ReceiveBeginPlay`
  (bind _asac_entity_controller_base (cast `/Game/ProjectAI/Core/AI/Controllers/AC_EntityController_Base` (`AIBlueprintHelperLibrary.GetAIController` self)))
  (bind _output_get (set `self.AIController` _asac_entity_controller_base))
  (`/Game/ProjectAI/Core/AI/Controllers/AC_EntityController_Base.Init` _output_get (`self.Behaviour`)))

(event `OnAlertState`)

(event `OnPassiveState`)

(fn `ChangeToAlert`
  (bind _bisstate (`/Game/ProjectAI/Core/AI/Controllers/AC_EntityController_Base.IsState` (`self.AIController`) "NewEnumerator1"))
  (if (not _bisstate)
    (`/Game/ProjectAI/Core/AI/Controllers/AC_EntityController_Base.SetState` (`self.AIController`) "NewEnumerator1")
    (`self.OnAlertState`)))

(fn `ChangeToPassive`
  (bind _bisstate (`/Game/ProjectAI/Core/AI/Controllers/AC_EntityController_Base.IsState` (`self.AIController`) "NewEnumerator0"))
  (if (not _bisstate)
    (`/Game/ProjectAI/Core/AI/Controllers/AC_EntityController_Base.SetState` (`self.AIController`) "NewEnumerator0")
    (`self.OnPassiveState`)))

(fn `UserConstructionScript`)