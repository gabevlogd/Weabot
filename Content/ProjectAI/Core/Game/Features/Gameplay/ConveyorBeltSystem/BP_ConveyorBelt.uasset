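; Conveyor belt that pushes overlapping actors, except ignored classes, along its forward vector every tick, either constantly or as a triggerable timed run.
; When triggerable, primary and secondary interacts raise and lower a counter, flipping direction at its threshold and mirroring elapsed time if mid-run.
; A dynamic material scrolls with the belt speed and matches mesh scale.
; BeginPlay re-enables collision a tick late before initializing the belt.
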(event `self.Collision.OnComponentBeginOverlap`
  (params (OverlappedComponent :type "PrimitiveComponent Object Reference") (OtherActor :type "Actor Object Reference") (OtherComp :type "PrimitiveComponent Object Reference") (OtherBodyIndex :type Integer) (bFromSweep :type Boolean) (SweepResult :type "HitResult Structure (by ref)"))
  ;[0 0 0] Actors detection
  (`self.TryAddDetectedActor` OtherActor))

(event `self.Collision.OnComponentEndOverlap`
  (params (OverlappedComponent :type "PrimitiveComponent Object Reference") (OtherActor :type "Actor Object Reference") (OtherComp :type "PrimitiveComponent Object Reference") (OtherBodyIndex :type Integer))
  ;[0 0 0] Actors detection
  (`KismetArrayLibrary.Array_RemoveItem` (`self.ActorsOnIt`) OtherActor))

(event `self.ReceiveBeginPlay`
  ;[0 0 0] Unreal Events
  (`PrimitiveComponent.SetCollisionEnabled` (`self.Collision`) "NoCollision")
  (`KismetSystemLibrary.DelayUntilNextTick`)
  (`PrimitiveComponent.SetCollisionEnabled` (`self.Collision`) "QueryAndPhysics")
  (`self.InitializeBelt`))

(event `self.ReceiveTick`
  (params (DeltaSeconds :type "Float (single-precision)"))
  ;[0 0 0] Unreal Events
  (`self.ActiveMovement`
    (:`true`
      (`self.PerformMovement`))))

(event `/Game/ProjectAI/Core/Game/Features/Gameplay/InteractSystem/Interfaces/BPI_Interactable.PrimaryInteract`
  ;[0 0 0] Belt Trigger
  (`self.IsTriggerable`
    (:`true`
      (bind _triggerbeltmovement (`self.IncrementTriggerCounter` 1 (`self.MaxTriggerCount`)))
      (if _triggerbeltmovement
        (`self.InitializeBeltMovement`)))))

(event `/Game/ProjectAI/Core/Game/Features/Gameplay/InteractSystem/Interfaces/BPI_Interactable.SecondaryInteract`
  ;[0 0 0] Belt Trigger
  (`self.IsTriggerable`
    (:`true`
      (bind _triggerbeltmovement (`self.IncrementTriggerCounter` -1 (- (`self.MaxTriggerCount`) 1)))
      (if _triggerbeltmovement
        (`self.InitializeBeltMovement`)))))

(fn `IncrementTriggerCounter`
  (params (CounterIncrement :type Integer) (TriggerValue :type Integer))
  (returns (TriggerBeltMovement :type Boolean))
  (bind _output_get (set `self.CurrentTriggerCount` (`KismetMathLibrary.Clamp` (+ (`self.CurrentTriggerCount`) CounterIncrement) 0 (`self.MaxTriggerCount`))))
  (return (== _output_get TriggerValue)))

(fn `InitializeBelt`
  (`self.UpdateMaterialTexSize`)
  (`self.IsTriggerable`
    (:`true`
      (if (`|EnumEquality` (`self.InitialState`) "NewEnumerator0")
        (set `self.ElapsedTime` 0.0)
        (set `self.Direction` "NewEnumerator0")
        (`self.SetMaterialSpeed` (`self.PositiveSpeed`))
        (else
          (set `self.ElapsedTime` (`self.Duration`))
          (set `self.Direction` "NewEnumerator1")
          (`self.SetMaterialSpeed` 0.0))))
    (:`false`
      (bind _output_get (set `self.CurrentSpeed` (`self.PositiveSpeed`)))
      (`self.SetMaterialSpeed` _output_get))))

(fn `InitializeBeltMovement`
  (`self.ResetTimer`)
  (if (`|EnumEquality` (`self.Direction`) "NewEnumerator0")
    (set `self.Direction` "NewEnumerator1")
    (`self.SetMaterialSpeed` (`self.NegativeSpeed`))
    (else
      (set `self.Direction` "NewEnumerator0")
      (`self.SetMaterialSpeed` (`self.PositiveSpeed`)))))

(fn `PerformMovement`
  (if (> (`KismetArrayLibrary.Array_Length` (`self.ActorsOnIt`)) 0)
    (for _array_element (`self.ActorsOnIt`)
      (`self.K2_AddActorWorldOffset` _array_element (* (`KismetMathLibrary.GetForwardVector` (`self.K2_GetActorRotation`)) (* (`self.CurrentSpeed`) (`GameplayStatics.GetWorldDeltaSeconds`))) false false))))

(fn `ResetTimer`
  (if (>= (`self.ElapsedTime`) (`self.Duration`))
    (set `self.ElapsedTime` 0.0)
    (else
      (set `self.ElapsedTime` (- (`self.Duration`) (`self.ElapsedTime`))))))

(fn `SetMaterialSpeed`
  (params (Speed :type "Float (double-precision)"))
  (`MaterialInstanceDynamic.SetScalarParameterValue` (`self.Material`) "Speed X" (* Speed 0.01)))

(fn `TryAddDetectedActor`
  (params (DetectedActor :type "Actor Object Reference"))
  (if (not (`KismetArrayLibrary.Array_Contains` (`self.ActorToIgnore`) (`GameplayStatics.GetObjectClass` DetectedActor)))
    (`KismetArrayLibrary.Array_Add` (`self.ActorsOnIt`) (`local.DetectedActor`))))

(fn `UpdateDirection`
  (if (`|EnumEquality` (`self.Direction`) "NewEnumerator0")
    (set `self.CurrentSpeed` (`self.PositiveSpeed`))
    (else
      (set `self.CurrentSpeed` (`self.NegativeSpeed`)))))

(fn `UpdateMaterialTexSize`
  (bind (_returnvalue_x _returnvalue_y) (`KismetMathLibrary.BreakVector` (`SceneComponent.K2_GetComponentScale` (`self.StaticMesh`))))
  (`MaterialInstanceDynamic.SetScalarParameterValue` (`self.Material`) "Texture Size X" _returnvalue_x)
  (`MaterialInstanceDynamic.SetScalarParameterValue` (`self.Material`) "Texture Size Y" _returnvalue_y))

(fn `UpdateTimer`
  (set `self.ElapsedTime` (+ (`self.ElapsedTime`) (`GameplayStatics.GetWorldDeltaSeconds`))))

(fn `UserConstructionScript`
  (`parent.UserConstructionScript`)
  (bind _returnvalue (`PrimitiveComponent.CreateDynamicMaterialInstance` (`self.StaticMesh`) 0 null "None"))
  (set `self.Material` _returnvalue))