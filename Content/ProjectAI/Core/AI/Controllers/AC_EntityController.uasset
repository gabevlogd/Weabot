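; AI controller for entities that starts a given behaviour tree through Init and prints an error if it fails to run.
; It keeps the entity's current state and disabled flag, mirroring both into the Blackboard, and offers getters to read or compare the state.
; Blackboard key names are looked up by row in the DT_BBKeys data table, so values are only written when the row is found.
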(event `Init`
  (params (Behaviour :type "BehaviorTree Object Reference"))
  (`self.RunBehaviour` Behaviour))

(event `self.ReceiveBeginPlay`)

(fn `GetState`
  (returns (CurrentState :type "/Game/ProjectAI/Core/AI/Data/E_EntityState Enum"))
  (return (`self.CurrentState`)))

(fn `IsState`
  (params (State :type "/Game/ProjectAI/Core/AI/Data/E_EntityState Enum" :default "NewEnumerator0"))
  (returns (bIsState :type Boolean))
  (return (`|EnumEquality` State (`self.CurrentState`))))

(fn `RunBehaviour`
  (params (Behaviour :type "BehaviorTree Object Reference"))
  (bind _returnvalue (`self.RunBehaviorTree` Behaviour))
  (if (not _returnvalue)
    (`self.PrintBehaviourError`)))

(fn `SetIsDisabled`
  (params (bIsDisabled :type Boolean))
  (bind _returnvalue (`|GetDataTableRow` "/Game/ProjectAI/Core/AI/Data/DT_BBKeys.DT_BBKeys" "IsDisabled")
    (:`then`
      (`BlackboardComponent.SetValueAsBool` (`self.Blackboard`) (break `/Game/ProjectAI/Core/AI/Data/S_BBKey` _returnvalue) bIsDisabled)
      (set `self.bIsDisabled` bIsDisabled))))

(fn `SetState`
  (params (State :type "/Game/ProjectAI/Core/AI/Data/E_EntityState Enum" :default "NewEnumerator0"))
  (bind _returnvalue (`|GetDataTableRow` "/Game/ProjectAI/Core/AI/Data/DT_BBKeys.DT_BBKeys" "State")
    (:`then`
      (bind _output_get (set `self.CurrentState` State))
      (`BlackboardComponent.SetValueAsEnum` (`self.Blackboard`) (break `/Game/ProjectAI/Core/AI/Data/S_BBKey` _returnvalue) _output_get))))

(fn `UserConstructionScript`)