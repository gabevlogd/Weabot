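; Possessable Android entity in the capture system that can lock onto an AndroidInteractable, enabling it until it leaves.
; Interact and Leave abilities alternate through DoOnce gates, driving tick-delayed lerps that align the actor, extend the IK arm and retract it.
; While interacting, it cannot walk or be grabbed; TransformSaver persists that state and loading restores the arm pose.
; Also handles a flashlight that changes the material's emissive intensity.
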(event `CheckInitialState`
  (bind _returnvalue_location (`KismetMathLibrary.BreakTransform` (`SceneComponent.GetSocketTransform` (`self.Mesh`) "Hand" "RTS_World")))
  (if (`self.IsInteracting`)
    (set `self.Start Closed` true)
    (`CharacterMovementComponent.DisableMovement` (`self.CharacterMovement`))
    ;[0 0 0] Set animation pose parameters
    (`self.K2_SetActorTransform` (`self.GetTransform`))
    (`KismetSystemLibrary.DelayUntilNextTick`)
    (set `self.StartArmLocation` _returnvalue_location)
    (`SceneComponent.K2_SetWorldLocation` (`self.Arm_IK`) (`SceneComponent.K2_GetComponentLocation` (`/Game/ProjectAI/Core/Props/Interactables/BP_AndroidInteractable.InteractionPoint` (`self.AndroidInteractable`))) false false)
    (set `self.CanMoveArm` true)
    (`/Game/ProjectAI/Core/Props/Interactables/BP_AndroidInteractable.Enable` (`self.AndroidInteractable`))))

(event `self.ReceiveBeginPlay`
  (`/Game/ProjectAI/Core/Game/Features/Gameplay/FlashlightSystem/SC_Flashlight.Init` (`self.SC_Flashlight`) (`self.LookPoint`))
  (`parent.ReceiveBeginPlay`)
  (`self.Load`))

(event `self.PossessionStarted`
  (params (PreviousEntity :type "/Game/ProjectAI/Core/Game/Features/Player/Base/BP_EntityBase Object Reference"))
  ;[0 0 0] Custom Events Override
  (`parent.PossessionStarted` PreviousEntity)
  (if (`self.IsInteracting`)
    (`CharacterMovementComponent.DisableMovement` (`self.CharacterMovement`))
    (`self.ShowHUDInteraction` "Leave" "/Game/ProjectAI/Core/Game/Inputs/Actions/IA_EntityAbility_1.IA_EntityAbility_1")))

(event `self.PossessionEndedVFX`
  ;[0 0 0] Custom Events Override
  (`/Game/ProjectAI/Core/Game/Features/Gameplay/FlashlightSystem/SC_Flashlight.DeactivateFlashlight` (`self.SC_Flashlight`))
  (`parent.PossessionEndedVFX`))

(event `EnhancedInput|/Game/ProjectAI/Core/Game/Inputs/Actions/IA_EntityAbility_0`
  (params (ActionValue :type Boolean) (ElapsedSeconds :type "Float (double-precision)") (TriggeredSeconds :type "Float (double-precision)") (InputAction :type "InputAction Object Reference" :default "/Game/ProjectAI/Core/Game/Inputs/Actions/IA_EntityAbility_0.IA_EntityAbility_0"))
  ;[0 0 0] Entity Abilities
  (:`Triggered`
    (`/Engine/EditorBlueprintResources/StandardMacros.IsValid` (`self.AndroidInteractable`)
      (:`Is Valid`
        (`/Engine/EditorBlueprintResources/StandardMacros.DoOnce` (`self.Start Closed`) :!label _label
          (:`Completed`
            (`CharacterMovementComponent.DisableMovement` (`self.CharacterMovement`))
            (`self.EnableInteractAnimA`)))))))

(event `ResetAbility_0`
  ;[0 0 0] Entity Abilities
  (set `self.IsInteracting` false)
  (`self.ShowHUDInteraction` "Interact" "/Game/ProjectAI/Core/Game/Inputs/Actions/IA_EntityAbility_0.IA_EntityAbility_0")
  (`CharacterMovementComponent.SetMovementMode` (`self.CharacterMovement`) "MOVE_Walking" 0)
  (goto _label :!via `Reset`))

(event `EnhancedInput|/Game/ProjectAI/Core/Game/Inputs/Actions/IA_EntityAbility_1`
  (params (ActionValue :type Boolean) (ElapsedSeconds :type "Float (double-precision)") (TriggeredSeconds :type "Float (double-precision)") (InputAction :type "InputAction Object Reference" :default "/Game/ProjectAI/Core/Game/Inputs/Actions/IA_EntityAbility_1.IA_EntityAbility_1"))
  ;[0 0 0] Entity Abilities
  (:`Triggered`
    (`/Engine/EditorBlueprintResources/StandardMacros.DoOnce` (not (`self.Start Closed`)) :!label _label_2
      (:`Completed`
        (`/Game/ProjectAI/Core/Props/Interactables/BP_AndroidInteractable.Disable` (`self.AndroidInteractable`))
        (`self.DisableInteractAnim`)))))

(event `ResetAbility_1`
  ;[0 0 0] Entity Abilities
  (set `self.IsInteracting` true)
  (`/Game/ProjectAI/Core/Props/Interactables/BP_AndroidInteractable.Enable` (`self.AndroidInteractable`))
  (`self.ShowHUDInteraction` "Leave" "/Game/ProjectAI/Core/Game/Inputs/Actions/IA_EntityAbility_1.IA_EntityAbility_1")
  (goto _label_2 :!via `Reset`))

(event `self.TransformSaver.OnPrepSave`
  (params (SaveGameData :type "DefaultSaveGame Object Reference") (SlotInfoItem :type "SlotInfoItem Object Reference") (Instigator :type "Object Object Reference"))
  ;[0 0 0] Saves
  (bind _asbp_paisave_game (cast `/Game/ProjectAI/Core/Game/Data/SaveSystemData/BP_PAISaveGame` SaveGameData))
  (`BlueprintMapLibrary.Map_Add` (`/Game/ProjectAI/Core/Game/Data/SaveSystemData/BP_PAISaveGame.AndroidInteraction` _asbp_paisave_game) (`Saver.GetUniqueSaveID` (`self.TransformSaver`)) (make `/Game/ProjectAI/Core/Game/Features/Player/Data/S_AndroidSaveData` (`self.IsInteracting`))))

(event `self.TransformSaver.OnLoadGameCompleted`
  (params (SlotName :type String) (UserIndex :type Integer) (SaveGameData :type "DefaultSaveGame Object Reference") (Instigator :type "Object Object Reference"))
  ;[0 0 0] Saves
  (`self.Load`))

(event `Load`
  ;[0 0 0] Saves
  (`|ExecutionSequence`
    (:`then_0`
      (bind _asbp_paisave_game (cast `/Game/ProjectAI/Core/Game/Data/SaveSystemData/BP_PAISaveGame` (`SSUtility.GetSaveGame`)))
      (set `self.IsInteracting` (break `/Game/ProjectAI/Core/Game/Features/Player/Data/S_AndroidSaveData` (`BlueprintMapLibrary.Map_Find` (`/Game/ProjectAI/Core/Game/Data/SaveSystemData/BP_PAISaveGame.AndroidInteraction` _asbp_paisave_game) (`Saver.GetUniqueSaveID` (`self.TransformSaver`))))))
    (:`then_1`
      (`self.CheckInitialState`))))

(event `EnhancedInput|/Game/ProjectAI/Core/Game/Inputs/Actions/IA_ToggleFlashlight`
  (params (ActionValue :type Boolean) (ElapsedSeconds :type "Float (double-precision)") (TriggeredSeconds :type "Float (double-precision)") (InputAction :type "InputAction Object Reference" :default "/Game/ProjectAI/Core/Game/Inputs/Actions/IA_ToggleFlashlight.IA_ToggleFlashlight"))
  (:`Triggered`
    (`/Game/ProjectAI/Core/Game/Features/Gameplay/FlashlightSystem/SC_Flashlight.ToggleFlashlight` (`self.SC_Flashlight`))))

(event `self.SC_Flashlight.OnFlashlightEnabled`
  ;[0 0 0] Flashlight Events
  (bind _maindynamicmaterial (`self.MainDynamicMaterial`)
    (:`then`
      (`MaterialInstanceDynamic.SetScalarParameterValue` _maindynamicmaterial "EmissiveIntensity" 5.0))
    (:`else`)))

(event `self.SC_Flashlight.OnFlashlightDisabled`
  ;[0 0 0] Flashlight Events
  (bind _maindynamicmaterial (`self.MainDynamicMaterial`)
    (:`then`
      (`MaterialInstanceDynamic.SetScalarParameterValue` _maindynamicmaterial "EmissiveIntensity" (`self.PowerOnEmissive`)))
    (:`else`)))

(event `EnableInteractAnimA`
  (bind _returnvalue (`self.GetTransform`))
  (bind (_returnvalue_location _returnvalue_rotation) (`KismetMathLibrary.BreakTransform` (`SceneComponent.GetSocketTransform` (`self.Mesh`) "Hand" "RTS_World")))
  (bind _returnvalue_2 (`SceneComponent.K2_GetComponentToWorld` (`/Game/ProjectAI/Core/Props/Interactables/BP_AndroidInteractable.TriggerHitBox` (`self.AndroidInteractable`))))
  ;[0 0 0] Allign actor before IK Arm animation
  (`self.AnimationCompleted` 0.5
    (:`true`
      (set `self.CanMoveArm` true)
      (bind _output_get (set `self.StartArmRotation` _returnvalue_rotation))
      (bind _output_get_2 (set `self.StartArmLocation` _returnvalue_location))
      (`SceneComponent.K2_SetWorldTransform` (`self.Arm_IK`) (`KismetMathLibrary.MakeTransform` _output_get_2 _output_get) false false)
      (set `self.AnimElapsedTime` 0.0)
      (`self.EnableInteractAnimB`))
    (:`false`
      (`self.K2_SetActorTransform` (`KismetMathLibrary.TLerp` (`KismetMathLibrary.MakeTransform` (`KismetMathLibrary.MakeVector` (.x (.location _returnvalue)) (.y (.location _returnvalue)) (.z (.location _returnvalue))) (.rotation _returnvalue)) (`KismetMathLibrary.MakeTransform` (`KismetMathLibrary.MakeVector` (.x (.location _returnvalue_2)) (.y (.location _returnvalue_2)) (.z (.location _returnvalue))) (.rotation _returnvalue_2)) (/ (`self.AnimElapsedTime`) (* (`self.AnimDuration`) 0.5))))
      (`KismetSystemLibrary.DelayUntilNextTick`)
      (`self.EnableInteractAnimA`))))

(event `EnableInteractAnimB`
  ;[0 0 0] IK Arm animation
  (`self.AnimationCompleted` 0.5
    (:`true`
      (set `self.AnimElapsedTime` 0.0)
      (`self.ResetAbility_1`))
    (:`false`
      (`SceneComponent.K2_SetWorldLocation` (`self.Arm_IK`) (`KismetMathLibrary.VLerp` (`self.StartArmLocation`) (`SceneComponent.K2_GetComponentLocation` (`/Game/ProjectAI/Core/Props/Interactables/BP_AndroidInteractable.InteractionPoint` (`self.AndroidInteractable`))) (/ (`self.AnimElapsedTime`) (* (`self.AnimDuration`) 0.5))) false false)
      (`KismetSystemLibrary.DelayUntilNextTick`)
      (`self.EnableInteractAnimB`))))

(event `DisableInteractAnim`
  ;[0 0 0] Reset Arm IK animation
  (`self.AnimationCompleted` 1.0
    (:`true`
      (set `self.CanMoveArm` false)
      (set `self.AnimElapsedTime` 0.0)
      (`self.ResetAbility_0`))
    (:`false`
      (`SceneComponent.K2_SetWorldLocation` (`self.Arm_IK`) (`KismetMathLibrary.VLerp` (`SceneComponent.K2_GetComponentLocation` (`/Game/ProjectAI/Core/Props/Interactables/BP_AndroidInteractable.InteractionPoint` (`self.AndroidInteractable`))) (`self.StartArmLocation`) (/ (`self.AnimElapsedTime`) (`self.AnimDuration`))) false false)
      (`KismetSystemLibrary.DelayUntilNextTick`)
      (`self.DisableInteractAnim`))))

(fn `GetCanBeGrabbed`
  (returns (bCanBeGrabbed :type Boolean))
  (return (and (not (`self.IsInteracting`)) (`self.bIsEntityGrabbable`))))

(fn `SetHealthBarSocket`
  (`parent.SetHealthBarSocket`)
  (`SceneComponent.K2_AttachToComponent` (`self.HealthBar`) (`self.HealthBarSocket`) "None" "SnapToTarget" "SnapToTarget" "SnapToTarget" true))

(fn `SetMergePoint`
  (`SceneComponent.K2_AttachToComponent` (`self.MergePoint`) (`self.Mesh`) (`self.MergePointSocket`) "SnapToTarget" "SnapToTarget" "KeepWorld" true))

(fn `ShowHUDInteraction`
  (params (InteractionText :type Text) (InputAction :type "InputAction Object Reference"))
  (`/Game/ProjectAI/Core/Game/UGameFramework/HUD/BP_PAIGameplayHUD.ShowInteraction` (`self.HUD`) (`SceneComponent.K2_GetComponentLocation` (`/Game/ProjectAI/Core/Props/Interactables/BP_AndroidInteractable.HUDInteractionPoint` (`self.AndroidInteractable`))) InteractionText InputAction))

(fn `UserConstructionScript`
  (`parent.UserConstructionScript`))