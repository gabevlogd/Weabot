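; Hook prop that grabs and releases actors on primary and secondary interact through its ACGrabber component.
; Each Tick it box-traces for grab targets and, while grabbing, positions the held actor below GrabPoint, offset by its bounds height.
; The held actor auto-releases when it strays from its desired location beyond DetachTolerance.
; Attach and detach events toggle the actor's gravity and its collision response on a custom channel, then notify listeners.
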(event `self.ReceiveTick`
  (params (DeltaSeconds :type "Float (single-precision)"))
  (`self.CheckGrab`
    (:`true`
      (`self.SetGrabbedActorLocation`)
      (`self.CheckDetachmentTolerance`))))

(event `OnAttach_Event`
  (`self.IgnoreGrabbedActorCollision` true)
  (`self.SetGrabbedActorGravity` false)
  (`self.OnAttach`))

(event `OnDetach_Event`
  (`self.IgnoreGrabbedActorCollision` false)
  (`self.SetGrabbedActorGravity` true)
  (`self.OnDetach`))

(event `/Game/ProjectAI/Core/Interactables/Interfaces/BPI_Interactable.PrimaryInteract`
  (`self.TryGrab`))

(event `/Game/ProjectAI/Core/Interactables/Interfaces/BPI_Interactable.SecondaryInteract`
  (`self.TryUngrab`))

(fn `CheckDetachmentTolerance`
  (bind (_grabbedactor _bisgrabbing _grabbedactordesiredlocation) (`/Game/ProjectAI/Core/Props/Hook/Components/AC_HookGrabber.GetGrabInfo` (`self.AC_Grabber`)))
  (if (!= (`self.K2_GetActorLocation` _grabbedactor) _grabbedactordesiredlocation :`ErrorTolerance` (`self.DetachTolerance`))
    (`self.TryUngrab`)))

(fn `SetGrabbedActorLocation`
  (bind _grabpoint (`self.GrabPoint`))
  (bind _grabbedactor (`/Game/ProjectAI/Core/Props/Hook/Components/AC_HookGrabber.GetGrabInfo` (`self.AC_Grabber`)))
  (`/Game/ProjectAI/Core/Props/Hook/Components/AC_HookGrabber.UpdateGrabbedActorLocation` (`self.AC_Grabber`) (+ (`SceneComponent.K2_GetComponentLocation` _grabpoint) (* (`SceneComponent.GetUpVector` _grabpoint) -1.0 (.z (`.BoxExtent` (`KismetSystemLibrary.GetComponentBounds` (`Actor.RootComponent` _grabbedactor)))) 2.0)) (`SceneComponent.K2_GetComponentRotation` (`self.GrabPoint`))))

(fn `TraceGrab`
  (`/Game/ProjectAI/Core/Props/Hook/Components/AC_HookGrabber.TraceGrab` (`self.AC_Grabber`) (`self.DefaultSceneRoot`) (`KismetMathLibrary.Conv_DoubleToVector` (/ (`self.BoxTraceSize`) 2.0)) (`self.K2_GetActorRotation`)))

(fn `TryGrab`
  (returns (bHasGrabbed :type Boolean))
  (bind _bhasgrabbed (`/Game/ProjectAI/Core/Props/Hook/Components/AC_HookGrabber.Grab` (`self.AC_Grabber`)))
  (if _bhasgrabbed
    (`self.OnAttach_Event`))
  (return _bhasgrabbed))

(fn `TryUngrab`
  (returns (bHasUngrabbed :type Boolean))
  (bind _bhasungrabbed (`/Game/ProjectAI/Core/Props/Hook/Components/AC_HookGrabber.Ungrab` (`self.AC_Grabber`)))
  (`self.OnDetach_Event`)
  (return _bhasungrabbed))

(fn `UserConstructionScript`
  (`parent.UserConstructionScript`))