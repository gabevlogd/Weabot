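; BP_MovingObjectsTrigger is a world trigger that switches a set of moving objects on and off.
; Its EnterTrigger event calls Activate on every entry in the MovingObjects array, and ExitTrigger calls Deactivate on each of them.
; The construction script only calls the parent version.
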(event `self.EnterTrigger`
  (params (OtherActor :type "Actor Object Reference"))
  (`self.TriggerOnMovingObjects`))

(event `self.ExitTrigger`
  (params (OtherActor :type "Actor Object Reference"))
  (`self.TriggerOffMovingObjects`))

(fn `TriggerOffMovingObjects`
  (for _array_element (`self.MovingObjects`)
    (`/Game/ProjectAI/Core/Game/Features/Gameplay/InteractSystem/Interfaces/BPI_Activable.Deactivate` _array_element)))

(fn `TriggerOnMovingObjects`
  (for _array_element (`self.MovingObjects`)
    (`/Game/ProjectAI/Core/Game/Features/Gameplay/InteractSystem/Interfaces/BPI_Activable.Activate` _array_element)))

(fn `UserConstructionScript`
  (`parent.UserConstructionScript`))