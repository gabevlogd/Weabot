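; Base player controller that sets up mappable Enhanced Input and tracks whether the player uses gamepad or keyboard and mouse.
; On BeginPlay it initializes ACEnhancedMappableKeysHandler and registers its mapping contexts.
; AnyKey presses and Mouse2D movement beyond a deadzone update the current key, broadcasting its glyph when it differs from the last.
; Comparing both keys detects switches between device families, which fire general and device-specific change events.
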(event `self.ReceiveBeginPlay`
  (`/Game/ProjectAI/Core/Game/Features/Inputs/MappableKeys/Components/AC_EnhancedMappableKeysHandler.Init` (`self.AC_EnhancedMappableKeysHandler`) (subsystem `EnhancedInputLocalPlayerSubsystem`))
  (`/Game/ProjectAI/Core/Game/Features/Inputs/MappableKeys/Components/AC_EnhancedMappableKeysHandler.RegisterMappableInputMappingContexts` (`self.AC_EnhancedMappableKeysHandler`) (`self.InputMappingContexts`)))

(event `InputVectorAxis|Mouse2D` :paused true
  (params (AxisValue :type "Vector Structure"))
  ;[1 0 0] Generic input events to determine the currently used input device.
  (if (!= AxisValue (0.0 0.0 0.0) :`ErrorTolerance` 0.2)
    (set `self.CurrentKey` "Mouse2D")
    (`self.IsSameInput` :!label _label
      (:`false`
        (if (`self.IsMouseKeyboardInput` (`self.CurrentKey`))
          (bind _glyph (`/Game/ProjectAI/Core/Game/Features/Inputs/InputKeyGlyphsSystem/Utility/BFL_InputGlyphUtility.GetInputKeyGlyph` (`self.CurrentKey`)))
          (`self.OnNewKeyboardMouseInput` _glyph)
          (set `self.bIsUsingGamepad` false)
          (else
            (bind _glyph_2 (`/Game/ProjectAI/Core/Game/Features/Inputs/InputKeyGlyphsSystem/Utility/BFL_InputGlyphUtility.GetInputKeyGlyph` (`self.CurrentKey`)))
            (`self.OnNewGamepadInput` _glyph_2)
            (set `self.bIsUsingGamepad` true)))
        (`self.HasChangedInput`
          (:`true`
            (`self.OnInputDeviceChanged` (`self.bIsUsingGamepad`))
            (if (`self.bIsUsingGamepad`)
              (`self.OnInputDeviceGamepad`)
              (else
                (`self.OnInputDeviceKeyboardMouse`))))
          (:`false`
            _))
        (set `self.LastKey` (`self.CurrentKey`))))))

(event `Key|AnyKey` :paused true
  (params (Key :type "Key Structure"))
  ;[1 0 0] Generic input events to determine the currently used input device.
  (:`Pressed`
    (set `self.CurrentKey` Key)
    (goto _label)))

(fn `UserConstructionScript`)