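; Activable siren light prop that glows brighter or dimmer when activated or deactivated.
; The construction script creates dynamic material instances for two mesh slots, tints both with a configurable color, and sets the starting glow from IsActiveOnBegin.
; Activate and Deactivate switch only the first material's EmissiveIntensity between configurable active and inactive values, so the change is purely a material effect.
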(event `/Game/ProjectAI/Core/Game/Features/Gameplay/InteractSystem/Interfaces/BPI_Activable.Activate`
  (`MaterialInstanceDynamic.SetScalarParameterValue` (`self.DynamicMaterial_0`) "EmissiveIntensity" (`self.ActiveIntensity`)))

(event `/Game/ProjectAI/Core/Game/Features/Gameplay/InteractSystem/Interfaces/BPI_Activable.Deactivate`
  (`MaterialInstanceDynamic.SetScalarParameterValue` (`self.DynamicMaterial_0`) "EmissiveIntensity" (`self.DactiveIntesity`)))

(fn `UserConstructionScript`
  (`parent.UserConstructionScript`)
  (bind _returnvalue (`PrimitiveComponent.CreateDynamicMaterialInstance` (`self.StaticMesh`) 0 "/Game/ProjectAI/Art/3D/Materials/M_DoorAsset_01/M_DoorAsset_02_Inst1.M_DoorAsset_02_Inst1" "None"))
  (set `self.DynamicMaterial_0` _returnvalue)
  (bind _returnvalue_2 (`PrimitiveComponent.CreateDynamicMaterialInstance` (`self.StaticMesh`) 1 "/Game/ProjectAI/Art/3D/Materials/M_DoorAsset_01/M_DoorAsset_01_Inst1.M_DoorAsset_01_Inst1" "None"))
  (set `self.DynamicMaterial_1` _returnvalue_2)
  (`MaterialInstanceDynamic.SetVectorParameterValue` (`self.DynamicMaterial_0`) "EmissiveColor" (`self.Color`))
  (`MaterialInstanceDynamic.SetVectorParameterValue` (`self.DynamicMaterial_1`) "color" (`self.Color`))
  (`MaterialInstanceDynamic.SetVectorParameterValue` (`self.DynamicMaterial_1`) "EmissiveColor" (`self.Color`))
  (if (`self.bIsActiveOnBegin`)
    (`MaterialInstanceDynamic.SetScalarParameterValue` (`self.DynamicMaterial_0`) "EmissiveIntensity" (`self.ActiveIntensity`))
    (else
      (`MaterialInstanceDynamic.SetScalarParameterValue` (`self.DynamicMaterial_0`) "EmissiveIntensity" (`self.DactiveIntesity`)))))