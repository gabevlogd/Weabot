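; Actor component that lets its user detect, grab, carry and release actors implementing BPI_Grabbable.
; TraceGrab box-traces from a target origin while nothing is held, caching the hit actor if it reports it can be grabbed.
; Grab and Ungrab toggle the held state and notify the actor through the interface.
; UpdateGrabbedActorLocation moves the held actor with a sweep to an offset target and records that desired location for GetGrabInfo.
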(fn `GetGrabInfo`
  (returns (GrabbedActor :type "Actor Object Reference") (bIsGrabbing :type Boolean) (GrabbedActorDesiredLocation :type "Vector Structure"))
  (return (`self.GrabbedActor`) (`self.bIsGrabbing`) (`self.GrabbedActorDesiredLocation`)))

(fn `Grab`
  (returns (bHasGrabbed :type Boolean))
  (bind _grabbedactor (`self.GrabbedActor`))
  (bind _returnvalue (and (`self.bCanGrabActor`) (`KismetSystemLibrary.IsValid` _grabbedactor)))
  (if _returnvalue
    (set `self.bIsGrabbing` true)
    (bind _asbpi_grabbable (cast `/Game/ProjectAI/Core/Interactables/GrabSystem/Interfaces/BPI_Grabbable` _grabbedactor))
    (`/Game/ProjectAI/Core/Interactables/GrabSystem/Interfaces/BPI_Grabbable.Grab` _asbpi_grabbable)
    (return _returnvalue)))

(fn `TraceGrab`
  (params (TargetOrigin :type "SceneComponent Object Reference") (Direction :type "Vector Structure") (HalfSize :type "Vector Structure") (Orientation :type "Rotator Structure"))
  (locals (NewLocalVar :type "Actor Object Reference"))
  (if (not (`self.bIsGrabbing`))
    (bind _outhit (`KismetSystemLibrary.BoxTraceSingle` (+ (`SceneComponent.K2_GetComponentLocation` TargetOrigin) (`self.RayOffset`)) (+ (`SceneComponent.K2_GetComponentLocation` TargetOrigin) (* Direction (`self.TraceLength`))) HalfSize Orientation "TraceTypeQuery4" false (`Actor.GetAllChildActors` (`self.GetOwner` TargetOrigin) true) "ForOneFrame"))
    (if (and (`GameplayStatics.BreakHitResult` _outhit) (`KismetSystemLibrary.DoesImplementInterface` (`.HitActor` (`GameplayStatics.BreakHitResult` _outhit)) "/Game/ProjectAI/Core/Interactables/GrabSystem/Interfaces/BPI_Grabbable.BPI_Grabbable_C"))
      (bind _asbpi_grabbable (cast `/Game/ProjectAI/Core/Interactables/GrabSystem/Interfaces/BPI_Grabbable` (`.HitActor` (`GameplayStatics.BreakHitResult` _outhit))))
      (bind _bcanbegrabbed (`/Game/ProjectAI/Core/Interactables/GrabSystem/Interfaces/BPI_Grabbable.GetCanBeGrabbed` _asbpi_grabbable))
      (if _bcanbegrabbed
        (set `self.GrabbedActor` (`.HitActor` (`GameplayStatics.BreakHitResult` _outhit)))
        (set `self.bCanGrabActor` true)
        (else
          (set `self.bCanGrabActor` false :!label _label)))
      (else
        (goto _label)))))

(fn `Ungrab`
  (if (`self.bIsGrabbing`)
    (set `self.bIsGrabbing` false)
    (bind _asbpi_grabbable (cast `/Game/ProjectAI/Core/Interactables/GrabSystem/Interfaces/BPI_Grabbable` (`self.GrabbedActor`)))
    (`/Game/ProjectAI/Core/Interactables/GrabSystem/Interfaces/BPI_Grabbable.Ungrab` _asbpi_grabbable)))

(fn `UpdateGrabbedActorLocation`
  (params (TargetLocation :type "Vector Structure"))
  (bind _returnvalue (+ TargetLocation (`self.GrabOffset`)))
  (if (and (`self.bIsGrabbing`) (`KismetSystemLibrary.IsValid` (`self.GrabbedActor`)))
    (`Actor.K2_SetActorLocation` (`self.GrabbedActor`) _returnvalue true false)
    (set `self.GrabbedActorDesiredLocation` _returnvalue)))