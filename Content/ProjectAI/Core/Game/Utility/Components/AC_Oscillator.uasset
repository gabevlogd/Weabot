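; AC_Oscillator is an actor component that bobs a target scene component up and down along its relative Z axis.
; Init stores the target, and each Tick adds a sine of the owner's time since creation, scaled by Frequency and Amplitude, to its current Z.
; The offset accumulates on the current position rather than a stored base, so the travel depends on frame rate.
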(event `Init`
  (params (SceneComponentTarget :type "SceneComponent Object Reference"))
  (set `self.Target` SceneComponentTarget))

(event `self.ReceiveTick`
  (params (DeltaSeconds :type "Float (single-precision)"))
  (`self.PerformOscillation` (`self.Target`)))

(fn `PerformOscillation`
  (params (SceneComponent :type "SceneComponent Object Reference"))
  (bind (_relativelocation_x _relativelocation_y _relativelocation_z) (`KismetMathLibrary.BreakVector` (`SceneComponent.RelativeLocation` SceneComponent)))
  (`SceneComponent.K2_SetRelativeLocation` SceneComponent (`KismetMathLibrary.MakeVector` _relativelocation_x _relativelocation_y (+ _relativelocation_z (* (`KismetMathLibrary.Sin` (* (`Actor.GetGameTimeSinceCreation` (`self.GetOwner` SceneComponent)) (`self.Frequency`))) (`self.Amplitude`)))) false false))