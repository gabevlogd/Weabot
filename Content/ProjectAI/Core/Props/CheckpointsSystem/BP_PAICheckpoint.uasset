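; Checkpoint prop that records a respawn point and saves the game when its trigger is entered.
; On entry it tries to set the checkpoint using the currently loaded level as key and its own transform, and runs a manual save only if that succeeds.
; During save preparation it stamps its icon on the slot info, but only for saves it instigated.
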(event `self.EnterTrigger`
  (params (OtherActor :type "Actor Object Reference"))
  (bind _returnvalue (`CSUtility.TrySetCheckpoint` (`/Game/ProjectAI/Core/Game/Utility/BFL_PAILevelsUtility.GetCurrentLevelLoaded`) (`self.GetTransform`)))
  (if _returnvalue
    (`SSUtility.ManualSave` self)))

(event `self.Saver.OnPrepSave`
  (params (SaveGameData :type "DefaultSaveGame Object Reference") (SlotInfoItem :type "SlotInfoItem Object Reference") (Instigator :type "Object Object Reference"))
  (if (== Instigator self)
    (bind _asbp_paislot_info_item (cast `/Game/ProjectAI/Core/Game/Data/SaveSystemData/BP_PAISlotInfoItem` SlotInfoItem))
    (set `/Game/ProjectAI/Core/Game/Data/SaveSystemData/BP_PAISlotInfoItem.SaveSlotIcon` (`self.Save Slot Icon`) _asbp_paislot_info_item)))

(fn `UserConstructionScript`)