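; BP_PhysicalHeal is a physical inventory item that heals the entity it hits.
; It extends the parent's hit event, casting the hit actor to BP_EntityBase and adding GainedHealth through that entity's health manager component.
; A successful hit draws a green debug sphere at the impact point, while other hits print a miss message; the item destroys itself either way.
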(event `self.HitActorEvent`
  (params (OtherActor :type "Actor Object Reference") (Hit :type "HitResult Structure"))
  (`parent.HitActorEvent` OtherActor Hit)
  (bind _asbp_entity_base (cast `/Game/ProjectAI/Core/Game/Features/Player/Base/BP_EntityBase` OtherActor)
    (:`then`
      (`/Game/ProjectAI/Core/Game/Features/Gameplay/HealthSystem/Components/AC_HealthManager.AddHealth` (`/Game/ProjectAI/Core/Game/Features/Player/Base/BP_EntityBase.AC_HealthManager` _asbp_entity_base) (`self.GainedHealth`))
      (`KismetSystemLibrary.DrawDebugSphere` (`.Location` (`GameplayStatics.BreakHitResult` Hit)) 500.0 12 (struct :`R` 0.04927 :`G` 1.0 :`A` 1.0) 3.0 3.0)
      (`self.K2_DestroyActor`))
    (:`CastFailed`
      (`KismetSystemLibrary.PrintString` "Missed Target")
      (`self.K2_DestroyActor`))))

(fn `UserConstructionScript`
  (`parent.UserConstructionScript`))