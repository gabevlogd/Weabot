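; Gameplay settings component that applies the player's saved look sensitivity and analog deadzones to input axes.
; It reads values from BP_GameplaySettingsSaveGame, scaling look input by gamepad or mouse sensitivity and world delta seconds.
; Gamepad look first passes through the right-stick deadzone, a tolerance check against zero that passes input unchanged or zeroes it, with a separate left-stick threshold available.
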(fn `ApplyAnalogDeadzone`
  (params (Axes :type "Vector2D Structure") (Analog :type "/Game/ProjectAI/Core/Game/Managers/GameSettings/GameplaySettings/Enums/E_Analog Enum" :default "NewEnumerator0"))
  (returns (ReturnValue :type "Vector2D Structure"))
  (bind _gameplaysettingssavegame (`self.GetGameplaySettingsSaveGame`))
  (if (!= Axes (0.0 0.0) :`ErrorTolerance` (select `/Game/ProjectAI/Core/Game/Managers/GameSettings/GameplaySettings/Enums/E_Analog` Analog :`NewEnumerator0` (`/Game/ProjectAI/Core/Game/Data/SaveSystemData/Settings/BP_GameplaySettingsSaveGame.LeftAnalogDeadzone` _gameplaysettingssavegame) :`NewEnumerator1` (`/Game/ProjectAI/Core/Game/Data/SaveSystemData/Settings/BP_GameplaySettingsSaveGame.RightAnalogDeadzone` _gameplaysettingssavegame) :!type "Float (single-precision)"))
    (return Axes)
    (else
      (return (0.0 0.0)))))

(fn `ApplyLookModifiers`
  (params (LookAxes :type "Vector2D Structure") (bIsGamepad :type Boolean))
  (returns (ReturnValue :type "Vector2D Structure"))
  (bind _returnvalue (`GameplayStatics.GetWorldDeltaSeconds`))
  (bind _gameplaysettingssavegame (`self.GetGameplaySettingsSaveGame`))
  (if bIsGamepad
    (bind _returnvalue_2 (`self.ApplyAnalogDeadzone` LookAxes "NewEnumerator1"))
    (return (* _returnvalue_2 (`/Game/ProjectAI/Core/Game/Data/SaveSystemData/Settings/BP_GameplaySettingsSaveGame.GamepadSens` _gameplaysettingssavegame) _returnvalue))
    (else
      (return (* LookAxes (`/Game/ProjectAI/Core/Game/Data/SaveSystemData/Settings/BP_GameplaySettingsSaveGame.MouseSens` _gameplaysettingssavegame) _returnvalue)))))

(fn `GetGameplaySettingsSaveGame`
  (returns (GameplaySettingsSaveGame :type "/Game/ProjectAI/Core/Game/Data/SaveSystemData/Settings/BP_GameplaySettingsSaveGame Object Reference"))
  (return (cast `/Game/ProjectAI/Core/Game/Data/SaveSystemData/Settings/BP_GameplaySettingsSaveGame` (`self.SettingsSaveGame`) :!pure true)))