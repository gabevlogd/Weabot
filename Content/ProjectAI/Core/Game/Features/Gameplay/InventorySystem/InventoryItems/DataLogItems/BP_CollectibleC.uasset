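; BP_CollectibleC is a data log collectible in the inventory system that animates its mesh during destruction.
; On BeginPlay it creates a dynamic material on the static mesh and binds to an inherited destruction update event.
; Each update spins the mesh in yaw, adds a sine-driven vertical bob offset, and ramps the material's Progress parameter over the destruction duration.
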(event `self.ReceiveBeginPlay`
  (`parent.ReceiveBeginPlay`)
  (add `self.OnDestructionUpdate` (`|CreateDelegate` :!event `OnDestructionUpdate_Event`))
  (bind _returnvalue (`PrimitiveComponent.CreateDynamicMaterialInstance` (`self.StaticMesh`) 0 null "None"))
  (set `self.DynamicMaterial` _returnvalue))

(event `OnDestructionUpdate_Event`
  (`SceneComponent.K2_AddLocalRotation` (`self.StaticMesh`) (* (`KismetMathLibrary.MakeRotator` 0.0 0.0 1.0) (* (`GameplayStatics.GetWorldDeltaSeconds`) (`self.AngularSpeed`))) false false)
  (`SceneComponent.K2_AddLocalOffset` (`self.StaticMesh`) (`KismetMathLibrary.MakeVector` 0.0 0.0 (* (`KismetMathLibrary.Sin` (* (`self.GetElapsedTime`) (`self.BobbingSpeed`))) (`self.BobbingAmplitude`))) false false)
  (`MaterialInstanceDynamic.SetScalarParameterValue` (`self.DynamicMaterial`) "Progress" (`KismetMathLibrary.Lerp` 0.0 0.7 (/ (`self.GetElapsedTime`) (`self.DestructionDuration`)))))

(fn `UserConstructionScript`
  (`parent.UserConstructionScript`))