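; Health bar Blueprint that shows a HealthManager's current health on a static mesh.
; Initialize creates a dynamic material instance, caches max health and binds to the manager's damage and health regain events.
; Updates map the health ratio to the material's U Pan offset and a green, yellow or red emissive color chosen by percentage thresholds.
; A separate function sets emissive intensity.
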(event `Initialize`
  (params (HealthManager :type "/Game/ProjectAI/Core/Game/Features/Gameplay/HealthSystem/Components/AC_HealthManager Object Reference"))
  (bind _staticmesh (`self.StaticMesh`))
  (`/Engine/EditorBlueprintResources/StandardMacros.IsValid` HealthManager
    (:`Is Valid`
      ;[0 0 0] Get Dynamic Material
      (bind _returnvalue (`PrimitiveComponent.CreateDynamicMaterialInstance` _staticmesh 0 (`PrimitiveComponent.GetMaterial` _staticmesh 0) "None"))
      (bind _output_get (set `self.HealthMaterial` _returnvalue))
      ;[0 0 0] Cache Data
      (bind _output_get_2 (set `self.HealthManager` HealthManager))
      (set `self.MaxHealth` (`/Game/ProjectAI/Core/Game/Features/Gameplay/HealthSystem/Components/AC_HealthManager.GetMaxHealth` _output_get_2))
      (add `/Game/ProjectAI/Core/Game/Features/Gameplay/HealthSystem/Components/AC_HealthManager.OnRegainingHealth` _output_get_2 (`|CreateDelegate` :!event `UpdateHealthBar`))
      (add `/Game/ProjectAI/Core/Game/Features/Gameplay/HealthSystem/Components/AC_HealthManager.OnTakeDamage` _output_get_2 (`|CreateDelegate` :!event `OnTakeDamage_Event`))
      (`self.UpdateHealthBar` (`self.MaxHealth`)))
    (:`Is Not Valid`
      (`KismetSystemLibrary.PrintString` "HealthBar Fail: HealthManager null"))))

(event `UpdateHealthBar`
  (params (Health :type "Float (double-precision)"))
  (bind _returnvalue (/ Health (`self.MaxHealth`)))
  (`MaterialInstanceDynamic.SetScalarParameterValue` (`self.HealthMaterial`) "U Pan" (+ 0.6 (* 0.3 (- 1.0 _returnvalue))))
  (`MaterialInstanceDynamic.SetVectorParameterValue` (`self.HealthMaterial`) "EmissiveColor" (`self.GetHealthBarColor` _returnvalue)))

(event `OnTakeDamage_Event`
  (params (Health :type "Float (double-precision)") (Damage :type "Float (double-precision)"))
  (`self.UpdateHealthBar` Health))

(fn `GetHealthBarColor`
  (params (HealthPercentage :type "Float (double-precision)"))
  (returns (NewParam :type "LinearColor Structure"))
  (`|ExecutionSequence`
    (:`then_0`
      (if (> HealthPercentage (`self.MediumPercentage`))
        (return (struct :`G` 1.0 :`A` 1.0))))
    (:`then_1`
      (if (> HealthPercentage (`self.LowPercentage`))
        (return (struct :`R` 1.0 :`G` 1.0 :`A` 1.0))))
    (:`then_2`
      (return (struct :`R` 1.0 :`A` 1.0)))))

(fn `SetMaterialEmissive`
  (params (Value :type "Float (single-precision)"))
  (`MaterialInstanceDynamic.SetScalarParameterValue` (`self.HealthMaterial`) "EmissiveIntensity" Value))

(fn `UserConstructionScript`)