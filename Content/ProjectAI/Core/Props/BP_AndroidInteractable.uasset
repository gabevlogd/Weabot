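; BP_AndroidInteractable is an interactable prop that makes itself available to any BP_WalkingEntity standing inside its trigger.
; Entering TriggerHitBox sets the entity's CanInteract flag and hands it a reference to the prop; leaving clears both.
; Enable and Disable events toggle IsActive and print debug text, but the overlap logic does not check that flag.
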(event `Enable`
  (set `self.IsActive` true)
  (`KismetSystemLibrary.PrintString` "Enable"))

(event `Disable`
  (set `self.IsActive` false)
  (`KismetSystemLibrary.PrintString` "Disable"))

(event `self.TriggerHitBox.OnComponentBeginOverlap`
  (params (OverlappedComponent :type "PrimitiveComponent Object Reference") (OtherActor :type "Actor Object Reference") (OtherComp :type "PrimitiveComponent Object Reference") (OtherBodyIndex :type Integer) (bFromSweep :type Boolean) (SweepResult :type "HitResult Structure (by ref)"))
  (bind _asbp_walking_entity (cast `/Game/ProjectAI/Core/Characters/Player/BranchEntitiesExamples/BP_WalkingEntity` OtherActor))
  (set `/Game/ProjectAI/Core/Characters/Player/BranchEntitiesExamples/BP_WalkingEntity.CanInteract` true _asbp_walking_entity)
  (set `/Game/ProjectAI/Core/Characters/Player/BranchEntitiesExamples/BP_WalkingEntity.AndroidInteractable` self _asbp_walking_entity))

(event `self.TriggerHitBox.OnComponentEndOverlap`
  (params (OverlappedComponent :type "PrimitiveComponent Object Reference") (OtherActor :type "Actor Object Reference") (OtherComp :type "PrimitiveComponent Object Reference") (OtherBodyIndex :type Integer))
  (bind _asbp_walking_entity (cast `/Game/ProjectAI/Core/Characters/Player/BranchEntitiesExamples/BP_WalkingEntity` OtherActor))
  (set `/Game/ProjectAI/Core/Characters/Player/BranchEntitiesExamples/BP_WalkingEntity.CanInteract` false _asbp_walking_entity)
  (set `/Game/ProjectAI/Core/Characters/Player/BranchEntitiesExamples/BP_WalkingEntity.AndroidInteractable` (`self.Null`) _asbp_walking_entity))

(fn `UserConstructionScript`)