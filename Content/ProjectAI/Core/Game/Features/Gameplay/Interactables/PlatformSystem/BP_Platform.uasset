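; BP_Platform is a moving platform that travels between PointA and PointB in response to Activate and Deactivate calls.
; A clamped trigger counter sends it to B upon reaching MaxTriggerCount and back to A upon dropping one below.
; Tick lerps it from its current location over a duration derived from distance and Speed.
; A collider fitted around the mesh pauses movement while actors of CanStopMovement classes overlap it.
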(event `self.ReceiveBeginPlay`
  ;[0 0 0] Unreal Events
  ;;[0.1059 0.1059 0.1059] Set start platform location
  (`self.K2_SetActorLocation` (`SceneComponent.K2_GetComponentLocation` (`self.PointA`)) false true)
  (`self.SetUpCollider`))

(event `self.ReceiveTick`
  (params (DeltaSeconds :type "Float (single-precision)"))
  ;[0 0 0] Unreal Events
  ;;[0.1059 0.1059 0.1059] Location Lerping
  (`self.LocationLerpCompleted`
    (:`false`
      (`self.PerformLocationLerp`))))

(event `/Game/ProjectAI/Core/Game/Features/Gameplay/InteractSystem/Interfaces/BPI_Activable.Activate`
  ;[0 0 0] Platform Trigger
  (bind _triggerplatformmovement (`self.IncrementTriggerCounter` 1 (`self.MaxTriggerCount`)))
  (if _triggerplatformmovement
    (`self.CalculateLerp Data` (`SceneComponent.K2_GetComponentLocation` (`self.PointB`)))))

(event `/Game/ProjectAI/Core/Game/Features/Gameplay/InteractSystem/Interfaces/BPI_Activable.Deactivate`
  ;[0 0 0] Platform Trigger
  (bind _triggerplatformmovement (`self.IncrementTriggerCounter` -1 (- (`self.MaxTriggerCount`) 1)))
  (if _triggerplatformmovement
    (`self.CalculateLerp Data` (`SceneComponent.K2_GetComponentLocation` (`self.PointA`)))))

(event `self.Collider.OnComponentBeginOverlap`
  (params (OverlappedComponent :type "PrimitiveComponent Object Reference") (OtherActor :type "Actor Object Reference") (OtherComp :type "PrimitiveComponent Object Reference") (OtherBodyIndex :type Integer) (bFromSweep :type Boolean) (SweepResult :type "HitResult Structure (by ref)"))
  ;[0 0 0] Block movement
  (`self.IsStoppingActor` OtherActor
    (:`true`
      (`KismetArrayLibrary.Array_Add` (`self.OverlappedActors`) OtherActor)
      (set `self.PauseMovement` true))))

(event `self.Collider.OnComponentEndOverlap`
  (params (OverlappedComponent :type "PrimitiveComponent Object Reference") (OtherActor :type "Actor Object Reference") (OtherComp :type "PrimitiveComponent Object Reference") (OtherBodyIndex :type Integer))
  ;[0 0 0] Block movement
  (`self.IsStoppingActor` OtherActor
    (:`true`
      (`KismetArrayLibrary.Array_RemoveItem` (`self.OverlappedActors`) OtherActor)
      (`self.UnpauseMovement`
        (:`true`
          (set `self.PauseMovement` false))))))

(fn `CalculateLerp Data`
  (params (EndLocation :type "Vector Structure"))
  ;[0 0 0] Set Locations
  (set `self.StartLocation` (`self.K2_GetActorLocation`))
  (set `self.EndLocation` EndLocation)
  ;[0 0 0] Reset Timer
  (set `self.ElapsedTime` 0.0)
  ;[0 0 0] Set Lerp Duration
  (set `self.LerpDuration` (/ (`KismetMathLibrary.Vector_Distance` (`self.StartLocation`) (`self.EndLocation`)) (`self.Speed`))))

(fn `IncrementTriggerCounter`
  (params (CounterIncrement :type Integer) (TriggerValue :type Integer))
  (returns (TriggerPlatformMovement :type Boolean))
  (bind _output_get (set `self.CurrentTriggerCount` (`KismetMathLibrary.Clamp` (+ (`self.CurrentTriggerCount`) CounterIncrement) 0 (`self.MaxTriggerCount`))))
  (return (== _output_get TriggerValue)))

(fn `PerformLocationLerp`
  ;[0 0 0] Setting New Location
  (`self.K2_SetActorLocation` (`KismetMathLibrary.VLerp` (`self.StartLocation`) (`self.EndLocation`) (/ (`self.ElapsedTime`) (`self.LerpDuration`))))
  (if (not (`self.PauseMovement`))
    ;[0 0 0] Update Elapsed Time
    (set `self.ElapsedTime` (+ (`self.ElapsedTime`) (`GameplayStatics.GetWorldDeltaSeconds`)))
    ;[0 0 0] Precisely set location after lerp completion
    (if (>= (`self.ElapsedTime`) (`self.LerpDuration`))
      (`self.K2_SetActorLocation` (`self.EndLocation`) false true))))

(fn `SetUpCollider`
  (bind (_origin _boxextent) (`KismetSystemLibrary.GetComponentBounds` (`self.StaticMesh`)))
  (`SceneComponent.K2_SetWorldLocation` (`self.Collider`) _origin false false)
  (`BoxComponent.SetBoxExtent` (`self.Collider`) (+ _boxextent 2.0) true))

(fn `UserConstructionScript`
  (`parent.UserConstructionScript`))