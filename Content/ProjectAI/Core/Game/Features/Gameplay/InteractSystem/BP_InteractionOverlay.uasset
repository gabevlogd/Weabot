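; BP_InteractionOverlay is an actor that displays an interaction prompt in the game through a WBP_Interaction widget held in its widget component.
; While ticking, it billboards toward the first player's camera by inverting camera pitch and offsetting yaw by 180 degrees.
; Enable and Disable toggle both visibility and ticking.
; SetText and SetInputAction feed the widget its text and input action, hiding the input image when no valid action is given.
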(event `self.ReceiveBeginPlay`
  (set `self.InteractionWidget` (cast `/Game/ProjectAI/Core/Game/Features/UI/Widgets/Systems/InteractSystem/WBP_Interaction` (`WidgetComponent.GetWidget` (`self.Widget`)) :!pure true)))

(event `self.ReceiveTick`
  (params (DeltaSeconds :type "Float (single-precision)"))
  (bind (_returnvalue_roll _returnvalue_pitch _returnvalue_yaw) (`KismetMathLibrary.BreakRotator` (`PlayerCameraManager.GetCameraRotation` (`PlayerController.PlayerCameraManager` (`GameplayStatics.GetPlayerController` 0)))))
  (`self.K2_SetActorRotation` (`KismetMathLibrary.MakeRotator` 0.0 (* _returnvalue_pitch -1.0) (+ _returnvalue_yaw 180.0))))

(event `Enable`
  (`self.SetActorHiddenInGame` false)
  (`self.SetActorTickEnabled` true))

(event `Disable`
  (`self.SetActorHiddenInGame` true)
  (`self.SetActorTickEnabled` false))

(fn `SetInputAction`
  (params (InputAction :type "InputAction Object Reference"))
  (`/Engine/EditorBlueprintResources/StandardMacros.IsValid` InputAction
    (:`Is Valid`
      (`/Game/ProjectAI/Core/Game/Features/UI/Widgets/Systems/InteractSystem/WBP_Interaction.SetInputAction` (`self.InteractionWidget`) InputAction)
      (`/Game/ProjectAI/Core/Game/Features/UI/Widgets/Systems/InteractSystem/WBP_Interaction.ShowInputImage` (`self.InteractionWidget`)))
    (:`Is Not Valid`
      (`/Game/ProjectAI/Core/Game/Features/UI/Widgets/Systems/InteractSystem/WBP_Interaction.HideInputImage` (`self.InteractionWidget`)))))

(fn `SetText`
  (params (InteractionText :type Text))
  (set `/Game/ProjectAI/Core/Game/Features/UI/Widgets/Systems/InteractSystem/WBP_Interaction.InteractionText` InteractionText (`self.InteractionWidget`)))

(fn `UserConstructionScript`)