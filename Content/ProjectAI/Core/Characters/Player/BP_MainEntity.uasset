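; BP_MainEntity is the player's main entity, which bobs while possessed and can possess the nearest detected entity.
; Possessing disables its collision and glides it onto the BP_BranchEntity's MergePoint via timeline.
; Returning re-enables collision and, if neither entity is dead, animates body and camera out of the host.
; It also handles respawn placement, the game-over widget, and filters health feedback against the controlled entity's health while unpossessed.
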(event `self.ReceiveBeginPlay`
  ;[0 0 0] Unreal Events
  (`parent.ReceiveBeginPlay`)
  (set `self.IsPossessed` true))

(event `self.ReceiveTick`
  (params (DeltaSeconds :type "Float (single-precision)"))
  ;[0 0 0] Unreal Events
  (`parent.ReceiveTick` DeltaSeconds)
  (`self.AddBobbingMotion` (`self.Mesh`) 0.5 0.0 3.0))

(event `self.TryPossessNewEntity`
  (bind _detectedentities (`self.DetectedEntities`))
  ;[0 0 0] Custom Events Override
  (if (> (`KismetArrayLibrary.Array_Length` _detectedentities) 0)
    (`self.PossessNewEntity` (`self.GetNearestEntity` _detectedentities) self)))

(event `self.PossessionEnded`
  (params (`New Entity` :type "/Game/ProjectAI/Core/Characters/Player/BP_EntityBase Object Reference"))
  (bind (_relativelocation_x _relativelocation_y _relativelocation_z) (`KismetMathLibrary.BreakVector` (`SceneComponent.RelativeLocation` (`self.Mesh`))))
  ;[0 0 0] Custom Events Override
  (`parent.PossessionEnded` `New Entity`)
  (`PrimitiveComponent.SetCollisionEnabled` (`self.CapsuleComponent`) "NoCollision")
  (set `self.ControlledEntity` `New Entity`)
  (bind _asbp_branch_entity (cast `/Game/ProjectAI/Core/Characters/Player/BP_BranchEntity` `New Entity`))
  (set `self.StartTransform` (`self.GetTransform`))
  (bind (_direction _alpha) (`Timeline|Timeline_1` :!via `PlayFromStart`)
    (:`Update`
      (bind (_returnvalue_location _returnvalue_rotation) (`KismetMathLibrary.BreakTransform` (`SceneComponent.K2_GetComponentToWorld` (`/Game/ProjectAI/Core/Characters/Player/BP_BranchEntity.MergePoint` _asbp_branch_entity))))
      (bind _returnvalue (`KismetMathLibrary.MakeTransform` _returnvalue_location _returnvalue_rotation))
      (`self.K2_SetActorTransform` (`KismetMathLibrary.TLerp` (`self.StartTransform`) _returnvalue _alpha))
      (`SceneComponent.K2_SetRelativeLocation` (`self.Mesh`) (`KismetMathLibrary.MakeVector` 0.0 0.0 (`KismetMathLibrary.Lerp` _relativelocation_z 0.0 _alpha)) false false))
    (:`Finished`
      (`self.K2_SetActorTransform` _returnvalue false true)
      (`/Game/ProjectAI/Core/Controllers/BP_PlayerController.ShowHUD` (`self.PlayerController`)))))

(event `self.PossessionStarted`
  (params (PreviousEntity :type "/Game/ProjectAI/Core/Characters/Player/BP_EntityBase Object Reference"))
  (bind _starttransform (`self.StartTransform`))
  (bind (_returnvalue_location _returnvalue_rotation) (`KismetMathLibrary.BreakTransform` (`SceneComponent.GetRelativeTransform` (`self.Camera`))))
  ;[0 0 0] Custom Events Override
  (`parent.PossessionStarted` PreviousEntity)
  (if (or (`/Game/ProjectAI/Core/Characters/Player/BP_EntityBase.IsDead` PreviousEntity) (`self.IsDead`))
    (`PrimitiveComponent.SetCollisionEnabled` (`self.CapsuleComponent`) "QueryAndPhysics" :!label _label)
    (else
      (bind _asbp_branch_entity (cast `/Game/ProjectAI/Core/Characters/Player/BP_BranchEntity` PreviousEntity))
      (bind _camera (`/Game/ProjectAI/Core/Characters/Player/BP_EntityBase.Camera` _asbp_branch_entity))
      (`SceneComponent.K2_SetWorldLocationAndRotation` (`self.Camera`) (`SceneComponent.K2_GetComponentLocation` _camera) (`SceneComponent.K2_GetComponentRotation` _camera) false false)
      (set `self.StartCamTrs` (`KismetMathLibrary.MakeTransform` _returnvalue_location _returnvalue_rotation))
      (bind (_returnvalue_location_2 _returnvalue_rotation_2) (`KismetMathLibrary.BreakTransform` (`SceneComponent.K2_GetComponentToWorld` (`/Game/ProjectAI/Core/Characters/Player/BP_BranchEntity.MergePoint` _asbp_branch_entity))))
      (set `self.StartTransform` (`KismetMathLibrary.MakeTransform` _returnvalue_location_2 _returnvalue_rotation_2))
      (set `self.EndTransform` (`KismetMathLibrary.MakeTransform` (+ (.location _starttransform) (* (`KismetMathLibrary.GetUpVector` (`KismetMathLibrary.MakeRotator` (.roll (.rotation _starttransform)) (.pitch (.rotation _starttransform)) (.yaw (.rotation _starttransform)))) 100.0)) (`KismetMathLibrary.MakeRotator` 0.0 0.0 (.yaw (.rotation _starttransform)))))
      (bind (_direction _alpha) (`Timeline|Timeline_0` :!via `PlayFromStart`)
        (:`Update`
          (`self.K2_SetActorTransform` (`KismetMathLibrary.TLerp` (`self.StartTransform`) (`self.EndTransform`) _alpha) false true)
          (bind (_returnvalue_location_3 _returnvalue_rotation_3) (`KismetMathLibrary.BreakTransform` (`KismetMathLibrary.TLerp` (`self.StartCamTrs`) (`KismetMathLibrary.MakeTransform` (0.0 0.0 0.0)) _alpha)))
          (`SceneComponent.K2_SetRelativeLocationAndRotation` (`self.Camera`) _returnvalue_location_3 _returnvalue_rotation_3 false false))
        (:`Finished`
          (goto _label))))))

(event `self.Respawn`
  (params (RespawnTransform :type "Transform Structure"))
  ;[0 0 0] Custom Events Override
  (`parent.Respawn` RespawnTransform)
  (`self.K2_SetActorLocationAndRotation` (.location RespawnTransform) (.rotation RespawnTransform)))

(fn `AddBobbingMotion`
  (params (Target :type "SceneComponent Object Reference") (BobbingAmplitude :type "Float (double-precision)") (BobbingPhase :type "Float (double-precision)") (BobbingSpeed :type "Float (double-precision)"))
  (if (`self.IsPossessed`)
    (`SceneComponent.K2_AddRelativeLocation` Target (`KismetMathLibrary.MakeVector` 0.0 0.0 (* (`KismetMathLibrary.Sin` (+ (* BobbingSpeed (`self.GetGameTimeSinceCreation`)) BobbingPhase)) BobbingAmplitude)) false false)))

(fn `GameOver`
  (bind _returnvalue (`GameplayStatics.GetPlayerController` 0))
  (`WidgetBlueprintLibrary.SetInputMode_UIOnlyEx` _returnvalue null "DoNotLock" true)
  (set `PlayerController.bShowMouseCursor` true _returnvalue)
  (bind _returnvalue_2 (`|CreateWidget` "/Game/ProjectAI/Core/UI/WBP_GameOverUI.WBP_GameOverUI_C"))
  (`UserWidget.AddToViewport` _returnvalue_2 0))

(fn `SetHealthFeedback`
  (params (Health :type "Float (double-precision)"))
  (if (`self.IsPossessed`)
    (`parent.SetHealthFeedback` Health)
    (else
      (bind _controlledentity (`self.ControlledEntity`)
        (:`then`
          (if (< Health (`/Game/ProjectAI/Core/Characters/Player/BP_EntityBase.Health` _controlledentity))
            (`parent.SetHealthFeedback` Health)))
        (:`else`)))))

(fn `UserConstructionScript`
  (`parent.UserConstructionScript`))