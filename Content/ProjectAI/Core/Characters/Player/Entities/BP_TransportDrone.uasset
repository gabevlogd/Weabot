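; BP_TransportDrone is a possessable drone entity that grabs and releases things with a hook.
; On BeginPlay it caches its BP_Hook child actor and sizes that hook's box trace to the capsule radius.
; The two entity ability inputs call the hook's grab and ungrab attempts.
; Tick oscillates the mesh through BPCOscillator, and the merge point snaps to a mesh socket.
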(event `self.ReceiveBeginPlay`
  (`parent.ReceiveBeginPlay`)
  (`self.SetHook`))

(event `self.PossessionEnded`
  (params (`New Entity` :type "/Game/ProjectAI/Core/Characters/Player/BP_EntityBase Object Reference"))
  (`parent.PossessionEnded` `New Entity`))

(event `self.ReceiveTick`
  (params (DeltaSeconds :type "Float (single-precision)"))
  (`parent.ReceiveTick` DeltaSeconds)
  (`self.MeshOscillation`))

(event `EnhancedInput|/Game/ProjectAI/Core/Inputs/Actions/IA_EntityAbility_0`
  (params (ActionValue :type Boolean) (ElapsedSeconds :type "Float (double-precision)") (TriggeredSeconds :type "Float (double-precision)") (InputAction :type "InputAction Object Reference" :default "/Game/ProjectAI/Core/Inputs/Actions/IA_EntityAbility_0.IA_EntityAbility_0"))
  (:`Triggered`
    (`/Game/ProjectAI/Core/Props/Hook/BP_Hook.TryGrab` (`self.HookActor`))))

(event `EnhancedInput|/Game/ProjectAI/Core/Inputs/Actions/IA_EntityAbility_1`
  (params (ActionValue :type Boolean) (ElapsedSeconds :type "Float (double-precision)") (TriggeredSeconds :type "Float (double-precision)") (InputAction :type "InputAction Object Reference" :default "/Game/ProjectAI/Core/Inputs/Actions/IA_EntityAbility_1.IA_EntityAbility_1"))
  (:`Triggered`
    (`/Game/ProjectAI/Core/Props/Hook/BP_Hook.TryUngrab` (`self.HookActor`))))

(fn `MeshOscillation`
  (`/Game/ProjectAI/Core/Utility/Components/ActorComponents/AC_Oscillator.Oscillation` (`self.BPC_Oscillator`) (`self.Mesh`)))

(fn `SetMergePoint`
  (`parent.SetMergePoint`)
  (`SceneComponent.K2_AttachToComponent` (`self.MergePoint`) (`self.Mesh`) (`self.MergePointSocket`) "SnapToTarget" "SnapToTarget" "KeepWorld" true))

(fn `UserConstructionScript`
  (`parent.UserConstructionScript`))