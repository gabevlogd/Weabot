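; BP_DamageZone is a volume actor that repeatedly damages actors while they stay inside it.
; DamageVolume overlap events keep a list of damageable actors inside, skipping exact classes listed in ActorToIgnore.
; The first entry starts a self-calling event that applies DamagePerHit to every listed actor, then waits one tick, stopping when the list empties.
; Damage lands every tick, so its rate depends on frame rate.
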(event `ApplyDamageEvent`
  (if (not (== (`KismetArrayLibrary.Array_Length` (`self.ActorsInZone`)) 0))
    (for _array_element (`self.ActorsInZone`)
      (`GameplayStatics.ApplyDamage` _array_element (`self.DamagePerHit`)))
    (`KismetSystemLibrary.DelayUntilNextTick`)
    (`self.ApplyDamageEvent`)))

(event `self.DamageVolume.OnComponentBeginOverlap`
  (params (OverlappedComponent :type "PrimitiveComponent Object Reference") (OtherActor :type "Actor Object Reference") (OtherComp :type "PrimitiveComponent Object Reference") (OtherBodyIndex :type Integer) (bFromSweep :type Boolean) (SweepResult :type "HitResult Structure (by ref)"))
  (`self.IsValidActor` OtherActor
    (:`True`
      (if (`Actor.bCanBeDamaged` OtherActor)
        (`KismetArrayLibrary.Array_Add` (`self.ActorsInZone`) OtherActor)
        (if (== (`KismetArrayLibrary.Array_Length` (`self.ActorsInZone`)) 1)
          (`self.ApplyDamageEvent`))))))

(event `self.DamageVolume.OnComponentEndOverlap`
  (params (OverlappedComponent :type "PrimitiveComponent Object Reference") (OtherActor :type "Actor Object Reference") (OtherComp :type "PrimitiveComponent Object Reference") (OtherBodyIndex :type Integer))
  (`self.IsValidActor` OtherActor
    (:`True`
      (if (`Actor.bCanBeDamaged` OtherActor)
        (`KismetArrayLibrary.Array_RemoveItem` (`self.ActorsInZone`) OtherActor)))))

(fn `UserConstructionScript`)