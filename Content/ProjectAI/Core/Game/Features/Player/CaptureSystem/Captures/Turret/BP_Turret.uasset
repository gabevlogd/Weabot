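; Possessable, stationary turret entity from the capture system that aims with control yaw and fires a laser to break destructible objects.
; A per-tick camera sphere trace sets the laser end point and activates the crosshair over Geometry Collections.
; The ability input starts the laser cycle; when the laser enables, it spawns a directional force field at the hit and shakes the camera.
; Possession toggles pitch limits and the HUD pointer.
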(event `self.ReceiveBeginPlay`
  ;[0 0 0] Unreal Events Override
  (`parent.ReceiveBeginPlay`)
  (`/Game/ProjectAI/Core/Game/Features/Gameplay/WeaponSystem/Laser/Components/AC_Laser.Init` (`self.AC_Laser`) null (`|MakeArray` (`self.FirePoint`))))

(event `self.ReceiveTick`
  (params (DeltaSeconds :type "Float (single-precision)"))
  ;[0 0 0] Unreal Events Override
  (`parent.ReceiveTick` DeltaSeconds)
  (`self.Aim`)
  (`/Game/ProjectAI/Core/Game/Features/Gameplay/WeaponSystem/Laser/Components/AC_Laser.UpdateCustomLaserEndPoint` (`self.AC_Laser`) (`self.GetLaserEndPoint`))
  (cast `GeometryCollectionActor` (`self.HittedActor`)
    (:`then`
      (`/Engine/EditorBlueprintResources/StandardMacros.DoOnce` false :!label _label
        (:`Completed`
          (bind _playerhudwidget (`/Game/ProjectAI/Core/Game/Utility/BFL_PAIGenericUtility.GetPlayerHUD`))
          (`/Game/ProjectAI/Core/Game/Features/UI/Widgets/Menus/PlayerHUD/WBP_PlayerHUD.ActiveCrosshair` _playerhudwidget)
          (goto _label_2 :!via `Reset`))))
    (:`CastFailed`
      (`/Engine/EditorBlueprintResources/StandardMacros.DoOnce` false :!label _label_2
        (:`Completed`
          (bind _playerhudwidget_2 (`/Game/ProjectAI/Core/Game/Utility/BFL_PAIGenericUtility.GetPlayerHUD`))
          (`/Game/ProjectAI/Core/Game/Features/UI/Widgets/Menus/PlayerHUD/WBP_PlayerHUD.DeactiveCrosshair` _playerhudwidget_2)
          (goto _label :!via `Reset`))))))

(event `EnhancedInput|/Game/ProjectAI/Core/Game/Inputs/Actions/IA_EntityAbility_0`
  (params (ActionValue :type Boolean) (ElapsedSeconds :type "Float (double-precision)") (TriggeredSeconds :type "Float (double-precision)") (InputAction :type "InputAction Object Reference" :default "/Game/ProjectAI/Core/Game/Inputs/Actions/IA_EntityAbility_0.IA_EntityAbility_0"))
  ;[0 0 0] Shoot
  (:`Triggered`
    (`/Game/ProjectAI/Core/Game/Features/Gameplay/WeaponSystem/Laser/Components/AC_Laser.StartLaserCycle` (`self.AC_Laser`))))

(event `self.AC_Laser.OnLaserEnabled`
  ;[0 0 0] Shoot
  (`self.TryDestroyGeometryCollection` (`self.HitPoint`) (`self.HitNormal`) (`self.HittedActor`))
  (`CameraShakeSourceComponent.StartCameraShake` :`self` (`self.ShootShakeSource`) :`InCameraShake` "/Game/ProjectAI/Core/Game/Features/Player/CaptureSystem/Captures/Turret/BP_TurretCameraShake.BP_TurretCameraShake_C"))

(event `self.PossessionStarted`
  (params (PreviousEntity :type "/Game/ProjectAI/Core/Game/Features/Player/Base/BP_EntityBase Object Reference"))
  ;[0 0 0] Custom Events Override
  (`parent.PossessionStarted` PreviousEntity)
  (`self.SetPitchAngleLimit` (`self.MinAimPitch`) (`self.MaxAimPitch`))
  (bind _playerhudwidget (`/Game/ProjectAI/Core/Game/Utility/BFL_PAIGenericUtility.GetPlayerHUD`))
  (`/Game/ProjectAI/Core/Game/Features/UI/Widgets/Menus/PlayerHUD/WBP_PlayerHUD.SetPointerEnabled` _playerhudwidget true))

(event `self.PossessionEnded`
  (params (`New Entity` :type "/Game/ProjectAI/Core/Game/Features/Player/Base/BP_EntityBase Object Reference"))
  ;[0 0 0] Custom Events Override
  (`parent.PossessionEnded` `New Entity`)
  (`self.SetPitchAngleLimit` -90.0 90.0)
  (bind _playerhudwidget (`/Game/ProjectAI/Core/Game/Utility/BFL_PAIGenericUtility.GetPlayerHUD`))
  (`/Game/ProjectAI/Core/Game/Features/UI/Widgets/Menus/PlayerHUD/WBP_PlayerHUD.SetPointerEnabled` _playerhudwidget false))

(fn `Aim`
  (bind (_returnvalue_roll _returnvalue_pitch _returnvalue_yaw) (`KismetMathLibrary.BreakRotator` (`self.GetControlRotation`)))
  (bind (_returnvalue_roll_2 _returnvalue_pitch_2) (`KismetMathLibrary.BreakRotator` (`self.K2_GetActorRotation`)))
  (`self.K2_SetActorRotation` (`KismetMathLibrary.MakeRotator` _returnvalue_roll_2 _returnvalue_pitch_2 _returnvalue_yaw)))

(fn `GetLaserEndPoint`
  (returns (ReturnValue :type "Vector Structure"))
  (bind _returnvalue (`SceneComponent.K2_GetComponentLocation` (`self.Camera`)))
  (bind (_outhit _returnvalue_2) (`KismetSystemLibrary.SphereTraceSingle` _returnvalue (+ _returnvalue (* (`KismetMathLibrary.GetForwardVector` (`self.GetControlRotation`)) (`/Game/ProjectAI/Core/Game/Features/Gameplay/WeaponSystem/Laser/Components/AC_Laser.MaxLenght` (`self.AC_Laser`)))) 5.0 "TraceTypeQuery2"))
  (bind (_bblockinghit _binitialoverlap _time _distance _location _impactpoint _normal _impactnormal _physmat _hitactor) (`GameplayStatics.BreakHitResult` _outhit))
  (set `self.HittedActor` _hitactor)
  (set `self.HitNormal` _impactnormal)
  (set `self.HitPoint` _impactpoint)
  (if _returnvalue_2
    (return _impactpoint)
    (else
      (return (+ (`SceneComponent.K2_GetComponentLocation` (`self.Camera`)) (* (`KismetMathLibrary.GetForwardVector` (`self.GetControlRotation`)) (`self.MaxShootDistance`)))))))

(fn `Move`
  (params (MoveInput :type "Vector Structure")))

(fn `PlayShootFX`
  (returns (ReturnValue :type "ParticleSystemComponent Object Reference"))
  (`CameraShakeSourceComponent.StartCameraShake` :`self` (`self.ShootShakeSource`) :`InCameraShake` "/Game/ProjectAI/Core/Game/Features/Player/CaptureSystem/Captures/Turret/BP_TurretCameraShake.BP_TurretCameraShake_C")
  (return null))

(fn `SetHealthBarSocket`
  (`parent.SetHealthBarSocket`)
  (`SceneComponent.K2_AttachToComponent` (`self.HealthBar`) (`self.HealthBarSocket`) "None" "SnapToTarget" "SnapToTarget" "SnapToTarget" true))

(fn `SetMergePoint`
  (`SceneComponent.K2_AttachToComponent` (`self.MergePoint`) (`self.Mesh`) (`self.MergePointSocket`) "SnapToTarget" "SnapToTarget" "KeepWorld" true))

(fn `SetPitchAngleLimit`
  (params (`View Pitch Min` :type "Float (single-precision)") (`View Pitch Max` :type "Float (single-precision)"))
  (bind _returnvalue (`GameplayStatics.GetPlayerCameraManager` 0))
  (set `PlayerCameraManager.ViewPitchMin` `View Pitch Min` _returnvalue)
  (set `PlayerCameraManager.ViewPitchMax` `View Pitch Max` _returnvalue))

(fn `Shoot`
  (bind _returnvalue (`SceneComponent.K2_GetComponentLocation` (`self.Camera`)))
  (`|ExecutionSequence`
    (:`then_0`
      (bind (_bsuccess _gameevents) (`/Game/ProjectAI/Core/Game/Managers/Events/Utility/BFL_GameEventsUtility.TryGetGameEvents`))
      (if _bsuccess
        (`/Game/ProjectAI/Core/Game/Managers/Events/AC_GameEvents.OnPlayerShoot` _gameevents)))
    (:`then_1`
      (bind _outhit (`KismetSystemLibrary.SphereTraceSingle` :`Start` _returnvalue :`End` (+ _returnvalue (* (`KismetMathLibrary.GetForwardVector` (`self.GetControlRotation`)) (`self.MaxShootDistance`))) :`Radius` 5.0 :`TraceChannel` "TraceTypeQuery2" :`DrawDebugType` "ForDuration"))
      (`self.TryDestroyGeometryCollection` (`.ImpactPoint` (`GameplayStatics.BreakHitResult` _outhit)) (`.ImpactNormal` (`GameplayStatics.BreakHitResult` _outhit)) (`.HitActor` (`GameplayStatics.BreakHitResult` _outhit))))))

(fn `TryDestroyGeometryCollection`
  (params (`Hit Point` :type "Vector Structure") (`Hit Normal` :type "Vector Structure") (`Hit Actor` :type "Actor Object Reference"))
  (cast `GeometryCollectionActor` `Hit Actor`)
  (bind _returnvalue (`|SpawnActorFromClass` (`self.ForceFieldType`) (`KismetMathLibrary.MakeTransform` `Hit Point` (`KismetMathLibrary.MakeRotFromZ` (* `Hit Normal` -1.0))) "Undefined" "MultiplyWithRoot" null null))
  (set `/Engine/EditorResources/FieldNodes/FS_MasterField.DirectionalMagnitude` (`self.ForceMagnitude`) _returnvalue)
  (`/Engine/EditorResources/FieldNodes/FS_MasterField.CE_Trigger` _returnvalue))

(fn `UserConstructionScript`
  (`parent.UserConstructionScript`))