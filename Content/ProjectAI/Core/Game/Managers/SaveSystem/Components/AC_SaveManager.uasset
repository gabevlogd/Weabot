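; AC_SaveManager is an actor component that saves and loads the game's SaveGame object in a named slot for user index 0.
; Load reads the slot if a save exists, otherwise CreateSaveFile makes a new SaveGame object and immediately writes it.
; Save writes the held SaveGame object to that slot.
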(event `Save`
  (`GameplayStatics.SaveGameToSlot` (`self.SaveGame`) (`self.Slot Name`)))

(event `Load`
  (bind _returnvalue (`GameplayStatics.DoesSaveGameExist` (`self.Slot Name`)))
  (if _returnvalue
    (bind _returnvalue_2 (`GameplayStatics.LoadGameFromSlot` (`self.Slot Name`)))
    (set `self.SaveGame` _returnvalue_2)
    (else
      (`self.CreateSaveFile`))))

(fn `CreateSaveFile`
  (bind _returnvalue (`GameplayStatics.CreateSaveGameObject` "/Script/Engine.SaveGame"))
  (set `self.SaveGame` _returnvalue)
  (`self.Save`))