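; Base component for settings managers that persist their settings through a SaveGame object in a named slot.
; Init stores the slot path and loads the existing save, or creates one from the configured SaveGame class if none exists.
; Saving writes the object back to that slot.
; Empty OnSavedSettings and OnLoadedSettings events serve as hooks, with the saved hook firing only on a successful write.
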(event `Init`
  (params (SaveFilePath :type String))
  (set `self.SaveFilePath` SaveFilePath)
  (`self.LoadSettingsSaveGame`))

(event `SaveSettingsSaveGame`
  (bind _returnvalue (`GameplayStatics.SaveGameToSlot` (`self.SettingsSaveGame`) (`self.SaveFilePath`)))
  (if _returnvalue
    (`self.OnSavedSettings` (`self.SettingsSaveGame`))))

(event `LoadSettingsSaveGame`
  (bind _returnvalue (`GameplayStatics.DoesSaveGameExist` (`self.SaveFilePath`)))
  (if _returnvalue
    (bind _returnvalue_2 (`GameplayStatics.LoadGameFromSlot` (`self.SaveFilePath`)))
    (set `self.SettingsSaveGame` _returnvalue_2)
    (else
      (bind _returnvalue_3 (`GameplayStatics.CreateSaveGameObject` (`self.SaveGameClass`)))
      (set `self.SettingsSaveGame` _returnvalue_3)))
  (`self.OnLoadedSettings` (`self.SettingsSaveGame`)))

(event `OnSavedSettings`
  (params (SettingsSaveGame :type "SaveGame Object Reference")))

(event `OnLoadedSettings`
  (params (SettingsSaveGame :type "SaveGame Object Reference")))