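; Socket actor that accepts a BP_SocketableBase of matching type on trigger overlap and snaps it in place.
; A placed socketable with a matching key activates the linked activable group through ACGroupTriggerActivable, while a wrong key still fills the socket.
; Grabbing the socketable out empties the socket and deactivates the group.
; Global grab events make the socket highlightable through custom depth only while it is empty and the player holds something.
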(event `self.ReceiveBeginPlay`
  (bind (_bsuccess _gameevents) (`/Game/ProjectAI/Core/Game/Managers/Events/Utility/BFL_GameEventsUtility.TryGetGameEvents`))
  (if _bsuccess
    (bind _output_get (set `self.GameEvents` _gameevents))
    (add `/Game/ProjectAI/Core/Game/Managers/Events/Components/AC_GameEvents.OnPlayerGrab` _output_get (delegate `OnPlayerGrab_Event`))
    (add `/Game/ProjectAI/Core/Game/Managers/Events/Components/AC_GameEvents.OnPlayerUngrab` _output_get (delegate `OnPlayerUngrab_Event`))))

(event `OnPlayerGrab_Event`
  (set `self.bIsPlayerGrabbing` true))

(event `OnPlayerUngrab_Event`
  (set `self.bIsPlayerGrabbing` false))

(event `self.SocketTrigger.OnComponentBeginOverlap`
  (params (OverlappedComponent :type "PrimitiveComponent Object Reference") (OtherActor :type "Actor Object Reference") (OtherComp :type "PrimitiveComponent Object Reference") (OtherBodyIndex :type Integer) (bFromSweep :type Boolean) (SweepResult :type "HitResult Structure (by ref)"))
  (`self.CheckSocketable` OtherActor))

(event `CheckSocketable`
  (params (Actor :type "Actor Object Reference"))
  (if (not (`self.bIsFilled`))
    (bind _asbp_socket_base (`self.IsSocketableValid` Actor)
      (:`True`
        (bind _output_get (set `self.CurrentSocketable` _asbp_socket_base))
        (add `/Game/ProjectAI/Core/Game/Features/Gameplay/ActivableSocketSystem/BP_SocketableBase.OnSocketableGrabbed` _output_get (`|CreateDelegate` :!event `OnSocketableGrabbed_Event`))
        (`self.Place Socketable in Socket`)
        (`self.HasSameKey` (`self.CurrentSocketable`)
          (:`true`
            (`/Game/ProjectAI/Core/Game/Features/Gameplay/InteractSystem/Components/AC_GroupTriggerActivable.ActivateAll` (`self.AC_GroupTriggerActivable`))))))))

(event `OnSocketableGrabbed_Event`
  (remove `/Game/ProjectAI/Core/Game/Features/Gameplay/ActivableSocketSystem/BP_SocketableBase.OnSocketableGrabbed` (`self.CurrentSocketable`) (`|CreateDelegate` :!event `OnSocketableGrabbed_Event`))
  (`self.RemoveSocketableFromSocket`)
  (`/Game/ProjectAI/Core/Game/Features/Gameplay/InteractSystem/Components/AC_GroupTriggerActivable.DeactivateAll` (`self.AC_GroupTriggerActivable`)))

(event `/Game/ProjectAI/Core/Game/Features/Gameplay/HighlightingSystem/BPI_Highlightable.StartHighlight`
  (`PrimitiveComponent.SetRenderCustomDepth` (`self.Base`) true))

(event `/Game/ProjectAI/Core/Game/Features/Gameplay/HighlightingSystem/BPI_Highlightable.StopHighlight`
  (`PrimitiveComponent.SetRenderCustomDepth` (`self.Base`) false))

(fn `CanBeHighlighted`
  (returns (Result :type Boolean))
  (return (and (not (`self.bIsFilled`)) (`self.bIsPlayerGrabbing`))))

(fn `Place Socketable in Socket`
  (bind _currentsocketable (`self.CurrentSocketable`)
    (:`then`
      (`self.K2_SetActorLocationAndRotation` :`self` _currentsocketable :`NewLocation` (`SceneComponent.K2_GetComponentLocation` (`self.SocketTrigger`)) :`bTeleport` true)
      (set `self.bIsFilled` true)
      (`/Game/ProjectAI/Core/Game/Features/Gameplay/ActivableSocketSystem/Interfaces/BPI_Socketable.PlaceSocket` (`self.CurrentSocketable`))
      (return))
    (:`else`)))

(fn `RemoveSocketableFromSocket`
  (`/Game/ProjectAI/Core/Game/Features/Gameplay/ActivableSocketSystem/Interfaces/BPI_Socketable.RemoveSocket` (`self.CurrentSocketable`))
  (set `self.bIsFilled` false))

(fn `UserConstructionScript`)