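; Aim preview actor for the throwing system that draws a path as spline mesh segments with a marker at its end.
; AddPoint stores points and tangents, then ShowSpline stretches a mesh between each consecutive pair and places HitPoint on the last point.
; Segments are pooled: BeginPlay fills OpenMeshes, GetMesh reuses or creates components, and ClearSpline hides and returns them, empties the path and hides HitPoint.
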(event `self.ReceiveBeginPlay`
  (for (_ _array_index) (`self.OpenMeshes`)
    (bind _returnvalue (`AddComponent|NODE_AddSplineMeshComponent-1` :`bManualAttachment` true))
    (`KismetArrayLibrary.Array_Set` (`self.OpenMeshes`) _array_index _returnvalue)))

(fn `AddPoint`
  (params (Point :type "Vector Structure") (Tangent :type "Vector Structure (by ref)"))
  (`KismetArrayLibrary.Array_Add` (`self.Points`) Point)
  (`KismetArrayLibrary.Array_Add` (`self.Tangents`) Tangent))

(fn `ClearSpline`
  (for _array_element (`self.ClosedMeshes`)
    (`self.ReleaseMesh` _array_element))
  (`KismetArrayLibrary.Array_Clear` (`self.ClosedMeshes`))
  (`KismetArrayLibrary.Array_Clear` (`self.Points`))
  (`KismetArrayLibrary.Array_Clear` (`self.Tangents`))
  (`self.HideHitPoint`))

(fn `GetMesh`
  (returns (SplineMesh :type "SplineMeshComponent Object Reference"))
  (locals (Mesh :type "SplineMeshComponent Object Reference"))
  (for (_array_element _array_index) (`self.OpenMeshes`)
    (`/Engine/EditorBlueprintResources/StandardMacros.IsValid` _array_element
      (:`Is Valid`
        (`KismetArrayLibrary.Array_Add` (`self.ClosedMeshes`) _array_element)
        (`SceneComponent.SetVisibility` _array_element true false)
        (`|VariableSetRef` (`local.Mesh`) _array_element)
        (`KismetArrayLibrary.Array_Remove` (`self.OpenMeshes`) _array_index)
        (break))))
  (`/Engine/EditorBlueprintResources/StandardMacros.IsValid` (`local.Mesh`)
    (:`Is Valid`
      (return (`local.Mesh`)))
    (:`Is Not Valid`
      (bind _returnvalue (`AddComponent|NODE_AddSplineMeshComponent-2` :`bManualAttachment` true))
      (`KismetArrayLibrary.Array_Add` (`self.ClosedMeshes`) _returnvalue)
      (return _returnvalue))))

(fn `HideHitPoint`
  (`SceneComponent.SetVisibility` (`self.HitPoint`) false false))

(fn `ReleaseMesh`
  (params (Mesh :type "SplineMeshComponent Object Reference (by ref)"))
  (`SceneComponent.SetVisibility` Mesh false false)
  (`KismetArrayLibrary.Array_Add` (`self.OpenMeshes`) Mesh))

(fn `ShowHitPoint`
  (params (NewLocation :type "Vector Structure"))
  (`SceneComponent.K2_SetWorldLocation` (`self.HitPoint`) NewLocation false false)
  (`SceneComponent.SetVisibility` (`self.HitPoint`) true false))

(fn `ShowSpline`
  (for _index (range (+ (- (`KismetArrayLibrary.Array_Length` (`self.Points`)) 2) 1))
    (bind _splinemesh (`self.GetMesh`))
    (bind _returnvalue (+ _index 1))
    (bind _output (`|GetArrayItem` (`self.Points`) _returnvalue))
    (`SplineMeshComponent.SetStartAndEnd` _splinemesh (`|GetArrayItem` (`self.Points`) _index) (`|GetArrayItem` (`self.Tangents`) _index) _output (`|GetArrayItem` (`self.Tangents`) _returnvalue) true)
    (if (== _index (- (`KismetArrayLibrary.Array_Length` (`self.Points`)) 2))
      (`self.ShowHitPoint` _output))))

(fn `UserConstructionScript`)