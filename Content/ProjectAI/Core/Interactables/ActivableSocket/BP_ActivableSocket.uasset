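; BP_ActivableSocket is an interactable socket that holds a socketable actor and activates linked interactables when given the correct key.
; On trigger overlap, it accepts a placeable BP_SocketableBase of matching SocketType, snaps it to the trigger with zero rotation and disables trigger collision.
; A key name matching CorrectKey calls InteractAll on ACGroupTriggerInteractable.
; The socketable's grab callback empties the socket and re-enables the trigger, without another InteractAll call.
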(event `self.SocketTrigger.OnComponentBeginOverlap`
  (params (OverlappedComponent :type "PrimitiveComponent Object Reference") (OtherActor :type "Actor Object Reference") (OtherComp :type "PrimitiveComponent Object Reference") (OtherBodyIndex :type Integer) (bFromSweep :type Boolean) (SweepResult :type "HitResult Structure (by ref)"))
  (if (not (`self.bIsFilled`))
    (bind _asbp_socket_base (`self.CheckSocketableActor` OtherActor)
      (:`True`
        (`self.PlaceInSocket` _asbp_socket_base)
        (`PrimitiveComponent.SetCollisionEnabled` (`self.SocketTrigger`) "NoCollision")
        (set `self.bIsFilled` true)
        (set `self.CurrentSocketable` _asbp_socket_base)
        (add `/Game/ProjectAI/Core/Interactables/ActivableSocket/BP_SocketableBase.OnSocketGrabbed` _asbp_socket_base (delegate `OnSocketGrabbed_Event`))
        (bind _key (`/Game/ProjectAI/Core/Interactables/ActivableSocket/Data/BP_SocketKeyData.GetKeyName` (`/Game/ProjectAI/Core/Interactables/ActivableSocket/BP_SocketableBase.SocketableKey` _asbp_socket_base)))
        (bind _key_2 (`/Game/ProjectAI/Core/Interactables/ActivableSocket/Data/BP_SocketKeyData.GetKeyName` (`self.CorrectKey`)))
        (if (== _key _key_2)
          (`/Game/ProjectAI/Core/Interactables/Components/AC_GroupTriggerInteractable.InteractAll` (`self.AC_GroupTriggerInteractable`))
          (`KismetSystemLibrary.PrintString` "Same kEy!"))))))

(event `OnSocketGrabbed_Event`
  (set `self.bIsFilled` false)
  (`self.RemoveFromSocket` (`self.CurrentSocketable`))
  (`PrimitiveComponent.SetCollisionEnabled` (`self.SocketTrigger`) "QueryOnly"))

(fn `PlaceInSocket`
  (params (Socketable :type "/Game/ProjectAI/Core/Interactables/ActivableSocket/BP_SocketableBase Object Reference"))
  (`/Game/ProjectAI/Core/Interactables/ActivableSocket/Interfaces/BPI_Socketable.PlaceSocket` Socketable)
  (`self.Set in Socket Location` Socketable))

(fn `RemoveFromSocket`
  (params (Socketable :type "/Game/ProjectAI/Core/Interactables/ActivableSocket/BP_SocketableBase Object Reference"))
  (`/Game/ProjectAI/Core/Interactables/ActivableSocket/Interfaces/BPI_Socketable.RemoveSocket` Socketable))

(fn `Set in Socket Location`
  (params (Actor :type "Actor Object Reference"))
  (`self.K2_SetActorLocation` Actor (`SceneComponent.K2_GetComponentLocation` (`self.SocketTrigger`)) false false)
  (`self.K2_SetActorRotation` :`self` Actor))

(fn `UserConstructionScript`)