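; BP_ActivableBase is the base Blueprint in the interact system for objects that can be activated and deactivated.
; On BeginPlay it calls Activate or Deactivate according to IsActiveOnBegin.
; Both events only set the IsActivableActive flag, which IsActivavableActive and GetIsActive each return.
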(event `self.ReceiveBeginPlay`
  (if (`self.bIsActiveOnBegin`)
    (`/Game/ProjectAI/Core/Game/Features/Gameplay/InteractSystem/Interfaces/BPI_Activable.Activate`)
    (else
      (`/Game/ProjectAI/Core/Game/Features/Gameplay/InteractSystem/Interfaces/BPI_Activable.Deactivate`))))

(event `/Game/ProjectAI/Core/Game/Features/Gameplay/InteractSystem/Interfaces/BPI_Activable.Activate`
  (set `self.bIsActivableActive` true))

(event `/Game/ProjectAI/Core/Game/Features/Gameplay/InteractSystem/Interfaces/BPI_Activable.Deactivate`
  (set `self.bIsActivableActive` false))

(fn `GetIsActive`
  (returns (bIsActivableActive :type Boolean))
  (return (`self.bIsActivableActive`)))

(fn `IsActivavableActive`
  (returns (bIsActivableActive :type Boolean))
  (return (`self.bIsActivableActive`)))

(fn `UserConstructionScript`)