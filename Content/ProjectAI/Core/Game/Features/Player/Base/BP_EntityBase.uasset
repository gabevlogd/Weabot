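; Base pawn for possessable player entities, with movement, health, interaction and timed invisibility.
; Possession swaps controller and highlighter state, then broadcasts through GameEvents, which also relays death.
; A radar overlap collects interactables; Tick shows a HUD prompt for the nearest.
; The health component drives screen-damage VFX and camera shake, while invisibility fades a dynamic material via a self-recalling per-tick event and blocks player sensing.
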(event `self.ReceiveBeginPlay`
  ;[0 0 0] Unreal Events
  (`PrimitiveComponent.IgnoreActorWhenMoving` (`self.EntityRadar`) self true)
  (`self.CacheGameMode`)
  (`self.CachePlayerController`)
  (`self.CacheGameEvents`)
  (`self.CacheHUD`)
  (`self.InitInvisibility`))

(event `TryPossessNewEntity`
  ;[0 0 0] Custom Events
)

(event `self.ReceiveTick`
  (params (DeltaSeconds :type "Float (single-precision)"))
  ;[0 0 0] Unreal Events
  (`self.LookForInteraction`))

(event `PossessNewEntity`
  (params (NewEntity :type "/Game/ProjectAI/Core/Game/Features/Player/Base/BP_EntityBase Object Reference") (PreviousEntity :type "/Game/ProjectAI/Core/Game/Features/Player/Base/BP_EntityBase Object Reference"))
  ;[0 0 0] Custom Events
  (`self.PossessionEnded` NewEntity)
  (`Controller.Possess` (`GameplayStatics.GetPlayerController` 0) NewEntity)
  (`self.PossessionStarted` NewEntity PreviousEntity)
  (bind (_bsuccess _gameevents) (`/Game/ProjectAI/Core/Game/Managers/Events/Utility/BFL_GameEventsUtility.TryGetGameEvents`))
  (`/Game/ProjectAI/Core/Game/Managers/Events/Components/AC_GameEvents.OnEntityChanged` _gameevents NewEntity PreviousEntity))

(event `EnhancedInput|/Game/ProjectAI/Core/Game/Inputs/Actions/IA_Look`
  (params (ActionValue :type "Vector2D Structure") (ElapsedSeconds :type "Float (double-precision)") (TriggeredSeconds :type "Float (double-precision)") (InputAction :type "InputAction Object Reference" :default "/Game/ProjectAI/Core/Game/Inputs/Actions/IA_Look.IA_Look"))
  ;[0 0 0] Movement
  (:`Triggered`
    (`self.Look` ActionValue)))

(event `EnhancedInput|/Game/ProjectAI/Core/Game/Inputs/Actions/IA_Move`
  (params (ActionValue :type "Vector Structure") (ElapsedSeconds :type "Float (double-precision)") (TriggeredSeconds :type "Float (double-precision)") (InputAction :type "InputAction Object Reference" :default "/Game/ProjectAI/Core/Game/Inputs/Actions/IA_Move.IA_Move"))
  ;[0 0 0] Movement
  (:`Triggered`
    (`self.Move` ActionValue)))

(event `PossessionStarted`
  (params (PreviousEntity :type "/Game/ProjectAI/Core/Game/Features/Player/Base/BP_EntityBase Object Reference"))
  ;[0 0 0] Custom Events
  (set `self.IsPossessed` true)
  (`self.DisableInput` (`GameplayStatics.GetPlayerController` 0))
  (`/Game/ProjectAI/Core/Game/Features/Gameplay/HealthSystem/Components/AC_HealthManager.ResetHpRegaining` (`self.AC_HealthManager`))
  (`/Game/ProjectAI/Core/Game/Features/Gameplay/HighlightingSystem/HighlighterComponent.Active` (`self.HighlighterComponent`) true))

(event `self.EntityRadar.OnComponentBeginOverlap`
  (params (OverlappedComponent :type "PrimitiveComponent Object Reference") (OtherActor :type "Actor Object Reference") (OtherComp :type "PrimitiveComponent Object Reference") (OtherBodyIndex :type Integer) (bFromSweep :type Boolean) (SweepResult :type "HitResult Structure (by ref)"))
  ;[0 0 0] Entity Detection
  (bind _asbpi_interactable (cast `/Game/ProjectAI/Core/Game/Features/Gameplay/InteractSystem/Interfaces/BPI_Interactable` OtherActor))
  (`self.AddInteractable` _asbpi_interactable))

(event `PossessionEnded`
  (params (`New Entity` :type "/Game/ProjectAI/Core/Game/Features/Player/Base/BP_EntityBase Object Reference"))
  ;[0 0 0] Custom Events
  (set `self.IsPossessed` false)
  (`self.SetActorTickEnabled` false)
  (`/Game/ProjectAI/Core/Game/Features/Gameplay/HealthSystem/Components/AC_HealthManager.ResetHpRegaining` (`self.AC_HealthManager`))
  (`/Game/ProjectAI/Core/Game/Features/Gameplay/HighlightingSystem/HighlighterComponent.Active` (`self.HighlighterComponent`) false))

(event `self.EntityRadar.OnComponentEndOverlap`
  (params (OverlappedComponent :type "PrimitiveComponent Object Reference") (OtherActor :type "Actor Object Reference") (OtherComp :type "PrimitiveComponent Object Reference") (OtherBodyIndex :type Integer))
  ;[0 0 0] Entity Detection
  (bind _asbpi_interactable (cast `/Game/ProjectAI/Core/Game/Features/Gameplay/InteractSystem/Interfaces/BPI_Interactable` OtherActor))
  (`self.RemoveInteractable` _asbpi_interactable))

(event `Respawn`
  (params (RespawnTransform :type "Transform Structure"))
  ;[0 0 0] Custom Events
  (`/Game/ProjectAI/Core/Game/Features/Gameplay/HealthSystem/Components/AC_HealthManager.RestoreHealth` (`self.AC_HealthManager`)))

(event `self.ReceiveAnyDamage`
  (params (Damage :type "Float (single-precision)") (DamageType :type "DamageType Object Reference") (InstigatedBy :type "Controller Object Reference") (DamageCauser :type "Actor Object Reference"))
  ;[0 0 0] Damage
  (`/Game/ProjectAI/Core/Game/Features/Gameplay/HealthSystem/Components/AC_HealthManager.TakeDamage` (`self.AC_HealthManager`) Damage))

(event `self.AC_HealthManager.OnRegainingHealth`
  (params (Health :type "Float (double-precision)"))
  ;[0 0 0] Health Manager Events
  (`self.SetHealthVFX` Health))

(event `self.AC_HealthManager.OnTakeDamage`
  (params (Health :type "Float (double-precision)") (Damage :type "Float (double-precision)"))
  ;[0 0 0] Health Manager Events
  (`self.SetHealthVFX` Health)
  (if (`self.IsPossessed`)
    (`CameraShakeSourceComponent.StartCameraShake` :`self` (`self.DamageShakeSource`) :`InCameraShake` "/Game/ProjectAI/Core/Game/Features/Player/BP_DamageCameraShake.BP_DamageCameraShake_C")))

(event `self.AC_HealthManager.OnDeath`
  ;[0 0 0] Health Manager Events
  (bind (_bsuccess _gameevents) (`/Game/ProjectAI/Core/Game/Managers/Events/Utility/BFL_GameEventsUtility.TryGetGameEvents`))
  (if _bsuccess
    (`/Game/ProjectAI/Core/Game/Managers/Events/Components/AC_GameEvents.OnEntityDeath` _gameevents)))

(event `InvisibilityTransitionAnim`
  (bind _output_get (set `self.ElapsedTime` (+ (`self.ElapsedTime`) (`GameplayStatics.GetWorldDeltaSeconds`))))
  (if (>= _output_get (`KismetMathLibrary.FClamp` (`self.InvisibilityTransitionTime`) 0.0 (`self.InvisibilityDuration`)))
    (`MaterialInstanceDynamic.SetScalarParameterValue` (`self.Invisibility`) "Opacity" (- 1.0 (`KismetMathLibrary.Conv_BoolToDouble` (`self.bIsInvisible`))))
    (`self.OnInvisibilityTransitionEnded`)
    (`/Game/ProjectAI/Core/Game/Managers/Events/Components/AC_GameEvents.OnPlayerEndInvisibility` (`self.GameEvents`))
    (else
      (`MaterialInstanceDynamic.SetScalarParameterValue` (`self.Invisibility`) "Opacity" (`KismetMathLibrary.Abs` (- (`KismetMathLibrary.Conv_BoolToDouble` (`self.bIsInvisible`)) (/ (`self.ElapsedTime`) (`KismetMathLibrary.FClamp` (`self.InvisibilityTransitionTime`) 0.0 (`self.InvisibilityDuration`))))))
      (`KismetSystemLibrary.DelayUntilNextTick`)
      (`self.InvisibilityTransitionAnim`))))

(event `InvisibilityTransitionEnded`
  (set `self.ElapsedTime` 0.0)
  (if (`self.bIsInvisible`)
    (`self.ResetInvisibility`)
    (else
      (`PrimitiveComponent.SetMaterial` (`self.Mesh`) 0 (`self.MainMaterial`)))))

(event `ResetInvisibility`
  (`KismetSystemLibrary.RetriggerableDelay` (`self.InvisibilityDuration`))
  (`self.SetInvisibility` false))

(fn `AddInteractable`
  (params (Interactable :type "/Game/ProjectAI/Core/Game/Features/Gameplay/InteractSystem/Interfaces/BPI_Interactable Interface"))
  (`KismetArrayLibrary.Array_Add` (`self.DetectedInteractables`) Interactable)
  (`self.OnInteractableDetected` Interactable))

(fn `CacheGameEvents`
  (bind (_bsuccess _gameevents) (`/Game/ProjectAI/Core/Game/Managers/Events/Utility/BFL_GameEventsUtility.TryGetGameEvents`))
  (if _bsuccess
    (set `self.GameEvents` _gameevents)))

(fn `CacheGameMode`
  (bind _asgm_paigameplay (cast `/Game/ProjectAI/Core/Game/UGameFramework/GameModes/GM_PAIGameplay` (`GameplayStatics.GetGameMode`)))
  (set `self.GameMode` _asgm_paigameplay))

(fn `CacheHUD`
  (bind _asbp_paigameplay_hud (cast `/Game/ProjectAI/Core/Game/UGameFramework/HUD/BP_PAIGameplayHUD` (`PlayerController.GetHUD` (`GameplayStatics.GetPlayerController` 0))))
  (set `self.HUD` _asbp_paigameplay_hud))

(fn `CachePlayerController`
  (bind _asbp_gameplay_player_controller (cast `/Game/ProjectAI/Core/Game/UGameFramework/Controllers/BP_GameplayPlayerController` (`GameplayStatics.GetPlayerController` 0)))
  (set `self.PlayerController` _asbp_gameplay_player_controller))

(fn `CanBeHighlighted`
  (returns (Result :type Boolean))
  (return (not (`self.IsPossessed`))))

(fn `CanSensePlayer`
  (returns (bCanSense :type Boolean))
  (return (and (`self.IsPossessed`) (not (`self.bIsInvisible`)))))

(fn `ClearInvisibilityTimer`
  (`KismetSystemLibrary.K2_ClearAndInvalidateTimerHandle` (`self.InvisibilityTimer`)))

(fn `GetMainTexture`
  (returns (Texture :type "Texture Object Reference"))
  (bind _returnvalue (`PrimitiveComponent.CreateDynamicMaterialInstance` (`self.Mesh`) 0 (`PrimitiveComponent.GetMaterial` (`self.Mesh`) 0) "None"))
  (bind _returnvalue_2 (`MaterialInstanceDynamic.K2_GetTextureParameterValue` _returnvalue "Texture"))
  (return _returnvalue_2))

(fn `GetNearestEntity`
  (params (Entities :type "Array of /Game/ProjectAI/Core/Game/Features/Player/Base/BP_EntityBase Object Reference"))
  (returns (Nearest :type "/Game/ProjectAI/Core/Game/Features/Player/Base/BP_EntityBase Object Reference"))
  (locals (NearestDistance :type "Float (double-precision)") (NearestEntity :type "/Game/ProjectAI/Core/Game/Features/Player/Base/BP_EntityBase Object Reference"))
  (if (> (`KismetArrayLibrary.Array_Length` Entities) 0)
    (bind _output_get (set `local.NearestEntity` (`|GetArrayItem` Entities)))
    (set `local.NearestDistance` (`self.GetDistanceTo` _output_get self))
    (for _array_element Entities
      (bind _returnvalue (`self.GetDistanceTo` _array_element self))
      (if (< _returnvalue (`local.NearestDistance`))
        (set `local.NearestEntity` _array_element)
        (set `local.NearestDistance` _returnvalue)))
    (return (`local.NearestEntity`))
    (else
      (return (`local.NearestEntity`)))))

(fn `GetNearestInteractable`
  (returns (Nearest :type "/Game/ProjectAI/Core/Game/Features/Gameplay/InteractSystem/Interfaces/BPI_Interactable Interface"))
  (locals (NearestInteractable :type "/Game/ProjectAI/Core/Game/Features/Gameplay/InteractSystem/Interfaces/BPI_Interactable Interface") (NearestDistance :type "Float (double-precision)" :default 10000.0) (Uninteractables :type "Array of Integer"))
  (for _array_element (`self.DetectedInteractables`)
    (bind _returnvalue (`self.GetDistanceTo` (cast `Actor` (`KismetSystemLibrary.Conv_InterfaceToObject` _array_element) :!pure true) self))
    (if (< _returnvalue (`local.NearestDistance`))
      (set `local.NearestInteractable` _array_element)
      (set `local.NearestDistance` _returnvalue)))
  (return (`local.NearestInteractable`)))

(fn `InitInvisibility`
  (set `self.MainMaterial` (`PrimitiveComponent.GetMaterial` (`self.Mesh`) 0))
  (bind _returnvalue (`PrimitiveComponent.CreateDynamicMaterialInstance` (`self.Mesh`) 0 "/Game/ProjectAI/MaterialLibrary/M_Invisibility.M_Invisibility" "None"))
  (set `self.Invisibility` _returnvalue)
  (`MaterialInstanceDynamic.SetTextureParameterValue` (`self.Invisibility`) "Texture" (`self.GetMainTexture`))
  (`PrimitiveComponent.SetMaterial` (`self.Mesh`) 0 (`self.MainMaterial`))
  (add `self.OnInvisibilityTransitionEnded` (`|CreateDelegate` :!event `InvisibilityTransitionEnded`)))

(fn `Look`
  (params (LookInput :type "Vector2D Structure"))
  (`self.AddControllerYawInput` LookInput_X)
  (`self.AddControllerPitchInput` LookInput_Y))

(fn `LookForInteraction`
  (bind _nearest (`self.GetNearestInteractable`))
  (if (`KismetArrayLibrary.Array_IsNotEmpty` (`self.DetectedInteractables`))
    (bind _return (`/Game/ProjectAI/Core/Game/Features/Gameplay/InteractSystem/Interfaces/BPI_Interactable.CanBeInteracted` _nearest))
    (if _return
      (bind (_location _text _inputaction) (`/Game/ProjectAI/Core/Game/Features/Gameplay/InteractSystem/Interfaces/BPI_Interactable.GetHUDInteractionInfo` _nearest))
      (`/Game/ProjectAI/Core/Game/UGameFramework/HUD/BP_PAIGameplayHUD.ShowInteraction` (`self.HUD`) _location _text _inputaction)
      (set `self.InteractionVisible` true)
      (else
        (if (`self.InteractionVisible`) :!label _label
          (`/Game/ProjectAI/Core/Game/UGameFramework/HUD/BP_PAIGameplayHUD.HideInteraction` (`self.HUD`))
          (set `self.InteractionVisible` false))))
    (else
      (goto _label))))

(fn `Move`
  (params (MoveInput :type "Vector Structure"))
  (bind (_returnvalue_roll _returnvalue_pitch _returnvalue_yaw) (`KismetMathLibrary.BreakRotator` (`self.GetControlRotation`)))
  (`self.AddMovementInput` (`KismetMathLibrary.GreaterGreater_VectorRotator` MoveInput (`KismetMathLibrary.MakeRotator` _returnvalue_roll 0.0 _returnvalue_yaw))))

(fn `PlayHealingEffects`
  (bind _returnvalue (`self.K2_GetActorLocation`))
  (`NiagaraFunctionLibrary.SpawnSystemAtLocation` "/Game/ProjectAI/Art/3D/Vfx/VFX_Healing_01_a.VFX_Healing_01_a" _returnvalue (struct) (1.0 1.0 1.0) true true "AutoRelease")
  (`GameplayStatics.PlaySoundAtLocation` "/Game/ProjectAI/Audio/Sounds/Healing_Sound.Healing_Sound" _returnvalue (struct) 1.0 1.0 0.0 "/Game/ProjectAI/Audio/Attenuations/SA_Healing.SA_Healing" null null null))

(fn `RemoveInteractable`
  (params (Interactable :type "/Game/ProjectAI/Core/Game/Features/Gameplay/InteractSystem/Interfaces/BPI_Interactable Interface (by ref)"))
  (bind _returnvalue (`KismetArrayLibrary.Array_RemoveItem` (`self.DetectedInteractables`) Interactable))
  (if _returnvalue
    (`self.OnInteractableUndetected` Interactable)))

(fn `SetHealthVFX`
  (params (Health :type "Float (double-precision)"))
  (`KismetMaterialLibrary.SetScalarParameterValue` "/Game/ProjectAI/MaterialLibrary/ScreenDamageEffect/MPC_ScreenDamage.MPC_ScreenDamage" "LostHealthPercentage" (- 1.0 (/ Health (`/Game/ProjectAI/Core/Game/Features/Gameplay/HealthSystem/Components/AC_HealthManager.GetMaxHealth` (`self.AC_HealthManager`))))))

(fn `SetInvisibility`
  (params (Invisible :type Boolean))
  (`/Game/ProjectAI/Core/Game/Managers/Events/Components/AC_GameEvents.OnPlayerStartInvisibility` (`self.GameEvents`))
  (bind _output_get (set `self.bIsInvisible` Invisible))
  (if _output_get
    (`PrimitiveComponent.SetMaterial` (`self.Mesh`) 0 (`self.Invisibility`))
    (`self.InvisibilityTransitionAnim`)
    (else
      (`self.InvisibilityTransitionAnim`))))

(fn `UserConstructionScript`)