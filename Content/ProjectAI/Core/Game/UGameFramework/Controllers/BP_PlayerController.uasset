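; Player controller for ProjectAI that sets up gameplay input and owns the in-game menu.
; On BeginPlay it registers and applies the gameplay mapping context, then creates the hidden menu widget when the game mode is GM_PAIGameplay.
; Toggling the menu swaps Enhanced Input contexts, input mode and mouse cursor, and input actions page through it.
; A debug X key spawns the wheel item selector widget.
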(event EventBeginPlay
  (Utilities|FlowControl|Sequence
    (:then_0
      (CallFunction|SwitchMappingContext 0 "/Game/ProjectAI/Core/Game/Inputs/IMC_GameplayInputs.IMC_GameplayInputs")
      (Actor|Tick|SetActorTickEnabled (Game|Player|GetPlayerPawn 0) true)
      (bind _output_get (Variables|Default|SetInputUserSetting (Class|EnhancedInputSubsystemInterface|GetUserSettings (PlayerController|LocalPlayerSubsystems|GetEnhancedInputLocalPlayerSubsystem))))
      (if (not (Class|EnhancedInputUserSettings|IsMappingContextRegistered _output_get "/Game/ProjectAI/Core/Game/Inputs/IMC_GameplayInputs.IMC_GameplayInputs"))
        (Class|EnhancedInputUserSettings|RegisterInputMappingContext _output_get "/Game/ProjectAI/Core/Game/Inputs/IMC_GameplayInputs.IMC_GameplayInputs")))
    (:then_1
      (Utilities|Casting|CastToGM_PAIGameplay (Game|GetGameMode))
      (CallFunction|InitUI))))

(event Custom|InitUI
  (bind _returnvalue (Game|ConstructObjectfromClass "/Game/ProjectAI/Core/Game/Features/UI/Widgets/Menus/GameplayMenu/WBP_GameplayMenu.WBP_GameplayMenu_C"))
  (bind _output_get (Variables|Default|SetUIGameMenu _returnvalue))
  (UserInterface|Viewport|AddtoViewport _output_get (Variables|Default|GetZOrderGameMenu))
  (CallFunction|HideGameMenu))

(event Input|EnhancedActionEvents|EnhancedInputActionIA_ToggleGameMenu
  (params (ActionValue :type Boolean) (ElapsedSeconds :type Float%20%28double-precision%29) (TriggeredSeconds :type Float%20%28double-precision%29) (InputAction :type Input%20Action%20Object%20Reference :default "/Game/ProjectAI/Core/Game/Inputs/Actions/IA_ToggleGameMenu.IA_ToggleGameMenu"))
  (Utilities|Casting|CastToGM_PAIGameplay (Game|GetGameMode))
  (CallFunction|ToggleGameMenu))

(event Input|EnhancedActionEvents|EnhancedInputActionIA_NextMenuPage
  (params (ActionValue :type Boolean) (ElapsedSeconds :type Float%20%28double-precision%29) (TriggeredSeconds :type Float%20%28double-precision%29) (InputAction :type Input%20Action%20Object%20Reference :default "/Game/ProjectAI/Core/Game/Inputs/UIActions/IA_NextMenuPage.IA_NextMenuPage"))
  (Default|NextMenuPage (Variables|Default|GetUIGameMenu)))

(event Input|EnhancedActionEvents|EnhancedInputActionIA_PreviousMenuPage
  (params (ActionValue :type Boolean) (ElapsedSeconds :type Float%20%28double-precision%29) (TriggeredSeconds :type Float%20%28double-precision%29) (InputAction :type Input%20Action%20Object%20Reference :default "/Game/ProjectAI/Core/Game/Inputs/UIActions/IA_PreviousMenuPage.IA_PreviousMenuPage"))
  (Default|PreviousMenuPage (Variables|Default|GetUIGameMenu)))

(event Input|KeyboardEvents|DebugKeyX
  (params (Key :type Key%20Structure :default "None") (ActionValue :type Input%20Action%20Value%20Structure))
  (:Pressed
    (bind _returnvalue (Game|ConstructObjectfromClass "/Game/ProjectAI/Core/Game/Features/UI/Widgets/Systems/InventorySystem/Selector/WBP_WheelItemSelector.WBP_WheelItemSelector_C"))
    (UserInterface|Viewport|AddtoViewport _returnvalue 0)))

(fn ConstructionScript)

(fn ShowGameMenu
  (bind _uigamemenu (Variables|Default|GetUIGameMenu))
  (Widget|SetVisibility _uigamemenu "Visible")
  (Default|OnShowMenu _uigamemenu)
  (CallFunction|SwitchMappingContext "/Game/ProjectAI/Core/Game/Inputs/IMC_GameplayInputs.IMC_GameplayInputs" "/Game/ProjectAI/Core/Game/Inputs/IMC_MenuInputs.IMC_MenuInputs")
  (Input|SetInputModeGameandUI self (Variables|Default|GetUIGameMenu) "DoNotLock" true false)
  (Variables|Default|SetbShowMouseCursor true))

(fn HideGameMenu
  (Widget|SetVisibility (Variables|Default|GetUIGameMenu) "Collapsed")
  (CallFunction|SwitchMappingContext "/Game/ProjectAI/Core/Game/Inputs/IMC_MenuInputs.IMC_MenuInputs" "/Game/ProjectAI/Core/Game/Inputs/IMC_GameplayInputs.IMC_GameplayInputs")
  (Input|SetInputModeGameOnly self true)
  (Variables|Default|SetbShowMouseCursor false))

(fn ToggleGameMenu
  (if (Widget|IsVisible (Variables|Default|GetUIGameMenu))
    (CallFunction|HideGameMenu)
    (Default|CallOnHideGameMenu)
    (else
      (CallFunction|ShowGameMenu)
      (Default|CallOnShowGameMenu))))

(fn SwitchMappingContext
  (params (From :type Input%20Mapping%20Context%20Object%20Reference) (To :type Input%20Mapping%20Context%20Object%20Reference))
  (bind _returnvalue (PlayerController|LocalPlayerSubsystems|GetEnhancedInputLocalPlayerSubsystem))
  (Input|RemoveMappingContext _returnvalue From "(bIgnoreAllPressedKeysUntilRelease=True,bForceImmediately=False,bNotifyUserSettings=False)")
  (Input|AddMappingContext _returnvalue To 0 "(bIgnoreAllPressedKeysUntilRelease=True,bForceImmediately=False,bNotifyUserSettings=False)"))