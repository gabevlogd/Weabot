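; Door actor that toggles its open/close animation when enough Activate calls arrive, and again when a Deactivate drops the count below that maximum.
; A clamped trigger counter drives a dynamic feedback material that pans with progress and turns from red to green when full.
; Each toggle sets the skeletal animation's play rate from Speed, plays a sound, and first nudges listed actor classes overlapping the collider out of the doorway.
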(event `self.ReceiveBeginPlay`
  ;[0 0 0] Unreal Events
  (`self.SetInitialDoorState`)
  (`self.UpdateActivationTrigger`))

(event `/Game/ProjectAI/Core/Game/Features/Gameplay/InteractSystem/Interfaces/BPI_Activable.Activate`
  ;[0 0 0] Door Trigger
  (bind _triggerdoormovement (`self.IncrementTriggerCounter` 1 (`self.MaxTriggersCount`)))
  (`self.UpdateActivationTrigger`)
  (if _triggerdoormovement
    (`self.TriggerAnimation`)))

(event `/Game/ProjectAI/Core/Game/Features/Gameplay/InteractSystem/Interfaces/BPI_Activable.Deactivate`
  ;[0 0 0] Door Trigger
  (bind _triggerdoormovement (`self.IncrementTriggerCounter` -1 (- (`self.MaxTriggersCount`) 1)))
  (`self.UpdateActivationTrigger`)
  (if _triggerdoormovement
    (`self.TriggerAnimation`)))

(event `self.Collider.OnComponentBeginOverlap`
  (params (OverlappedComponent :type "PrimitiveComponent Object Reference") (OtherActor :type "Actor Object Reference") (OtherComp :type "PrimitiveComponent Object Reference") (OtherBodyIndex :type Integer) (bFromSweep :type Boolean) (SweepResult :type "HitResult Structure (by ref)"))
  ;[0 0 0] Checks actors in between door
  (if (`KismetArrayLibrary.Array_Contains` (`self.MustBeMoved`) (`GameplayStatics.GetObjectClass` OtherActor))
    (`KismetArrayLibrary.Array_Add` (`self.ActorsToMove`) OtherActor)))

(event `self.Collider.OnComponentEndOverlap`
  (params (OverlappedComponent :type "PrimitiveComponent Object Reference") (OtherActor :type "Actor Object Reference") (OtherComp :type "PrimitiveComponent Object Reference") (OtherBodyIndex :type Integer))
  ;[0 0 0] Checks actors in between door
  (if (`KismetArrayLibrary.Array_Contains` (`self.MustBeMoved`) (`GameplayStatics.GetObjectClass` OtherActor))
    (`KismetArrayLibrary.Array_RemoveItem` (`self.ActorsToMove`) OtherActor)))

(fn `IncrementTriggerCounter`
  (params (CounterIncrement :type Integer) (TriggerValue :type Integer))
  (returns (TriggerDoorMovement :type Boolean))
  (bind _output_get (set `self.CurrentTriggersCount` (`KismetMathLibrary.Clamp` (+ (`self.CurrentTriggersCount`) CounterIncrement) 0 (`self.MaxTriggersCount`))))
  (return (== _output_get TriggerValue)))

(fn `MoveActorsInBetween`
  (for _array_element (`self.ActorsToMove`)
    (bind _returnvalue_x (`KismetMathLibrary.BreakVector` (`KismetMathLibrary.InverseTransformLocation` (`self.GetTransform`) (`self.K2_GetActorLocation` _array_element))))
    (`self.K2_AddActorWorldOffset` _array_element (* (`self.GetActorForwardVector`) 100.0 (`KismetMathLibrary.SignOfFloat` _returnvalue_x)) false false))
  (return))

(fn `SetInitialDoorState`
  (if (`|EnumEquality` (`self.InitialState`) "NewEnumerator0")
    (`SkeletalMeshComponent.SetPosition` (`self.Mesh_Door_01_b_Open`) (`AnimSequenceBase.SequenceLength` (`self.DoorAnimationSequence`)) true)
    (set `self.Speed` (`KismetMathLibrary.Abs` (`self.Speed`)))
    (else
      (`SkeletalMeshComponent.SetPosition` (`self.Mesh_Door_01_b_Open`) 0.0 true)
      (set `self.Speed` (* (`KismetMathLibrary.Abs` (`self.Speed`)) -1.0)))))

(fn `TriggerAnimation`
  (locals (Sound :type "SoundBase Object Reference"))
  (bind _mesh_door_01_b_open (`self.Mesh_Door_01_b_Open`))
  (`self.MoveActorsInBetween`)
  (bind _result (`/Engine/EditorBlueprintResources/StandardMacros.NegateFloat` (`self.Speed`))
    (:`  `
      (`SkeletalMeshComponent.SetPlayRate` (`self.Mesh_Door_01_b_Open`) _result)
      (`|ExecutionSequence`
        (:`then_0`
          (if (`SkeletalMeshComponent.IsPlaying` (`self.Mesh_Door_01_b_Open`))
            (`SkeletalMeshComponent.SetPosition` (`self.Mesh_Door_01_b_Open`) (`SkeletalMeshComponent.GetPosition` (`self.Mesh_Door_01_b_Open`)) true)
            (elif (> (`self.Speed`) 0.0)
              (`SkeletalMeshComponent.SetPosition` (`self.Mesh_Door_01_b_Open`) 0.0 true)
              (else
                (`SkeletalMeshComponent.SetPosition` (`self.Mesh_Door_01_b_Open`) (`AnimSequenceBase.SequenceLength` (`self.DoorAnimationSequence`)) true)))))
        (:`then_1`
          (`SkeletalMeshComponent.Play` _mesh_door_01_b_open false)
          (if (> (`SkeletalMeshComponent.GetPlayRate` _mesh_door_01_b_open) 0.0)
            (set `local.Sound` (`self.OpenSound`))
            (else
              (set `local.Sound` (`self.CloseSound`))))
          (`GameplayStatics.PlaySound2D` (`local.Sound`) 1.0 1.0 0.0 null null))))))

(fn `UpdateActivationTrigger`
  (bind _returnvalue (/ (`KismetMathLibrary.Conv_IntToDouble` (`self.CurrentTriggersCount`)) (`KismetMathLibrary.Conv_IntToDouble` (`self.MaxTriggersCount`))))
  (`MaterialInstanceDynamic.SetScalarParameterValue` (`self.ActivationFeedbackMaterial`) "U Pan" _returnvalue)
  (if (== _returnvalue 1.0)
    (`MaterialInstanceDynamic.SetVectorParameterValue` (`self.ActivationFeedbackMaterial`) "EmissiveColor" (struct :`G` 1.0 :`A` 1.0))
    (else
      (`MaterialInstanceDynamic.SetVectorParameterValue` (`self.ActivationFeedbackMaterial`) "EmissiveColor" (struct :`R` 1.0 :`A` 1.0)))))

(fn `UserConstructionScript`
  (bind _activationfeedback (`self.ActivationFeedback`))
  (if (`self.UseConstructionScript`)
    (bind _returnvalue (`PrimitiveComponent.CreateDynamicMaterialInstance` _activationfeedback 0 (`PrimitiveComponent.GetMaterial` _activationfeedback 0) "None"))
    (bind _output_get (set `self.ActivationFeedbackMaterial` _returnvalue))
    (`MaterialInstanceDynamic.SetScalarParameterValue` _output_get "TriggerCount" (`KismetMathLibrary.Conv_IntToDouble` (`self.MaxTriggersCount`)))))