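; AC_MovementSound is an actor component that plays a sound on its owning Character that varies with movement speed.
; On BeginPlay it adds an audio component to the owner, assigns the configured sound and attenuation, and starts playback at idle pitch.
; Every Tick it lerps pitch and volume between idle and moving values, using velocity length divided by the Character's MaxWalkSpeed as the alpha.
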(event `self.ReceiveBeginPlay`
  (bind _ascharacter (cast `Character` (`self.GetOwner`)))
  (bind _output_get (set `self.Owner` _ascharacter))
  ;[0 0 0] SetUp Audio Component
  (bind _returnvalue (`|AddComponentByClass` :`self` _output_get :`Class` "/Script/Engine.AudioComponent"))
  (bind _output_get_2 (set `self.AudioSource` _returnvalue))
  (`AudioComponent.SetSound` _output_get_2 (`self.Sound`))
  (set `AudioComponent.AttenuationSettings` (`self.Attenuation Settings`) (`self.AudioSource`))
  (`AudioComponent.SetPitchMultiplier` (`self.AudioSource`) (`self.IdlePitch`))
  (`AudioComponent.Play` (`self.AudioSource`) 0.0))

(event `self.ReceiveTick`
  (params (DeltaSeconds :type "Float (single-precision)"))
  (bind _returnvalue (/ (`KismetMathLibrary.VSize` (`Actor.GetVelocity` (`self.Owner`))) (`CharacterMovementComponent.MaxWalkSpeed` (`Character.CharacterMovement` (`self.Owner`)))))
  ;[0 0 0] Perform Movement Audio
  (`AudioComponent.SetPitchMultiplier` (`self.AudioSource`) (`KismetMathLibrary.Lerp` (`self.IdlePitch`) (`self.MovingPitch`) _returnvalue))
  (`AudioComponent.SetVolumeMultiplier` (`self.AudioSource`) (`KismetMathLibrary.Lerp` (`self.IdleVolume`) (`self.MovingVolume`) _returnvalue)))