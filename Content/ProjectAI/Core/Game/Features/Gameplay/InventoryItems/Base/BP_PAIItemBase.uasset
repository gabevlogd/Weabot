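; BP_PAIItemBase is the base Blueprint for inventory items, handling what happens when an item is selected, removed or used.
; For throwable items, selection passes the item's PhysicalItem to the ACThrower component on the player's BP_EntityCatcher pawn, and removal clears it.
; UseSelf has an empty implementation.
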(event `UseSelf`)

(event `OnSelect`
  (if (`self.bThrowable`)
    (bind _asbp_entity_catcher (cast `/Game/ProjectAI/Core/Game/Features/Player/CaptureSystem/BP_EntityCatcher` (`Controller.K2_GetPawn` (`self.GetPlayerController` 0))))
    (`/Game/ProjectAI/Core/Game/Features/Gameplay/ThrowingSystem/AC_Thrower.SetActorToThrow` (`/Game/ProjectAI/Core/Game/Features/Player/CaptureSystem/BP_EntityCatcher.AC_Thrower` _asbp_entity_catcher) (`self.PhysicalItem`))))

(event `self.OnRemove`
  (if (`self.bThrowable`)
    (bind _asbp_entity_catcher (cast `/Game/ProjectAI/Core/Game/Features/Player/CaptureSystem/BP_EntityCatcher` (`Controller.K2_GetPawn` (`self.GetPlayerController` 0))))
    (`/Game/ProjectAI/Core/Game/Features/Gameplay/ThrowingSystem/AC_Thrower.SetActorToThrow` (`/Game/ProjectAI/Core/Game/Features/Player/CaptureSystem/BP_EntityCatcher.AC_Thrower` _asbp_entity_catcher) null)))