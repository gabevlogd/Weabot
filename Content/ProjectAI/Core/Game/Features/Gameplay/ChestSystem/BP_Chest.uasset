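; BP_Chest is an interactable, highlightable loot chest that opens once and grants its reward items to the player's inventory.
; Interacting plays the open animation and sound, then adds RewardData through the game mode's PlayerInventorySystem after a delay derived from animation length.
; The Saver stores the opened state by unique ID, and loading restores it by snapping an opened chest to the animation's final frame.
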(event `self.ReceiveBeginPlay`
  ;[0 0 0] Initialize chest
  (`self.Load`)
  (`|ExecutionSequence`
    (:`then_0`
      (bind _asgm_paigameplay (cast `/Game/ProjectAI/Core/Game/UGameFramework/GameModes/GM_PAIGameplay` (`GameplayStatics.GetGameMode`)))
      (set `self.Player Inventory System` (`/Game/ProjectAI/Core/_Debug/Code/Code_b/GM_DebugGamemode_1a.PlayerInventorySystem` _asgm_paigameplay)))
    (:`then_1`
      (`SkeletalMeshComponent.SetAnimation` (`self.SkeletalMesh`) (`self.OpenAnimation`))
      (`SkeletalMeshComponent.SetPlayRate` (`self.SkeletalMesh`) 10.0))))

(event `/Game/ProjectAI/Core/Game/Features/Gameplay/InteractSystem/Interfaces/BPI_Interactable.EnableInteract`
  ;[0 0 0] Trigger chest opening
  (if (not (`self.Opened`))
    (set `self.Opened` true)
    (`SkeletalMeshComponent.Play` (`self.SkeletalMesh`) false)
    (`GameplayStatics.PlaySound2D` (`self.OpenSound`) 1.0 1.0 0.0 null null)
    (`KismetSystemLibrary.Delay` (/ (`AnimSequenceBase.SequenceLength` (`self.OpenAnimation`)) (`SkeletalMeshComponent.GetPlayRate` (`self.SkeletalMesh`))))
    (`self.AddRewardToInventory`)))

(event `self.Saver.OnPrepSave`
  (params (SaveGameData :type "DefaultSaveGame Object Reference") (SlotInfoItem :type "SlotInfoItem Object Reference") (Instigator :type "Object Object Reference"))
  ;[0 0 0] Save data
  (bind _asbp_paisave_game (cast `/Game/ProjectAI/Core/Game/Data/SaveSystemData/BP_PAISaveGame` SaveGameData))
  (`BlueprintMapLibrary.Map_Add` (`/Game/ProjectAI/Core/Game/Data/SaveSystemData/BP_PAISaveGame.Chests` _asbp_paisave_game) (`Saver.GetUniqueSaveID` (`self.Saver`)) (make `/Game/ProjectAI/Core/Game/Features/Gameplay/ChestSystem/Data/S_ChestSaveData` (`self.Opened`))))

(event `Load`
  ;[0 0 0] Save data
  (`|ExecutionSequence`
    (:`then_0`
      (bind _asbp_paisave_game (cast `/Game/ProjectAI/Core/Game/Data/SaveSystemData/BP_PAISaveGame` (`SSUtility.GetSaveGame`)))
      (bind (_value _returnvalue) (`BlueprintMapLibrary.Map_Find` (`/Game/ProjectAI/Core/Game/Data/SaveSystemData/BP_PAISaveGame.Chests` _asbp_paisave_game) (`Saver.GetUniqueSaveID` (`self.Saver`))))
      (if _returnvalue
        (set `self.Opened` (break `/Game/ProjectAI/Core/Game/Features/Gameplay/ChestSystem/Data/S_ChestSaveData` _value))))
    (:`then_1`
      (`self.SetInitialState`))))

(event `/Game/ProjectAI/Core/Game/Features/Gameplay/HighlightingSystem/BPI_Highlightable.StopHighlight`
  (`PrimitiveComponent.SetRenderCustomDepth` (`self.SkeletalMesh`) false))

(event `/Game/ProjectAI/Core/Game/Features/Gameplay/HighlightingSystem/BPI_Highlightable.StartHighlight`
  (`PrimitiveComponent.SetRenderCustomDepth` (`self.SkeletalMesh`) true))

(event `self.Saver.OnLoadGameCompleted`
  (params (SlotName :type String) (UserIndex :type Integer) (SaveGameData :type "DefaultSaveGame Object Reference") (Instigator :type "Object Object Reference"))
  (`self.Load`))

(fn `AddRewardToInventory`
  (for _array_element (`self.RewardData`)
    (`/Engine/EditorBlueprintResources/StandardMacros.IsValid` _array_element
      (:`Is Valid`
        (`InventorySystem.AddItem` (`self.Player Inventory System`) _array_element)))))

(fn `CanBeHighlighted`
  (returns (Result :type Boolean))
  (return (not (`self.Opened`))))

(fn `CanBeInteracted`
  (returns (Return :type Boolean))
  (return (not (`self.Opened`))))

(fn `GetHUDInteractionInfo`
  (returns (Location :type "Vector Structure") (Text :type Text) (InputAction :type "InputAction Object Reference"))
  (return (+ (`SceneComponent.K2_GetComponentLocation` (`self.Top`)) (0.0 0.0 50.0)) "Open" "/Game/ProjectAI/Core/Game/Inputs/Actions/IA_Interact.IA_Interact"))

(fn `SetInitialState`
  (if (`self.Opened`)
    (`SkeletalMeshComponent.SetPosition` (`self.SkeletalMesh`) (`AnimSequenceBase.SequenceLength` (`self.OpenAnimation`)) false)))

(fn `UserConstructionScript`)