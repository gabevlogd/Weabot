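; Base AI controller for entities that runs a given behavior tree and tracks possessed entities as targets.
; Perception updates select a possessed entity as target; Tick keeps it while possessed and sensed by sight, otherwise clears it and searches currently seen actors.
; Target enter, process and exit calls report these changes.
; State and disabled setters write to the Blackboard using key names looked up in a DataTable.
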(event `Init`
  (params (Behaviour :type "BehaviorTree Object Reference"))
  ;[1 0 0] Initialization
  (`self.RunBehaviour` Behaviour))

(event `self.AIPerception.OnPerceptionUpdated`
  (params (UpdatedActors :type "Array of Actor Object Reference (by ref)"))
  (`self.FindTarget` UpdatedActors))

(event `self.ReceiveTick`
  (params (DeltaSeconds :type "Float (single-precision)"))
  (bind _targetactor (`self.TargetActor`)
    (:`then`
      (bind (_stimulus _bissensed) (`self.Can Sense Actor` _targetactor "NewEnumerator1"))
      (bind _bispossessed (`/Game/ProjectAI/Core/Game/Features/Player/Interfaces/BPI_Player.GetIsPossessed` (`self.TargetActor`)))
      (if (and _bispossessed _bissensed)
        (`self.OnTargetProcess` (`self.TargetActor`))
        (else
          (`self.OnTargetExit` (`self.TargetActor`))
          (set `self.TargetActor` null) ; Clear Target
          ;[0 0 0] Try find a new target
          (`self.FindTarget` (`AIPerceptionComponent.GetCurrentlyPerceivedActors` (`self.AIPerception`) "/Script/AIModule.AISense_Sight")))))
    (:`else`)))

(fn `Can Sense Actor`
  (params (Actor :type "Actor Object Reference") (Sense :type "/Game/ProjectAI/Core/Game/Features/AI/Data/Enums/E_EntitySense Enum" :default "NewEnumerator0"))
  (returns (Stimulus :type "AIStimulus Structure") (bIsSensed :type Boolean))
  (bind _info (`AIPerceptionComponent.GetActorsPerception` (`self.AIPerception`) Actor))
  (for _array_element (`.LastSensedStimuli` (break `ActorPerceptionBlueprintInfo` _info))
    (bind _returnvalue (`AIPerceptionSystem.GetSenseClassForStimulus` _array_element))
    (if (== _returnvalue (select `/Game/ProjectAI/Core/Game/Features/AI/Data/Enums/E_EntitySense` Sense :`NewEnumerator1` "/Script/AIModule.AISense_Sight" :`NewEnumerator2` "/Script/AIModule.AISense_Hearing" :`NewEnumerator3` "/Script/AIModule.AISense_Damage" :!type "Object Class Reference"))
      (return _array_element (`.bSuccessfullySensed` (break `AIStimulus` _array_element))))))

(fn `FindTarget`
  (params (Array :type "Array of Actor Object Reference"))
  (for _array_element Array
    (bind _asbp_entity_base (cast `/Game/ProjectAI/Core/Game/Features/Player/Base/BP_EntityBase` _array_element))
    (bind _bispossessed (`/Game/ProjectAI/Core/Game/Features/Player/Interfaces/BPI_Player.GetIsPossessed` _asbp_entity_base))
    (if _bispossessed
      (set `self.TargetActor` _asbp_entity_base)
      (`self.OnTargetEnter` (`self.TargetActor`)))))

(fn `GetState`
  (returns (CurrentState :type "/Game/ProjectAI/Core/Game/Features/AI/Data/Enums/E_EntityState Enum"))
  (return (`self.CurrentState`)))

(fn `IsState`
  (params (State :type "/Game/ProjectAI/Core/Game/Features/AI/Data/Enums/E_EntityState Enum" :default "NewEnumerator0"))
  (returns (bIsState :type Boolean))
  (return (`|EnumEquality` State (`self.CurrentState`))))

(fn `RunBehaviour`
  (params (Behaviour :type "BehaviorTree Object Reference"))
  (bind _returnvalue (`self.RunBehaviorTree` Behaviour))
  (if (not _returnvalue)
    (`self.PrintBehaviourError`)))

(fn `SetIsDisabled`
  (params (bIsDisabled :type Boolean))
  (bind _returnvalue (`|GetDataTableRow` "/Game/ProjectAI/Core/Game/Features/AI/Data/Tables/DT_BBKeys.DT_BBKeys" "IsDisabled")
    (:`then`
      (`BlackboardComponent.SetValueAsBool` (`self.Blackboard`) (break `/Game/ProjectAI/Core/Game/Features/AI/Data/Structs/S_BBKey` _returnvalue) bIsDisabled)
      (set `self.bIsDisabled` bIsDisabled))))

(fn `SetState`
  (params (State :type "/Game/ProjectAI/Core/Game/Features/AI/Data/Enums/E_EntityState Enum" :default "NewEnumerator0"))
  (bind _returnvalue (`|GetDataTableRow` "/Game/ProjectAI/Core/Game/Features/AI/Data/Tables/DT_BBKeys.DT_BBKeys" "State")
    (:`then`
      (bind _output_get (set `self.CurrentState` State))
      (`BlackboardComponent.SetValueAsEnum` (`self.Blackboard`) (break `/Game/ProjectAI/Core/Game/Features/AI/Data/Structs/S_BBKey` _returnvalue) _output_get))))

(fn `UserConstructionScript`)