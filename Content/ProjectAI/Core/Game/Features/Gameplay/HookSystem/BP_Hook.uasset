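; BP_Hook is a grabbing hook, parented to a BP_EntityBase, that attaches to and releases objects.
; It initializes a grabber component with its grab bounds, then primary interact grabs and secondary interact ungrabs through it.
; A successful grab calls OnAttach, while any ungrab attempt calls OnDetach.
; Grabber availability events toggle a HUD prompt for possessed entities, placed at the grab point with a camera-relative offset.
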(event `self.ReceiveBeginPlay`
  (`self.Init`))

(event `Init`
  ;[1 0 0] Initialization
  (`/Game/ProjectAI/Core/Game/Features/Gameplay/HookSystem/Components/AC_HookGrabber.Init` (`self.AC_Grabber`) (`self.GrabBounds`)))

(event `/Game/ProjectAI/Core/Game/Features/Gameplay/InteractSystem/Interfaces/BPI_Interactable.PrimaryInteract`
  ;[1 0 0] Events
  (`self.TryGrab`))

(event `/Game/ProjectAI/Core/Game/Features/Gameplay/InteractSystem/Interfaces/BPI_Interactable.SecondaryInteract`
  ;[1 0 0] Events
  (`self.TryUngrab`))

(event `self.AC_Grabber.OnCanBeGrabbed`
  (`self.ShowGrabInteraction`)
  (set `self.HUDHidden` false))

(event `self.AC_Grabber.OnCantBeGrabbed`
  (if (not (`self.HUDHidden`))
    (`self.HideGrabInteraction`)
    (set `self.HUDHidden` true)))

(fn `HideGrabInteraction`
  (bind _asbp_entity_base (cast `/Game/ProjectAI/Core/Game/Features/Player/Base/BP_EntityBase` (`self.GetParentActor`)))
  (if (`/Game/ProjectAI/Core/Game/Features/Player/Base/BP_EntityBase.IsPossessed` _asbp_entity_base)
    (`/Game/ProjectAI/Core/Game/UGameFramework/HUD/BP_PAIGameplayHUD.HideInteraction` (`/Game/ProjectAI/Core/Game/Features/Player/Base/BP_EntityBase.HUD` _asbp_entity_base))))

(fn `ShowGrabInteraction`
  (bind _returnvalue (`SceneComponent.K2_GetComponentLocation` (`self.GrabPoint`)))
  (bind _asbp_entity_base (cast `/Game/ProjectAI/Core/Game/Features/Player/Base/BP_EntityBase` (`self.GetParentActor`)))
  (if (`/Game/ProjectAI/Core/Game/Features/Player/Base/BP_EntityBase.IsPossessed` _asbp_entity_base)
    (bind _camera (`/Game/ProjectAI/Core/Game/Features/Player/Base/BP_EntityBase.Camera` _asbp_entity_base))
    (`/Game/ProjectAI/Core/Game/UGameFramework/HUD/BP_PAIGameplayHUD.ShowInteraction` (`/Game/ProjectAI/Core/Game/Features/Player/Base/BP_EntityBase.HUD` _asbp_entity_base) (+ _returnvalue (* (`KismetMathLibrary.Normal` (- (`SceneComponent.K2_GetComponentLocation` _camera) _returnvalue) 0.0) 100.0) (* (`SceneComponent.GetRightVector` _camera) 100.0)) (`self.GrabInteractionText`) "/Game/ProjectAI/Core/Game/Inputs/Actions/IA_EntityAbility_0.IA_EntityAbility_0")))

(fn `TryGrab`
  (returns (bHasGrabbed :type Boolean))
  (bind _bhasgrabbed (`/Game/ProjectAI/Core/Game/Features/Gameplay/HookSystem/Components/AC_HookGrabber.Grab` (`self.AC_Grabber`)))
  (if _bhasgrabbed
    (`self.OnAttach`)
    (`self.HideGrabInteraction`))
  (return _bhasgrabbed))

(fn `TryUngrab`
  (returns (bHasUngrabbed :type Boolean))
  (bind _bhasungrabbed (`/Game/ProjectAI/Core/Game/Features/Gameplay/HookSystem/Components/AC_HookGrabber.Ungrab` (`self.AC_Grabber`)))
  (`self.OnDetach`)
  (return _bhasungrabbed))

(fn `UserConstructionScript`
  (`parent.UserConstructionScript`))