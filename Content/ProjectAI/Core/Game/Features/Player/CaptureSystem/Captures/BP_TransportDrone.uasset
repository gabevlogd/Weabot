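; BP_TransportDrone is a player-possessable drone that carries things with a magnetic hook.
; It caches the BP_Hook child actor, and two entity ability inputs try to grab or ungrab through it; ending possession also releases.
; The hook grabber's grab and ungrab events toggle the magnet force Niagara effect and play sounds.
; Overrides make the drone itself ungrabbable, outline body and magnet on highlight, and attach merge point and health bar.
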(event `self.ReceiveBeginPlay`
  (`parent.ReceiveBeginPlay`)
  (`self.Init`))

(event `Init`
  ;[1 0 0] Initialization
  (`self.SetHook`)
  (add `/Game/ProjectAI/Core/Game/Features/Gameplay/HookSystem/Components/AC_HookGrabber.OnGrab` (`/Game/ProjectAI/Core/Game/Features/Gameplay/HookSystem/BP_Hook.AC_Grabber` (`self.HookActor`)) (`|CreateDelegate` :!event `OnGrab_Event`))
  (add `/Game/ProjectAI/Core/Game/Features/Gameplay/HookSystem/Components/AC_HookGrabber.OnUngrab` (`/Game/ProjectAI/Core/Game/Features/Gameplay/HookSystem/BP_Hook.AC_Grabber` (`self.HookActor`)) (`|CreateDelegate` :!event `OnUngrab_Event`)))

(event `EnhancedInput|/Game/ProjectAI/Core/Game/Inputs/Actions/IA_EntityAbility_0`
  (params (ActionValue :type Boolean) (ElapsedSeconds :type "Float (double-precision)") (TriggeredSeconds :type "Float (double-precision)") (InputAction :type "InputAction Object Reference" :default "/Game/ProjectAI/Core/Game/Inputs/Actions/IA_EntityAbility_0.IA_EntityAbility_0"))
  ;[1 0 0] Events
  (:`Triggered`
    (`/Game/ProjectAI/Core/Game/Features/Gameplay/HookSystem/BP_Hook.TryGrab` (`self.HookActor`))))

(event `OnGrab_Event`
  (`ActorComponent.Activate` (`self.NS_MagnetForce`) false)
  (`GameplayStatics.PlaySound2D` "/Engine/EditorSounds/GamePreview/StartSimulate.StartSimulate" 1.0 1.0 0.0 null null))

(event `EnhancedInput|/Game/ProjectAI/Core/Game/Inputs/Actions/IA_EntityAbility_1`
  (params (ActionValue :type Boolean) (ElapsedSeconds :type "Float (double-precision)") (TriggeredSeconds :type "Float (double-precision)") (InputAction :type "InputAction Object Reference" :default "/Game/ProjectAI/Core/Game/Inputs/Actions/IA_EntityAbility_1.IA_EntityAbility_1"))
  ;[1 0 0] Events
  (:`Triggered`
    (`/Game/ProjectAI/Core/Game/Features/Gameplay/HookSystem/BP_Hook.TryUngrab` (`self.HookActor`))))

(event `OnUngrab_Event`
  (`ActorComponent.Deactivate` (`self.NS_MagnetForce`))
  (`GameplayStatics.PlaySound2D` "/Engine/EditorSounds/GamePreview/EndSimulate.EndSimulate" 1.0 1.0 0.0 null null))

(event `self.PossessionEnded`
  (params (`New Entity` :type "/Game/ProjectAI/Core/Game/Features/Player/Base/BP_EntityBase Object Reference"))
  ;[1 0 0] Events
  (`parent.PossessionEnded` `New Entity`)
  (`/Game/ProjectAI/Core/Game/Features/Gameplay/HookSystem/BP_Hook.TryUngrab` (`self.HookActor`)))

(event `/Game/ProjectAI/Core/Game/Features/Gameplay/HighlightingSystem/BPI_Highlightable.StopHighlight`
  (`PrimitiveComponent.SetRenderCustomDepth` (`self.Mesh`) false)
  (`PrimitiveComponent.SetRenderCustomDepth` (`self.Magnet`) false))

(event `/Game/ProjectAI/Core/Game/Features/Gameplay/HighlightingSystem/BPI_Highlightable.StartHighlight`
  (`PrimitiveComponent.SetRenderCustomDepth` (`self.Mesh`) true)
  (`PrimitiveComponent.SetRenderCustomDepth` (`self.Magnet`) true))

(fn `GetCanBeGrabbed`
  (returns (bCanBeGrabbed :type Boolean))
  (return false))

(fn `SetHealthBarSocket`
  (`parent.SetHealthBarSocket`)
  (`SceneComponent.K2_AttachToComponent` (`self.HealthBar`) (`self.HealthBarSocket`) "None" "SnapToTarget" "SnapToTarget" "SnapToTarget" true))

(fn `SetMergePoint`
  (`parent.SetMergePoint`)
  (`SceneComponent.K2_AttachToComponent` (`self.MergePoint`) (`self.Mesh`) (`self.MergePointSocket`) "SnapToTarget" "SnapToTarget" "KeepWorld" true))

(fn `UserConstructionScript`
  (`parent.UserConstructionScript`))