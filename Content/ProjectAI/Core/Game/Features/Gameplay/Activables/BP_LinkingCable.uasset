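; BP_LinkingCable is an activable cable that glows to show whether it is powered.
; The construction script creates a dynamic material on CableMesh, applying its color and an initial emissive intensity from IsActiveOnBegin.
; Activate increments a trigger count and sets the active intensity.
; Deactivate decrements the count and dims the cable only at zero, so overlapping triggers keep it lit.
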(event `/Game/ProjectAI/Core/Game/Features/Gameplay/InteractSystem/Interfaces/BPI_Activable.Activate`
  (`parent.Activate`)
  (set `self.CurrentTriggerCount` (+ (`self.CurrentTriggerCount`) 1))
  (`MaterialInstanceDynamic.SetScalarParameterValue` (`self.DynamicMaterial`) "EmissiveIntensity" (`self.ActiveIntensity`)))

(event `/Game/ProjectAI/Core/Game/Features/Gameplay/InteractSystem/Interfaces/BPI_Activable.Deactivate`
  (`parent.Deactivate`)
  (bind _output_get (set `self.CurrentTriggerCount` (- (`self.CurrentTriggerCount`) 1)))
  (if (== _output_get 0)
    (`MaterialInstanceDynamic.SetScalarParameterValue` (`self.DynamicMaterial`) "EmissiveIntensity" (`self.DactiveIntesity`))))

(fn `UserConstructionScript`
  (`parent.UserConstructionScript`)
  (bind _returnvalue (`PrimitiveComponent.CreateDynamicMaterialInstance` (`self.CableMesh`) 0 null "None"))
  (bind _output_get (set `self.DynamicMaterial` _returnvalue))
  (`MaterialInstanceDynamic.SetVectorParameterValue` _output_get "Color" (`self.Color`))
  (if (`self.bIsActiveOnBegin`)
    (`MaterialInstanceDynamic.SetScalarParameterValue` (`self.DynamicMaterial`) "EmissiveIntensity" (`self.ActiveIntensity`))
    (else
      (`MaterialInstanceDynamic.SetScalarParameterValue` (`self.DynamicMaterial`) "EmissiveIntensity" (`self.DactiveIntesity`)))))