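; Hook system component that lets a hook pick up and carry actors implementing BPI_Grabbable beneath an assigned grab root.
; While idle, Tick box-traces along the root's down vector for a grab candidate.
; Grab notifies the actor, disables its gravity and ignores a custom collision channel; Ungrab restores both.
; While held, the actor is swept below the root matching its yaw, auto-releasing if blocked beyond DetachTolerance.
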(event `Init`
  (params (GrabRoot :type "SceneComponent Object Reference"))
  (set `self.GrabRootComponent` GrabRoot))

(event `self.ReceiveTick`
  (params (DeltaSeconds :type "Float (single-precision)"))
  (`self.GrabRootComponent`
    (:`then`
      (if (`self.bIsGrabbing`)
        (`self.UpdateGrabbedActorLocation`)
        (`self.CheckDetachmentTolerance`)
        (else
          (`self.TraceGrab`))))
    (:`else`)))

(fn `CheckDetachmentTolerance`
  (if (!= (`Actor.K2_GetActorLocation` (`self.GrabbedActor`)) (`self.GrabbedActorDesiredLocation`) :`ErrorTolerance` (`self.DetachTolerance`))
    (`self.Ungrab`)))

(fn `GetGrabInfo`
  (returns (GrabbedActor :type "Actor Object Reference") (bIsGrabbing :type Boolean) (GrabbedActorDesiredLocation :type "Vector Structure"))
  (return (`self.GrabbedActor`) (`self.bIsGrabbing`) (`self.GrabbedActorDesiredLocation`)))

(fn `Grab`
  (returns (bHasGrabbed :type Boolean))
  (bind _grabbedactor (`self.GrabbedActor`))
  (bind _returnvalue (and (`self.bCanGrabActor`) (`KismetSystemLibrary.IsValid` _grabbedactor)))
  (if _returnvalue
    (set `self.bIsGrabbing` true)
    (bind _asbpi_grabbable (cast `/Game/ProjectAI/Core/Game/Features/Gameplay/HookSystem/Interfaces/BPI_Grabbable` _grabbedactor))
    (`/Game/ProjectAI/Core/Game/Features/Gameplay/HookSystem/Interfaces/BPI_Grabbable.Grab` _asbpi_grabbable)
    (set `self.RotationOffset` (`Actor.K2_GetActorRotation` _grabbedactor))
    (`self.IgnoreGrabbedActorCollision` true)
    (`self.SetGrabbedActorGravity` false)
    (return _returnvalue)))

(fn `TraceGrab`
  (locals (NewLocalVar :type "Actor Object Reference"))
  (bind _grabrootcomponent (`self.GrabRootComponent`))
  (bind _grabrootcomponent_2 (`self.GrabRootComponent`))
  (bind _outhit (`KismetSystemLibrary.BoxTraceSingle` :`Start` (+ (`SceneComponent.K2_GetComponentLocation` _grabrootcomponent) (0.0 0.0 0.0)) :`End` (+ (`SceneComponent.K2_GetComponentLocation` _grabrootcomponent) (* (`SceneComponent.GetUpVector` _grabrootcomponent) (`self.TraceLength`) -1.0)) :`HalfSize` (`.BoxExtent` (`KismetSystemLibrary.GetComponentBounds` _grabrootcomponent_2)) :`Orientation` (`SceneComponent.K2_GetComponentRotation` _grabrootcomponent_2) :`TraceChannel` "TraceTypeQuery4" :`DrawDebugType` "ForOneFrame"))
  (if (and (`GameplayStatics.BreakHitResult` _outhit) (`KismetSystemLibrary.DoesImplementInterface` (`.HitActor` (`GameplayStatics.BreakHitResult` _outhit)) "/Game/ProjectAI/Core/Game/Features/Gameplay/HookSystem/Interfaces/BPI_Grabbable.BPI_Grabbable_C"))
    (bind _asbpi_grabbable (cast `/Game/ProjectAI/Core/Game/Features/Gameplay/HookSystem/Interfaces/BPI_Grabbable` (`.HitActor` (`GameplayStatics.BreakHitResult` _outhit))))
    (bind _bcanbegrabbed (`/Game/ProjectAI/Core/Game/Features/Gameplay/HookSystem/Interfaces/BPI_Grabbable.GetCanBeGrabbed` _asbpi_grabbable))
    (if _bcanbegrabbed
      (set `self.GrabbedActor` (`.HitActor` (`GameplayStatics.BreakHitResult` _outhit)))
      (set `self.bCanGrabActor` true)
      (else
        (set `self.bCanGrabActor` false :!label _label)))
    (else
      (goto _label))))

(fn `Ungrab`
  (returns (bHasUngrabbed :type Boolean))
  (if (`self.bIsGrabbing`)
    (set `self.bIsGrabbing` false)
    (bind _asbpi_grabbable (cast `/Game/ProjectAI/Core/Game/Features/Gameplay/HookSystem/Interfaces/BPI_Grabbable` (`self.GrabbedActor`)))
    (`/Game/ProjectAI/Core/Game/Features/Gameplay/HookSystem/Interfaces/BPI_Grabbable.Ungrab` _asbpi_grabbable))
  (`self.IgnoreGrabbedActorCollision` false)
  (`self.SetGrabbedActorGravity` true)
  (return (`self.bIsGrabbing`)))

(fn `UpdateGrabbedActorLocation`
  (bind _grabrootcomponent (`self.GrabRootComponent`))
  (bind (_returnvalue_roll _returnvalue_pitch _returnvalue_yaw) (`KismetMathLibrary.BreakRotator` (`SceneComponent.K2_GetComponentRotation` (`self.GrabRootComponent`))))
  (bind _returnvalue (+ (`SceneComponent.K2_GetComponentLocation` _grabrootcomponent) (* (`SceneComponent.GetUpVector` _grabrootcomponent) -1.0 (.z (`.BoxExtent` (`KismetSystemLibrary.GetComponentBounds` (`self.GrabRootComponent`)))) 2.0) (0.0 0.0 0.0)))
  (`Actor.K2_SetActorLocation` (`self.GrabbedActor`) _returnvalue true false)
  (`Actor.K2_SetActorRotation` (`self.GrabbedActor`) (`KismetMathLibrary.MakeRotator` 0.0 0.0 _returnvalue_yaw) false)
  (set `self.GrabbedActorDesiredLocation` _returnvalue))