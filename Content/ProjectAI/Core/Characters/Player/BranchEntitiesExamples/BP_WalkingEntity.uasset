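; BP_WalkingEntity is an example walking branch entity for the player, built on character movement and a parent entity class.
; When its lifespan ends, it runs the parent logic, then cuts max walk speed by the SpeedPercentageDecrease fraction.
; SetMergePoint snaps the MergePoint component's location and rotation to a named socket on the mesh while keeping world scale.
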(event `/Game/ProjectAI/Core/Characters/Player/BP_EntityBase.LifespanEnded`
  (bind _charactermovement (`self.CharacterMovement`))
  (`parent.LifespanEnded`)
  (set `CharacterMovementComponent.MaxWalkSpeed` (* (`CharacterMovementComponent.MaxWalkSpeed` _charactermovement) (- 1.0 (`self.SpeedPercentageDecrease`))) _charactermovement))

(fn `SetMergePoint`
  (`SceneComponent.K2_AttachToComponent` (`self.MergePoint`) (`self.Mesh`) (`self.MergePointSocket`) "SnapToTarget" "SnapToTarget" "KeepWorld" true))

(fn `UserConstructionScript`
  (`parent.UserConstructionScript`))