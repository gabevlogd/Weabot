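; Inventory system actor component that tracks a single selected item and broadcasts selection changes.
; SelectItem clears all removal bindings on the previous item, binds to the new one's removal event, casts it to BP_PAIItemBase, then stores it, calls OnSelect and fires OnSelectedItem.
; When the selected item is removed, the component unbinds, clears the reference and fires OnDeselectedItem.
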(event `SelectItem`
  (params (Item :type "ItemBase Object Reference"))
  (bind _selecteditem (`self.SelectedItem`)
    (:`then`
      (clear `ItemBase.OnItemRemoved` _selecteditem))
    (:`else`
      _))
  (add `ItemBase.OnItemRemoved` Item (delegate `OnItemRemoved_Event`))
  (bind _asbp_paiitem_base (cast `/Game/ProjectAI/Core/Game/Features/Gameplay/InventorySystem/InventoryItems/Base/BP_PAIItemBase` Item))
  (bind _output_get (set `self.SelectedItem` _asbp_paiitem_base))
  (`/Game/ProjectAI/Core/Game/Features/Gameplay/InventorySystem/InventoryItems/Base/BP_PAIItemBase.OnSelect` _output_get)
  (`self.OnSelectedItem` _output_get))

(event `OnItemRemoved_Event`
  (remove `ItemBase.OnItemRemoved` (`self.SelectedItem`) (delegate `OnItemRemoved_Event`))
  (set `self.SelectedItem` null)
  (`self.OnDeselectedItem`))