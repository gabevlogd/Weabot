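; Double sliding door prop that opens once a required number of triggers are active and closes when the count falls one short.
; PrimaryInteract and SecondaryInteract raise and lower a clamped trigger counter.
; Each threshold stops the opposite timeline and plays the opening or closing one from the start.
; Both timelines lerp the Left and Right panels from their current location, so reversals start mid-slide.
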(event `/Game/ProjectAI/Core/Interactables/Interfaces/BPI_Interactable.PrimaryInteract`
  (bind _output_get (set `self.CurrentTriggersCount` (`KismetMathLibrary.Clamp` (+ (`self.CurrentTriggersCount`) 1) 0 (`self.MaxTriggersCount`))))
  (if (== _output_get (`self.MaxTriggersCount`))
    (`|ExecutionSequence`
      (:`then_0`
        (bind (_direction _alpha) (`Timeline|Timeline_0` :!via `Stop` :!label _label)
          (:`Update`
            (`SceneComponent.K2_SetRelativeLocation` (`self.Right`) (`KismetMathLibrary.VLerp` (`SceneComponent.RelativeLocation` (`self.Right`)) (0.0 -50.0 120.0) _alpha) false false)
            (`SceneComponent.K2_SetRelativeLocation` (`self.Left`) (`KismetMathLibrary.VLerp` (`SceneComponent.RelativeLocation` (`self.Left`)) (0.0 50.0 120.0) _alpha) false false))))
      (:`then_1`
        (bind (_direction_2 _alpha_2) (`Timeline|Timeline` :!via `PlayFromStart` :!label _label_2)
          (:`Update`
            (`SceneComponent.K2_SetRelativeLocation` (`self.Right`) (`KismetMathLibrary.VLerp` (`SceneComponent.RelativeLocation` (`self.Right`)) (0.0 -100.0 120.0) _alpha_2) false false)
            (`SceneComponent.K2_SetRelativeLocation` (`self.Left`) (`KismetMathLibrary.VLerp` (`SceneComponent.RelativeLocation` (`self.Left`)) (0.0 100.0 120.0) _alpha_2) false false)))))))

(event `/Game/ProjectAI/Core/Interactables/Interfaces/BPI_Interactable.SecondaryInteract`
  (bind _output_get (set `self.CurrentTriggersCount` (`KismetMathLibrary.Clamp` (- (`self.CurrentTriggersCount`) 1) 0 (`self.MaxTriggersCount`))))
  (if (== _output_get (- (`self.MaxTriggersCount`) 1))
    (`|ExecutionSequence`
      (:`then_0`
        (goto _label_2 :!via `Stop`))
      (:`then_1`
        (goto _label :!via `PlayFromStart`)))))

(fn `UserConstructionScript`)