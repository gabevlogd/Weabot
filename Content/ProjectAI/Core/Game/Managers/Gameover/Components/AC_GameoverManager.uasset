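; Game over manager component that restarts play through a level reload or provides a checkpoint respawn for the player pawn.
; TriggerGameover calls ReloadLevel, which opens the loading screen level rather than respawning in place.
; RespawnControllerPawn, not called within this graph, respawns the first player's BP_EntityBase pawn at the current checkpoint transform if one has been reached, then fires OnRespawn.
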(event `TriggerGameover`
  (`self.ReloadLevel`))

(fn `ReloadLevel`
  (`GameplayStatics.OpenLevelBySoftObjectPtr` "/Game/ProjectAI/Maps/Menus/LoadingScreens/LV_LoadingScreen.LV_LoadingScreen"))

(fn `RespawnControllerPawn`
  (bind (_outtransform _outhaseverreachedcheckpoint _returnvalue) (`CSUtility.TryGetCurrentCheckpointTransform`))
  (if (and _outhaseverreachedcheckpoint _returnvalue)
    (bind _asbp_entity_base (cast `/Game/ProjectAI/Core/Game/Features/Player/Base/BP_EntityBase` (`Controller.K2_GetPawn` (`GameplayStatics.GetPlayerController` 0))))
    (`/Game/ProjectAI/Core/Game/Features/Player/Base/BP_EntityBase.Respawn` _asbp_entity_base _outtransform)
    (`self.OnRespawn`)))