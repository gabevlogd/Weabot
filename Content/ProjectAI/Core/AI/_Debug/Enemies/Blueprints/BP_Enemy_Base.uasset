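; Base enemy character with health, melee attacks, hit reactions, a camera-facing healthbar and ragdoll death.
; Sight perception and attack-radius overlaps with the player set states on its AIC_Enemy_Base controller until death.
; Melee plays random montages at varied speeds, while HitTrace sphere-traces at a given socket to damage the player.
; Incoming damage is throttled by a DoOnce-and-delay gate, then updates health and briefly shows the healthbar.
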(event `M_MeleeAttack`
  (bind (_attackspeed_min _attackspeed_max) (break `/Game/ProjectAI/Core/Utility/Structs/S_FloatRange` (`self.AttackSpeed`)))
  ;[0.3857 0 1] Montages
  (`|PlayMontage` (`self.Mesh`) (`KismetArrayLibrary.Array_Random` (`self.AttackMontages`)) (`KismetMathLibrary.RandomFloatInRange` _attackspeed_min _attackspeed_max)
    (:`OnCompleted`
      _)
    (:`OnInterrupted`
      _))
  (`self.OnAttackEnd`))

(event `self.ReceiveBeginPlay`
  (`self.Init`))

(event `self.ReceiveTick`
  (params (DeltaSeconds :type "Float (single-precision)"))
  (`self.ComponentLookAtPlayerCamera` (`self.Healthbar`)))

(event `M_ReactHit`
  ;[0.3857 0 1] Montages
  (`|PlayMontage` (`self.Mesh`) "/Game/ProjectAI/Core/AI/_Debug/Enemies/Animations/Montages/AM_Enemy_Hit.AM_Enemy_Hit"))

(event `self.AIPerception.OnTargetPerceptionUpdated`
  (params (Actor :type "Actor Object Reference") (Stimulus :type "AIStimulus Structure"))
  (cast `/Game/ProjectAI/Core/Characters/Interfaces/BPI_Player` Actor)
  (bind (_stimulus _bissensed) (`self.CanSenseActor` Actor "NewEnumerator1"))
  (if _bissensed
    (`self.ChangeState` "NewEnumerator4")
    (else
      (`self.ChangeState` "NewEnumerator0"))))

(event `self.AttackRadius.OnComponentBeginOverlap`
  (params (OverlappedComponent :type "PrimitiveComponent Object Reference") (OtherActor :type "Actor Object Reference") (OtherComp :type "PrimitiveComponent Object Reference") (OtherBodyIndex :type Integer) (bFromSweep :type Boolean) (SweepResult :type "HitResult Structure (by ref)"))
  (cast `/Game/ProjectAI/Core/Characters/Interfaces/BPI_Player` OtherActor)
  (`self.ChangeState` "NewEnumerator3"))

(event `self.AttackRadius.OnComponentEndOverlap`
  (params (OverlappedComponent :type "PrimitiveComponent Object Reference") (OtherActor :type "Actor Object Reference") (OtherComp :type "PrimitiveComponent Object Reference") (OtherBodyIndex :type Integer))
  (cast `/Game/ProjectAI/Core/Characters/Interfaces/BPI_Player` OtherActor)
  (`self.ChangeState` "NewEnumerator4"))

(event `self.ReceiveAnyDamage`
  (params (Damage :type "Float (single-precision)") (DamageType :type "DamageType Object Reference") (InstigatedBy :type "Controller Object Reference") (DamageCauser :type "Actor Object Reference"))
  (`/Engine/EditorBlueprintResources/StandardMacros.DoOnce` false :!label _label
    (:`Completed`
      (`self.Receive Damage` Damage)
      (`KismetSystemLibrary.Delay` 0.3)
      (goto _label :!via `Reset`))))

(event `Death`
  (`/Game/ProjectAI/Core/AI/_Debug/Enemies/Controllers/AIC_Enemy_Base.SetIsDead` (`self.AIEnemyController`) true)
  (`self.Enable Ragdoll`)
  (`self.OnDeath`))

(fn `CanSenseActor`
  (params (Actor :type "Actor Object Reference") (Sense :type "/Game/ProjectAI/Core/AI/_Debug/Utility/Enums/E_Sense Enum" :default "NewEnumerator0"))
  (returns (Stimulus :type "AIStimulus Structure") (bIsSensed :type Boolean))
  (bind _info (`AIPerceptionComponent.GetActorsPerception` (`self.AIPerception`) Actor))
  (for _array_element (`.LastSensedStimuli` (break `ActorPerceptionBlueprintInfo` _info))
    (bind _returnvalue (`AIPerceptionSystem.GetSenseClassForStimulus` _array_element))
    (if (== _returnvalue (select `/Game/ProjectAI/Core/AI/_Debug/Utility/Enums/E_Sense` Sense :`NewEnumerator1` "/Script/AIModule.AISense_Sight" :`NewEnumerator2` "/Script/AIModule.AISense_Hearing" :`NewEnumerator3` "/Script/AIModule.AISense_Damage" :!type "Object Class Reference"))
      (return _array_element (`.bSuccessfullySensed` (break `AIStimulus` _array_element))))))

(fn `ChangeState`
  (params (State :type "/Game/ProjectAI/Core/AI/_Debug/Enemies/Behaviours/E_EnemyState Enum" :default "NewEnumerator0"))
  (`self.IsDead`
    (:`false`
      (`/Game/ProjectAI/Core/AI/_Debug/Enemies/Controllers/AIC_Enemy_Base.SetState` (`self.AIEnemyController`) State))))

(fn `Enable Ragdoll`
  (`PrimitiveComponent.SetSimulatePhysics` (`self.Mesh`) true)
  (`PrimitiveComponent.SetCollisionEnabled` (`self.CapsuleComponent`) "NoCollision"))

(fn `HideHealthbar`
  (`SceneComponent.SetVisibility` (`self.Healthbar`) false false))

(fn `HitTrace`
  (params (Target :type "SceneComponent Object Reference") (InSocketName :type Name))
  (bind _returnvalue (`SceneComponent.GetSocketLocation` Target InSocketName))
  (bind _outhit (`KismetSystemLibrary.SphereTraceSingleForObjects` :`Start` _returnvalue :`End` _returnvalue :`Radius` (`self.HitSphereRadius`) :`ObjectTypes` (`|MakeArray` "ObjectTypeQuery3" :!type "EObjectTypeQuery Enum") :`DrawDebugType` "ForDuration"))
  (cast `/Game/ProjectAI/Core/Characters/Interfaces/BPI_Player` (`.HitActor` (`GameplayStatics.BreakHitResult` _outhit)))
  (`GameplayStatics.ApplyDamage` (`.HitActor` (`GameplayStatics.BreakHitResult` _outhit)) (`self.AttackDamage`) null self))

(fn `Init`
  (`|ExecutionSequence`
    (:`then_0`
      (bind _asaic_enemy_base (cast `/Game/ProjectAI/Core/AI/_Debug/Enemies/Controllers/AIC_Enemy_Base` (`AIBlueprintHelperLibrary.GetAIController` self)))
      (set `self.AIEnemyController` _asaic_enemy_base)
      (`self.ChangeState` "NewEnumerator0")
      (bind _aswbp_enemy_healthbar (cast `/Game/ProjectAI/Core/AI/_Debug/Enemies/UI/WBP_EnemyHealthbar` (`WidgetComponent.GetWidget` (`self.Healthbar`))))
      (set `self.WBP_EnemyHealthbar` _aswbp_enemy_healthbar))
    (:`then_1`
      (set `self.CurrentHealth` (`self.MaxHealth`)))))

(fn `Receive Damage`
  (params (Damage :type "Float (double-precision)"))
  (bind _returnvalue (- (`self.CurrentHealth`) Damage))
  (`self.IsDead`
    (:`false`
      (if (<= _returnvalue 0.0)
        (set `self.CurrentHealth` 0.0)
        (`self.Death`)
        (else
          (set `self.CurrentHealth` _returnvalue)))
      (`self.M_ReactHit`)
      (set `/Game/ProjectAI/Core/AI/_Debug/Enemies/UI/WBP_EnemyHealthbar.HealthbarPercent` (/ (`self.CurrentHealth`) (`self.MaxHealth`)) (`self.WBP_EnemyHealthbar`))
      (`self.ShowHealthbar`)
      (`KismetSystemLibrary.K2_SetTimer` null "HideHealthbar" 5.0))))

(fn `ShowHealthbar`
  (`SceneComponent.SetVisibility` (`self.Healthbar`) true false))

(fn `UserConstructionScript`)