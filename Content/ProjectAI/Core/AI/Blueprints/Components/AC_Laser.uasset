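; Actor component that gives its owner a damaging Niagara laser beam with a timed charge, fire and shut-off cycle.
; Init creates the hidden beam, and StartCycle toggles it after delays, with sounds and start/end calls.
; While enabled, externally driven TraceLaser line-traces between given points, clips the beam at blocking hits and damages BPI_Player actors.
; The socket-search macro is left unconnected, so only one beam is created.
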(event `Init`
  (params (SocketsMesh :type "MeshComponent Object Reference"))
  (set `self.LasersMesh` SocketsMesh)
  (`self.CreateLaser`)
  (`self.DisableLaser`))

(event `StartCycle`
  (bind _returnvalue (`Actor.K2_GetActorLocation` (`self.GetOwner`)))
  (`self.OnStartLaserCycle`)
  (`KismetSystemLibrary.Delay` (`self.ChargeTime`))
  (`self.Enable Laser`)
  (`GameplayStatics.PlaySoundAtLocation` (`self.EnableLaserSound`) _returnvalue (struct) 3.0 (`KismetMathLibrary.RandomFloatInRange` 1.0 1.3) 0.0 "/Game/ProjectAI/Audio/Attenuations/SA_DroneSFX.SA_DroneSFX" null null null)
  (`KismetSystemLibrary.Delay` (`self.LaserEnabledTime`))
  (`GameplayStatics.PlaySoundAtLocation` (`self.DisableLasersSound`) _returnvalue (struct) 3.0 (`KismetMathLibrary.RandomFloatInRange` 1.0 1.3) 0.0 "/Game/ProjectAI/Audio/Attenuations/SA_Laser.SA_Laser" null null null)
  (`self.DisableLaser`)
  (`self.OnEndLaserCycle`))

(fn `CalculateTraceLaser`
  (params (Start :type "Vector Structure") (End :type "Vector Structure") (LaserColor :type "LinearColor Structure (by ref)") (LaserWidth :type "Float (single-precision) (by ref)") (Laser :type "NiagaraComponent Object Reference (by ref)"))
  (returns (`Hit Blocking Hit` :type Boolean) (HitLocation :type "Vector Structure") (`Out Hit Actor` :type "Actor Object Reference"))
  (locals (NSLaser :type "NiagaraComponent Object Reference"))
  (bind _nslaser (`local.NSLaser`))
  (bind _output_get (set `local.NSLaser` Laser))
  (`NiagaraComponent.SetVariableVec3` _output_get "User.Beam Start" Start)
  (bind _outhit (`KismetSystemLibrary.LineTraceSingle` :`Start` Start :`End` End :`TraceChannel` "TraceTypeQuery3" :`DrawDebugType` "ForOneFrame" :`TraceColor` (struct :`R` 1.0 :`G` 1.0 :`B` 1.0 :`A` 1.0) :`TraceHitColor` (struct :`R` 1.0 :`G` 1.0 :`B` 1.0 :`A` 1.0)))
  (if (`GameplayStatics.BreakHitResult` _outhit)
    (`NiagaraComponent.SetVariableVec3` (`local.NSLaser`) "User.Beam End" (`.Location` (`GameplayStatics.BreakHitResult` _outhit)))
    (else
      (`NiagaraComponent.SetVariableVec3` (`local.NSLaser`) "User.Beam End" End)))
  (`NiagaraComponent.SetVariableFloat` _nslaser "User.Beam Width" LaserWidth)
  (`NiagaraComponent.SetVariableLinearColor` _nslaser "User.Color" LaserColor)
  (return (`GameplayStatics.BreakHitResult` _outhit) (`.Location` (`GameplayStatics.BreakHitResult` _outhit)) (`.HitActor` (`GameplayStatics.BreakHitResult` _outhit))))

(fn `CreateLaser`
  (bind _returnvalue (`|AddComponentByClass` :`self` (`self.GetOwner`) :`Class` "/Script/Niagara.NiagaraComponent" :`bManualAttachment` true))
  (`NiagaraComponent.SetAsset` _returnvalue "/Game/ProjectAI/Art/Particles/NS_Laser.NS_Laser" true)
  (set `self.Laser` _returnvalue))

(fn `DisableLaser`
  (`self.SetVisibility` (`self.Laser`) false false)
  (set `self.bAreLasersEnabled` false))

(fn `Enable Laser`
  (`self.SetVisibility` (`self.Laser`) true false)
  (set `self.bAreLasersEnabled` true))

(fn `TraceLaser`
  (params (Start :type "Vector Structure") (LaserEndPoint :type "Vector Structure"))
  (if (`self.bAreLasersEnabled`)
    (bind (_hit_blocking_hit _hitlocation _out_hit_actor) (`self.CalculateTraceLaser` Start LaserEndPoint (`self.LaserColor`) (`self.LaserWidth`) (`self.Laser`)))
    (if (`KismetSystemLibrary.DoesImplementInterface` _out_hit_actor "/Game/ProjectAI/Core/Characters/Interfaces/BPI_Player.BPI_Player_C")
      (`GameplayStatics.ApplyDamage` _out_hit_actor (`self.LaserDamage`) null (`self.GetOwner`))))
  (return))