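; Base Blueprint for patrolling AI entities that supplies patrol targets by patrol type: around itself, within a patrol zone, or along waypoints.
; GetPatrolData returns a position and radius from the actor's location, the PatrolZone, or the current waypoint with capsule radius.
; Waypoint patrols start at the first point on BeginPlay and advance on each arrival, looping back to the start.
; Around and zone arrival handlers are empty hooks.
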(event `self.ReceiveBeginPlay`
  (`parent.ReceiveBeginPlay`)
  (`self.InitWaypoints`))

(event `OnPatrolDestinationReached`
  (switch `/Game/ProjectAI/Core/AI/Data/E_PatrolMode` (`self.PatrolType`)
    (:`NewEnumerator1`
      (`self.OnAroundDestinationReached`))
    (:`NewEnumerator0`
      (`self.OnPatrolZoneDestinationReached`))
    (:`NewEnumerator3`
      (`self.OnWaypointReached`))))

(event `OnAroundDestinationReached`)

(event `OnPatrolZoneDestinationReached`)

(event `OnWaypointReached`
  (`self.SetNextWaypoint`))

(fn `GetPatrolData`
  (returns (Position :type "Vector Structure") (Radius :type "Float (single-precision)"))
  (bind _patrolzone (`self.PatrolZone`))
  (switch `/Game/ProjectAI/Core/AI/Data/E_PatrolMode` (`self.PatrolType`)
    (:`NewEnumerator2`
      (return (0.0 0.0 0.0) 0.0))
    (:`NewEnumerator1`
      (return (`self.K2_GetActorLocation`) (`self.EntityPatrolRadius`)))
    (:`NewEnumerator0`
      (bind _returnvalue (`/Game/ProjectAI/Core/AI/Blueprints/Bases/BP_PatrolZone.GetRadius` _patrolzone))
      (return (`self.K2_GetActorLocation` _patrolzone) _returnvalue))
    (:`NewEnumerator3`
      (return (`self.CurrentWaypoint`) (`CapsuleComponent.GetScaledCapsuleRadius` (`self.CapsuleComponent`))))))

(fn `InitWaypoints`
  (if (and (`|EnumEquality` (`self.PatrolType`) "NewEnumerator3") (`KismetArrayLibrary.Array_IsValidIndex` (`self.Waypoints`)))
    (`self.SetCurrentWaypoint` 0)))

(fn `SetCurrentWaypoint`
  (params (WaypointIndex :type Integer))
  (set `self.CurrentWaypoint` (`self.K2_GetActorLocation` (`|GetArrayItem` (`self.Waypoints`) WaypointIndex)))
  (set `self.CurrentWaypointIndex` WaypointIndex))

(fn `UserConstructionScript`
  (`parent.UserConstructionScript`))