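; Base character for possessable entities, with look and move input, possession hand-off and health that doubles as lifespan.
; EntityRadar overlaps track nearby entities, with a nearest-entity helper; the interact input calls an empty TryPossessNewEntity hook.
; Possession swaps the controller, toggles tick, briefly disables input and notifies the game mode.
; UpdateLifespan, uncalled here, drains health and reports expiry; damage subtracts a MaxHealth fraction, gated by a cooldown.
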(event `self.ReceiveBeginPlay`
  ;[0 0 0] Unreal Events
  (`PrimitiveComponent.IgnoreActorWhenMoving` (`self.EntityRadar`) self true)
  (set `self.Health` (`self.MaxHealth`))
  (`self.SetGameMode`)
  (`self.SetPlayerController`))

(event `TryPossessNewEntity`
  ;[0 0 0] Custom Events
)

(event `PossessNewEntity`
  (params (NewEntity :type "/Game/ProjectAI/Core/Characters/Player/BP_EntityBase Object Reference") (PreviousEntity :type "/Game/ProjectAI/Core/Characters/Player/BP_EntityBase Object Reference"))
  ;[0 0 0] Custom Events
  (`self.PossessionEnded` NewEntity)
  (`Controller.Possess` (`GameplayStatics.GetPlayerController` 0) NewEntity)
  (`self.PossessionStarted` NewEntity PreviousEntity)
  (`/Game/ProjectAI/Core/GameModes/GM_Code_0a.OnEntityChanged` (`self.GameMode`) NewEntity PreviousEntity))

(event `EnhancedInput|/Game/ProjectAI/Core/Inputs/Actions/IA_Look`
  (params (ActionValue :type "Vector2D Structure") (ElapsedSeconds :type "Float (double-precision)") (TriggeredSeconds :type "Float (double-precision)") (InputAction :type "InputAction Object Reference" :default "/Game/ProjectAI/Core/Inputs/Actions/IA_Look.IA_Look"))
  ;[0 0 0] Movement
  (:`Triggered`
    (`self.Look` ActionValue)))

(event `EnhancedInput|/Game/ProjectAI/Core/Inputs/Actions/IA_Move`
  (params (ActionValue :type "Vector Structure") (ElapsedSeconds :type "Float (double-precision)") (TriggeredSeconds :type "Float (double-precision)") (InputAction :type "InputAction Object Reference" :default "/Game/ProjectAI/Core/Inputs/Actions/IA_Move.IA_Move"))
  ;[0 0 0] Movement
  (:`Triggered`
    (`self.Move` ActionValue)))

(event `LifespanEnded`
  ;[0 0 0] Custom Events
  (`/Game/ProjectAI/Core/GameModes/GM_Code_0a.OnLifespanEnded` (`self.GameMode`)))

(event `EnhancedInput|/Game/ProjectAI/Core/Inputs/Actions/IA_Interact`
  (params (ActionValue :type Boolean) (ElapsedSeconds :type "Float (double-precision)") (TriggeredSeconds :type "Float (double-precision)") (InputAction :type "InputAction Object Reference" :default "/Game/ProjectAI/Core/Inputs/Actions/IA_Interact.IA_Interact"))
  ;[0 0 0] Entity Change
  (:`Triggered`
    (`self.TryPossessNewEntity`)))

(event `PossessionStarted`
  (params (PreviousEntity :type "/Game/ProjectAI/Core/Characters/Player/BP_EntityBase Object Reference"))
  (bind _returnvalue (`GameplayStatics.GetPlayerController` 0))
  ;[0 0 0] Custom Events
  (set `self.IsPossessed` true)
  (`self.DisableInput` _returnvalue)
  (`KismetSystemLibrary.Delay` 1.0)
  (`self.EnableInput` _returnvalue)
  (`self.SetActorTickEnabled` true))

(event `self.EntityRadar.OnComponentBeginOverlap`
  (params (OverlappedComponent :type "PrimitiveComponent Object Reference") (OtherActor :type "Actor Object Reference") (OtherComp :type "PrimitiveComponent Object Reference") (OtherBodyIndex :type Integer) (bFromSweep :type Boolean) (SweepResult :type "HitResult Structure (by ref)"))
  ;[0 0 0] Entity Detection
  (bind _asbp_entity_base (cast `/Game/ProjectAI/Core/Characters/Player/BP_EntityBase` OtherActor))
  (`self.AddDetectedEntity` _asbp_entity_base))

(event `PossessionEnded`
  (params (`New Entity` :type "/Game/ProjectAI/Core/Characters/Player/BP_EntityBase Object Reference"))
  ;[0 0 0] Custom Events
  (set `self.IsPossessed` false)
  (`self.SetActorTickEnabled` false)
  (`NavMovementComponent.StopActiveMovement` (`self.CharacterMovement`)))

(event `self.EntityRadar.OnComponentEndOverlap`
  (params (OverlappedComponent :type "PrimitiveComponent Object Reference") (OtherActor :type "Actor Object Reference") (OtherComp :type "PrimitiveComponent Object Reference") (OtherBodyIndex :type Integer))
  ;[0 0 0] Entity Detection
  (bind _asbp_entity_base (cast `/Game/ProjectAI/Core/Characters/Player/BP_EntityBase` OtherActor))
  (`self.RemoveUndetectedEntity` _asbp_entity_base))

(event `self.ReceiveAnyDamage`
  (params (Damage :type "Float (single-precision)") (DamageType :type "DamageType Object Reference") (InstigatedBy :type "Controller Object Reference") (DamageCauser :type "Actor Object Reference"))
  ;[0 0 0] Damage
  (`self.ReciveDamage` Damage))

(fn `AddDetectedEntity`
  (params (`Detected Entity` :type "/Game/ProjectAI/Core/Characters/Player/BP_EntityBase Object Reference (by ref)"))
  (`KismetArrayLibrary.Array_Add` (`self.DetectedEntities`) `Detected Entity`))

(fn `GetIsPossessed`
  (returns (bIsPossessed :type Boolean))
  (return (`self.IsPossessed`)))

(fn `GetNearestEntity`
  (params (Entities :type "Array of /Game/ProjectAI/Core/Characters/Player/BP_EntityBase Object Reference"))
  (returns (Nearest :type "/Game/ProjectAI/Core/Characters/Player/BP_EntityBase Object Reference"))
  (locals (NearestDistance :type "Float (double-precision)") (NearestEntity :type "/Game/ProjectAI/Core/Characters/Player/BP_EntityBase Object Reference"))
  (if (> (`KismetArrayLibrary.Array_Length` Entities) 0)
    (bind _output_get (set `local.NearestEntity` (`|GetArrayItem` Entities)))
    (set `local.NearestDistance` (`self.GetDistanceTo` _output_get self))
    (for _array_element Entities
      (bind _returnvalue (`self.GetDistanceTo` _array_element self))
      (if (< _returnvalue (`local.NearestDistance`))
        (set `local.NearestEntity` _array_element)
        (set `local.NearestDistance` _returnvalue)))
    (return (`local.NearestEntity`))
    (else
      (return (`local.NearestEntity`)))))

(fn `Look`
  (params (LookInput :type "Vector2D Structure"))
  (`self.AddControllerYawInput` LookInput_X)
  (`self.AddControllerPitchInput` LookInput_Y))

(fn `Move`
  (params (MoveInput :type "Vector Structure"))
  (bind (_returnvalue_roll _returnvalue_pitch _returnvalue_yaw) (`KismetMathLibrary.BreakRotator` (`self.GetControlRotation`)))
  (`self.AddMovementInput` (`KismetMathLibrary.GreaterGreater_VectorRotator` MoveInput (`KismetMathLibrary.MakeRotator` _returnvalue_roll 0.0 _returnvalue_yaw))))

(fn `RemoveUndetectedEntity`
  (params (`Undetected Entity` :type "/Game/ProjectAI/Core/Characters/Player/BP_EntityBase Object Reference (by ref)"))
  (`KismetArrayLibrary.Array_RemoveItem` (`self.DetectedEntities`) `Undetected Entity`))

(fn `SetGameMode`
  (bind _asgm_code_0a (cast `/Game/ProjectAI/Core/GameModes/GM_Code_0a` (`GameplayStatics.GetGameMode`)))
  (set `self.GameMode` _asgm_code_0a))

(fn `SetPlayerController`
  (bind _asbp_player_controller (cast `/Game/ProjectAI/Core/Controllers/BP_PlayerController` (`GameplayStatics.GetPlayerController` 0)))
  (set `self.PlayerController` _asbp_player_controller))

(fn `UpdateLifespan`
  (params (`Delta Seconds` :type "Float (double-precision)"))
  (bind _output_get (set `self.Health` (- (`self.Health`) `Delta Seconds`)))
  (if (and (<= _output_get 0.0) (not (`self.IsDead`)))
    (set `self.IsDead` true)
    (`self.LifespanEnded`)))

(fn `UserConstructionScript`)