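; Player entity that possesses nearby BP_EntityCaptureBase entities and returns as the controlled body when possession comes back to it.
; Tick shows a HUD prompt over the nearest detected entity; capture input possesses it if a line trace to its MergePoint is unobstructed.
; Per-frame recursive lerps animate mesh and camera into MergePoint or out to ExitPoint, then restore input and health VFX.
; It also handles respawn, bobbing motion and a flashlight toggle.
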(event `self.ReceiveBeginPlay`
  ;[0 0 0] Unreal Events
  (`parent.ReceiveBeginPlay`)
  (set `self.IsPossessed` true)
  (add `self.EnterAnimEnded` (`|CreateDelegate` :!event `EnterAnimEnded_Event`))
  (add `self.ExitAnimEnded` (`|CreateDelegate` :!event `ExitAnimEnded_Event`)))

(event `EnterAnimEnded_Event` :!signature `self.EnterAnimEnded`
  (params (NewEntity :type "/Game/ProjectAI/Core/Game/Features/Player/Base/BP_EntityBase Object Reference"))
  ;[0 0 0] Custom Events
  (`self.EnableInput` NewEntity (`GameplayStatics.GetPlayerController` 0))
  (`self.SetActorTickEnabled` NewEntity true)
  (`self.SetHealthVFX` NewEntity (`/Game/ProjectAI/Core/Game/Features/Gameplay/HealthSystem/Components/AC_HealthManager.GetCurrentHealth` (`/Game/ProjectAI/Core/Game/Features/Player/Base/BP_EntityBase.AC_HealthManager` NewEntity))))

(event `self.ReceiveTick`
  (params (DeltaSeconds :type "Float (single-precision)"))
  ;[0 0 0] Unreal Events
  (`parent.ReceiveTick` DeltaSeconds)
  (`self.LookForEntityInteraction`))

(event `ExitAnimEnded_Event`
  ;[0 0 0] Custom Events
  (`self.EnableInput` (`GameplayStatics.GetPlayerController` 0))
  (`self.SetActorTickEnabled` true)
  (`PrimitiveComponent.SetCollisionEnabled` (`self.CapsuleComponent`) "QueryAndPhysics")
  (`self.SetHealthVFX` (`/Game/ProjectAI/Core/Game/Features/Gameplay/HealthSystem/Components/AC_HealthManager.GetCurrentHealth` (`self.AC_HealthManager`))))

(event `self.TryPossessNewEntity`
  (bind _detectedentities (`self.DetectedEntities`))
  (bind _nearest (`self.GetNearestEntity` _detectedentities))
  ;[0 0 0] Custom Events Override
  (if (> (`KismetArrayLibrary.Array_Length` _detectedentities) 0)
    (`self.CanEnterCapture` _nearest
      (:`True`
        (`self.PossessNewEntity` _nearest self)))))

(event `EnhancedInput|/Game/ProjectAI/Core/Game/Inputs/Actions/IA_EnterCapture`
  (params (ActionValue :type Boolean) (ElapsedSeconds :type "Float (double-precision)") (TriggeredSeconds :type "Float (double-precision)") (InputAction :type "InputAction Object Reference" :default "/Game/ProjectAI/Core/Game/Inputs/Actions/IA_EnterCapture.IA_EnterCapture"))
  ;[0 0 0] Input Actions
  (:`Triggered`
    (`self.TryPossessNewEntity`)))

(event `EnhancedInput|/Game/ProjectAI/Core/Game/Inputs/Actions/IA_ToggleFlashlight`
  (params (ActionValue :type Boolean) (ElapsedSeconds :type "Float (double-precision)") (TriggeredSeconds :type "Float (double-precision)") (InputAction :type "InputAction Object Reference" :default "/Game/ProjectAI/Core/Game/Inputs/Actions/IA_ToggleFlashlight.IA_ToggleFlashlight"))
  ;[0 0 0] Input Actions
  (:`Triggered`
    (`self.ToggleFlashlight`)))

(event `self.PossessionEnded`
  (params (`New Entity` :type "/Game/ProjectAI/Core/Game/Features/Player/Base/BP_EntityBase Object Reference"))
  ;[0 0 0] Custom Events Override
  (`parent.PossessionEnded` `New Entity`)
  (`/Game/ProjectAI/Core/Game/UGameFramework/HUD/BP_PAIGameplayHUD.HideInteraction` (`self.HUD`))
  (`PrimitiveComponent.SetCollisionEnabled` (`self.CapsuleComponent`) "NoCollision")
  (bind _output_get (set `self.ControlledEntity` `New Entity`))
  (`self.StartEnterAnimation` _output_get))

(event `self.PossessionStarted`
  (params (PreviousEntity :type "/Game/ProjectAI/Core/Game/Features/Player/Base/BP_EntityBase Object Reference"))
  ;[0 0 0] Custom Events Override
  (`parent.PossessionStarted` PreviousEntity)
  (if (or (`/Game/ProjectAI/Core/Game/Features/Gameplay/HealthSystem/Components/AC_HealthManager.GetDeathState` (`/Game/ProjectAI/Core/Game/Features/Player/Base/BP_EntityBase.AC_HealthManager` PreviousEntity)) (`/Game/ProjectAI/Core/Game/Features/Gameplay/HealthSystem/Components/AC_HealthManager.GetDeathState` (`self.AC_HealthManager`)))
    (`self.ExitAnimEnded_Event`)
    (else
      (`self.StartExitAnimation` PreviousEntity))))

(event `self.Respawn`
  (params (RespawnTransform :type "Transform Structure"))
  ;[0 0 0] Custom Events Override
  (`parent.Respawn` RespawnTransform)
  (`self.K2_SetActorLocationAndRotation` (.location RespawnTransform) (.rotation RespawnTransform)))

(event `EnterAnim`
  ;[0 0 0] Animations
  (`self.AnimationCompleted`
    (:`False`
      (`self.LerpMeshTransform` (`self.StartTransform`) (`SceneComponent.K2_GetComponentToWorld` (`/Game/ProjectAI/Core/Game/Features/Player/CaptureSystem/Base/BP_EntityCaptureBase.MergePoint` (cast `/Game/ProjectAI/Core/Game/Features/Player/CaptureSystem/Base/BP_EntityCaptureBase` (`self.ControlledEntity`) :!pure true))) (`self.GetLerpValue`))
      (`self.LerpCameraTransform` (`/Game/ProjectAI/Core/Game/Features/Player/Base/BP_EntityBase.Camera` (`self.ControlledEntity`)) (`self.StartCamTransform`) (struct) (`self.GetLerpValue`))
      (`KismetSystemLibrary.DelayUntilNextTick`)
      (`self.EnterAnim`))
    (:`True`
      (`self.LerpMeshTransform` (struct) (`SceneComponent.K2_GetComponentToWorld` (`/Game/ProjectAI/Core/Game/Features/Player/CaptureSystem/Base/BP_EntityCaptureBase.MergePoint` (cast `/Game/ProjectAI/Core/Game/Features/Player/CaptureSystem/Base/BP_EntityCaptureBase` (`self.ControlledEntity`) :!pure true))) 1.0)
      (`self.LerpCameraTransform` (`/Game/ProjectAI/Core/Game/Features/Player/Base/BP_EntityBase.Camera` (`self.ControlledEntity`)) (struct) (struct) 1.0)
      (`self.EnterAnimEnded` (`self.ControlledEntity`))
      (`KismetSystemLibrary.PrintString` (`KismetStringLibrary.Concat_StrStr` "Animation ended, total duration: " (`KismetStringLibrary.Conv_DoubleToString` (`self.AnimElapsedTime`)))))))

(event `ExitAnim`
  ;[0 0 0] Animations
  (`self.AnimationCompleted`
    (:`False`
      (`self.LerpMeshTransform` (`self.StartTransform`) (`self.EndTransform`) (`self.GetLerpValue`))
      (`self.LerpCameraTransform` (`self.Camera`) (`self.StartCamTransform`) (struct) (`self.GetLerpValue`))
      (`KismetSystemLibrary.DelayUntilNextTick`)
      (`self.ExitAnim`))
    (:`True`
      (`SceneComponent.K2_SetRelativeLocationAndRotation` :`self` (`self.Mesh`))
      (`self.LerpCameraTransform` (`self.Camera`) (struct) (struct) 1.0)
      (`self.ExitAnimEnded`)
      (`KismetSystemLibrary.PrintString` (`KismetStringLibrary.Concat_StrStr` "Animation ended, total duration: " (`KismetStringLibrary.Conv_DoubleToString` (`self.AnimElapsedTime`)))))))

(fn `AddBobbingMotion`
  (params (Target :type "SceneComponent Object Reference") (BobbingAmplitude :type "Float (double-precision)") (BobbingPhase :type "Float (double-precision)") (BobbingSpeed :type "Float (double-precision)"))
  (bind (_relativelocation_x _relativelocation_y) (`KismetMathLibrary.BreakVector` (`SceneComponent.RelativeLocation` Target)))
  (if (`self.IsPossessed`)
    (`SceneComponent.K2_SetRelativeLocation` Target (`KismetMathLibrary.MakeVector` _relativelocation_x _relativelocation_y (* (`KismetMathLibrary.Sin` (+ (* BobbingSpeed (- (`self.GetGameTimeSinceCreation`) 0.0)) BobbingPhase)) BobbingAmplitude)) false false)))

(fn `CacheCameraAnimationData`
  (params (CaptureEntity :type "/Game/ProjectAI/Core/Game/Features/Player/Base/BP_EntityBase Object Reference"))
  (locals (FromCamera :type "CameraComponent Object Reference") (ToCamera :type "CameraComponent Object Reference"))
  (bind _fromcamera (`local.FromCamera`))
  (bind _tocamera (`local.ToCamera`))
  (bind _camera (`/Game/ProjectAI/Core/Game/Features/Player/Base/BP_EntityBase.Camera` CaptureEntity))
  (`|ExecutionSequence`
    (:`then_0`
      (if (`self.IsPossessed`)
        (set `local.FromCamera` _camera)
        (set `local.ToCamera` (`self.Camera`))
        (else
          (set `local.FromCamera` (`self.Camera`))
          (set `local.ToCamera` _camera))))
    (:`then_1`
      (`SceneComponent.K2_SetWorldLocationAndRotation` _tocamera (`SceneComponent.K2_GetComponentLocation` _fromcamera) (`SceneComponent.K2_GetComponentRotation` _fromcamera) false false)
      (set `self.StartCamTransform` (`SceneComponent.GetRelativeTransform` _tocamera)))))

(fn `GetLerpValue`
  (returns (ReturnValue :type "Float (double-precision)"))
  (return (/ (`self.AnimElapsedTime`) (`self.AnimDuration`))))

(fn `LerpCameraTransform`
  (params (TargetCamera :type "SceneComponent Object Reference") (StartTransform :type "Transform Structure (by ref)") (EndTransform :type "Transform Structure (by ref)") (LerpValue :type "Float (single-precision)"))
  (bind (_returnvalue_location _returnvalue_rotation) (`KismetMathLibrary.BreakTransform` (`KismetMathLibrary.TLerp` StartTransform EndTransform LerpValue)))
  (`SceneComponent.K2_SetRelativeLocationAndRotation` TargetCamera _returnvalue_location _returnvalue_rotation false false))

(fn `LerpMeshTransform`
  (params (StartTransform :type "Transform Structure (by ref)") (EndTransform :type "Transform Structure (by ref)") (LerpValue :type "Float (single-precision)"))
  (bind (_returnvalue_location _returnvalue_rotation) (`KismetMathLibrary.BreakTransform` (`KismetMathLibrary.TLerp` StartTransform EndTransform LerpValue)))
  (`SceneComponent.K2_SetWorldLocationAndRotation` (`self.Mesh`) _returnvalue_location _returnvalue_rotation false false))

(fn `LookForEntityInteraction`
  (bind (_origin _boxextent _sphereradius) (`KismetSystemLibrary.GetComponentBounds` (`Character.Mesh` (`self.GetNearestEntity` (`self.DetectedEntities`)))))
  (if (> (`KismetArrayLibrary.Array_Length` (`self.DetectedEntities`)) 0)
    (`/Game/ProjectAI/Core/Game/UGameFramework/HUD/BP_PAIGameplayHUD.ShowInteraction` (`self.HUD`) (+ _origin (`KismetMathLibrary.MakeVector` 0.0 0.0 _sphereradius)) (`self.CaptureInteractionText`))
    (else
      (`/Game/ProjectAI/Core/Game/UGameFramework/HUD/BP_PAIGameplayHUD.HideInteraction` (`self.HUD`)))))

(fn `SetHealthVFX`
  (params (Health :type "Float (double-precision)"))
  (if (`self.IsPossessed`)
    (`parent.SetHealthVFX` Health)
    (else
      (bind _controlledentity (`self.ControlledEntity`)
        (:`then`
          (if (< Health (`/Game/ProjectAI/Core/Game/Features/Gameplay/HealthSystem/Components/AC_HealthManager.GetCurrentHealth` (`/Game/ProjectAI/Core/Game/Features/Player/Base/BP_EntityBase.AC_HealthManager` _controlledentity)))
            (`parent.SetHealthVFX` Health)))
        (:`else`)))))

(fn `StartEnterAnimation`
  (params (NewEntity :type "/Game/ProjectAI/Core/Game/Features/Player/Base/BP_EntityBase Object Reference"))
  (`self.CacheCameraAnimationData` NewEntity)
  (set `self.StartTransform` (`SceneComponent.K2_GetComponentToWorld` (`self.Mesh`)))
  (set `self.AnimElapsedTime` 0.0)
  (`self.EnterAnim`))

(fn `StartExitAnimation`
  (params (PreviousEntity :type "/Game/ProjectAI/Core/Game/Features/Player/Base/BP_EntityBase Object Reference"))
  (bind _asbp_entity_capture_base (cast `/Game/ProjectAI/Core/Game/Features/Player/CaptureSystem/Base/BP_EntityCaptureBase` PreviousEntity))
  (bind (_returnvalue_location _returnvalue_rotation) (`KismetMathLibrary.BreakTransform` (`SceneComponent.K2_GetComponentToWorld` (`/Game/ProjectAI/Core/Game/Features/Player/CaptureSystem/Base/BP_EntityCaptureBase.MergePoint` _asbp_entity_capture_base))))
  (set `self.StartTransform` (`KismetMathLibrary.MakeTransform` _returnvalue_location _returnvalue_rotation))
  (bind (_returnvalue_location_2 _returnvalue_rotation_2) (`KismetMathLibrary.BreakTransform` (`SceneComponent.K2_GetComponentToWorld` (`/Game/ProjectAI/Core/Game/Features/Player/CaptureSystem/Base/BP_EntityCaptureBase.ExitPoint` _asbp_entity_capture_base))))
  (set `self.EndTransform` (`KismetMathLibrary.MakeTransform` _returnvalue_location_2 _returnvalue_rotation_2))
  (set `self.AnimElapsedTime` 0.0)
  (`self.CacheCameraAnimationData` PreviousEntity)
  (`self.ExitAnim`))

(fn `UserConstructionScript`
  (`parent.UserConstructionScript`))