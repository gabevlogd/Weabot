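; Player character entity that can be possessed from another entity and hand possession back to it, as long as it is not falling.
; On possession, a timeline blends the camera from the previous entity's view, then attaches that entity to a merge-point socket, detaching it when possession ends.
; Grab and Ungrab toggle gravity, with grabbing also forcing falling movement.
; SetMergePoint runs at BeginPlay but is empty here.
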(event `self.ReceiveBeginPlay`
  (`parent.ReceiveBeginPlay`)
  (`self.SetMergePoint`))

(event `self.PossessionStarted`
  (params (PreviousEntity :type "/Game/ProjectAI/Core/Characters/Player/BP_EntityBase Object Reference"))
  (bind _camera (`/Game/ProjectAI/Core/Characters/Player/BP_EntityBase.Camera` PreviousEntity))
  (bind (_returnvalue_location _returnvalue_rotation) (`KismetMathLibrary.BreakTransform` (`SceneComponent.GetRelativeTransform` (`self.Camera`))))
  ;[0 0 0] Custom Events Override
  (`parent.PossessionStarted` PreviousEntity)
  (`SceneComponent.K2_SetWorldLocationAndRotation` (`self.Camera`) (`SceneComponent.K2_GetComponentLocation` _camera) (`SceneComponent.K2_GetComponentRotation` _camera) false false)
  (set `self.StartCamTrs` (`KismetMathLibrary.MakeTransform` _returnvalue_location _returnvalue_rotation))
  (bind (_direction _alpha) (`Timeline|Timeline_0` :!via `PlayFromStart`)
    (:`Update`
      (bind (_returnvalue_location_2 _returnvalue_rotation_2) (`KismetMathLibrary.BreakTransform` (`KismetMathLibrary.TLerp` (`self.StartCamTrs`) (`KismetMathLibrary.MakeTransform` (0.0 0.0 0.0)) _alpha)))
      (`SceneComponent.K2_SetRelativeLocationAndRotation` (`self.Camera`) _returnvalue_location_2 _returnvalue_rotation_2 false false))
    (:`Finished`
      (bind _output_get (set `self.Previous Entity` PreviousEntity))
      (`self.K2_AttachToComponent` _output_get (`self.MergePoint`) (`self.MergePointSocket`) "KeepWorld" "KeepWorld" "KeepWorld" true))))

(event `self.PossessionEnded`
  (params (`New Entity` :type "/Game/ProjectAI/Core/Characters/Player/BP_EntityBase Object Reference"))
  ;[0 0 0] Custom Events Override
  (`parent.PossessionEnded` `New Entity`)
  (`self.K2_DetachFromActor` (`self.Previous Entity`) "KeepWorld" "KeepWorld" "KeepWorld"))

(event `self.TryPossessNewEntity`
  ;[0 0 0] Custom Events Override
  (if (not (`NavMovementComponent.IsFalling` (`self.CharacterMovement`)))
    (`self.PossessNewEntity` (`self.Previous Entity`) self)))

(event `/Game/ProjectAI/Core/Interactables/GrabSystem/Interfaces/BPI_Grabbable.Grab`
  (bind _charactermovement (`self.CharacterMovement`))
  (set `CharacterMovementComponent.GravityScale` 0.0 _charactermovement)
  (`CharacterMovementComponent.SetMovementMode` _charactermovement "MOVE_Falling" 0))

(event `/Game/ProjectAI/Core/Interactables/GrabSystem/Interfaces/BPI_Grabbable.Ungrab`
  (set `CharacterMovementComponent.GravityScale` 1.0 (`self.CharacterMovement`)))

(fn `GetCanBeGrabbed`
  (returns (bCanBeGrabbed :type Boolean))
  (return (`self.bIsEntityGrabbable`)))

(fn `SetMergePoint`)

(fn `UserConstructionScript`
  (`parent.UserConstructionScript`))