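; Actor component that lets its owner react when one specific quest is achieved.
; On BeginPlay it looks up the quest manager and, if found, binds to its OnQuestAchieved event.
; When the achieved quest matches QuestToListen, it fires its OnThisQuestTriggered dispatcher.
; Matching compares quest references directly; a task ID comparison is left unused.
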(event `self.ReceiveBeginPlay`
  (bind (_questmanager _hasfound) (`/Game/ProjectAI/Core/Game/Gameplay/QuestSystem/Utility/BFL_QSUtility.TryGetQuestManager`))
  (if _hasfound
    (add `/Game/ProjectAI/Core/Game/Gameplay/QuestSystem/Components/AC_QuestManager.OnQuestAchieved` _questmanager (delegate `OnQuestAchieved_Event`))))

(event `OnQuestAchieved_Event`
  (params (Quest :type "/Game/ProjectAI/Core/Game/Gameplay/QuestSystem/Data/BP_QuestData Object Reference"))
  (if (== Quest (`self.QuestToListen`))
    (`self.OnThisQuestTriggered`)))