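; Quest manager component that runs an ordered diary of quests, tracking the current one by index.
; Each quest initializes on start and replaces the on-screen widget with its own widget class.
; AchieveTask marks the current quest's unfinished tasks and raises task, quest and diary completion notifications.
; Advancing requires a separate TryGoNextQuest call once all tasks are done; completing the diary can optionally hide the quest widget.
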(event `self.ReceiveBeginPlay`
  (`self.IsDiaryEmpty`
    (:`True`
      (`KismetSystemLibrary.PrintString` "QS: Quests Diary is Empty." true true (struct :`R` 1.0 :`G` 1.0 :`A` 1.0)))
    (:`False`
      (`self.InitQuest`))))

(event `InitQuest`
  (`/Game/ProjectAI/Core/Game/Gameplay/Systems/QuestSystem/Data/BP_QuestData.Init` (`self.CurrentQuest`))
  (`self.InitQuestWidget`))

(event `AchieveTask`
  (params (Task :type "/Game/ProjectAI/Core/Game/Gameplay/Systems/QuestSystem/Data/BP_TaskData Object Reference"))
  (`self.DoesCurrentQuestHasTask` Task
    (:`true`
      (set `/Game/ProjectAI/Core/Game/Gameplay/Systems/QuestSystem/Data/BP_TaskData.bIsAchieved` true Task)
      (`self.OnTaskAchieved` Task)
      (`KismetSystemLibrary.PrintString` "QS: Task Achieved." true true (struct :`R` 1.0 :`G` 1.0 :`B` 1.0 :`A` 1.0))
      (`self.IsCurrentQuestAchieved`
        (:`true`
          (`KismetSystemLibrary.PrintString` "QS: Current Quest Achieved." true true (struct :`R` 0.125 :`G` 1.0 :`B` 1.0 :`A` 1.0))
          (`self.OnQuestAchieved` (`self.CurrentQuest`))
          (`self.IsDiaryCompleted`
            (:`true`
              (`self.CompleteDiary`)
              (`KismetSystemLibrary.PrintString` "QS: Quests Diary Completed." true true (struct :`R` 0.125 :`G` 1.0 :`B` 1.0 :`A` 1.0)))))))))

(event `InitQuestWidget`
  (bind _currentquestwidget (`self.CurrentQuestWidget`)
    (:`then`
      (`Widget.RemoveFromParent` _currentquestwidget))
    (:`else`
      _))
  (bind _returnvalue (`|CreateWidget` (`/Game/ProjectAI/Core/Game/Gameplay/Systems/QuestSystem/Data/BP_QuestData.QuestWidget` (`self.CurrentQuest`))))
  (bind _output_get (set `self.CurrentQuestWidget` _returnvalue))
  (`/Game/ProjectAI/Core/Game/Gameplay/Systems/QuestSystem/UI/WBP_QuestBase.BuildWidget` _output_get (`self.CurrentQuest`))
  (`UserWidget.AddToViewport` _returnvalue 0))

(fn `CompleteDiary`
  (`self.OnDiaryCompleted`)
  (if (`self.bHideQuestBoxOnDiaryCompleted`)
    (`Widget.RemoveFromParent` (`self.CurrentQuestWidget`))))

(fn `GetCurrentQuest`
  (returns (CurrentQuest :type "/Game/ProjectAI/Core/Game/Gameplay/Systems/QuestSystem/Data/BP_QuestData Object Reference"))
  (return (`self.CurrentQuest`)))

(fn `TryGoNextQuest`
  (`self.IsCurrentQuestAchieved`
    (:`true`
      (`self.IsDiaryCompleted`
        (:`false`
          (set `self.CurrentQuestIndex` (+ (`self.CurrentQuestIndex`) 1))
          (`self.InitQuest`))))
    (:`false`
      (`self.OnCantGoNextQuest`)
      (`KismetSystemLibrary.PrintString` "QS: Tried to go to next quest with not all tasks achieved." true true (struct :`R` 1.0 :`G` 1.0 :`B` 1.0 :`A` 1.0)))))