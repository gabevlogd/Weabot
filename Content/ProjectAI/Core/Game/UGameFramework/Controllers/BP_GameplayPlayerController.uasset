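; Gameplay player controller that creates and manages the wheel, game and pause menus and uses the selected inventory item on input.
; Menus receive inventory and data log components found on the game mode through data-table tags.
; Toggling allows one open menu at a time, swapping Enhanced Input mapping contexts, input mode and cursor visibility.
; The wheel cursor follows an input axis, or mouse position each tick without a gamepad.
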(event `self.ReceiveBeginPlay`
  (`parent.ReceiveBeginPlay`)
  (`self.InitUI`)
  (`self.Switch Mapping Context` null "/Game/ProjectAI/Core/Game/Inputs/IMC_GameplayInputs.IMC_GameplayInputs")
  (`self.SetActorTickEnabled` (`GameplayStatics.GetPlayerPawn` 0) true)
  (`WidgetBlueprintLibrary.SetInputMode_GameOnly` (`GameplayStatics.GetPlayerController` 0)))

(event `self.ReceiveTick`
  (params (DeltaSeconds :type "Float (single-precision)"))
  (`self.UIControllerTick` DeltaSeconds))

(event `EnhancedInput|/Game/ProjectAI/Core/Game/Inputs/Actions/IA_UseItem`
  (params (ActionValue :type Boolean) (ElapsedSeconds :type "Float (double-precision)") (TriggeredSeconds :type "Float (double-precision)") (InputAction :type "InputAction Object Reference" :default "/Game/ProjectAI/Core/Game/Inputs/Actions/IA_UseItem.IA_UseItem"))
  (:`Triggered`
    (bind _asgm_paigameplay (cast `/Game/ProjectAI/Core/Game/UGameFramework/GameModes/GM_PAIGameplay` (`GameplayStatics.GetGameMode`)))
    (bind _selecteditem (`/Game/ProjectAI/Core/Game/Features/Gameplay/InventorySystem/Components/AC_PAIINventorySystem.SelectedItem` (`/Game/ProjectAI/Core/Game/UGameFramework/GameModes/GM_PAIGameplay.PlayerInventorySystem` _asgm_paigameplay))
      (:`then`
        (`/Game/ProjectAI/Core/Game/Features/Gameplay/InventorySystem/InventoryItems/Base/BP_PAIItemBase.UseSelf` _selecteditem))
      (:`else`))))

(event `InitUI`
  (bind _returnvalue (`self.GetPlayerInventory`))
  (bind _returnvalue_2 (`self.GetDataLog`))
  (bind _returnvalue_3 (`|GenericCreateObject` "/Game/ProjectAI/Core/Game/Features/UI/Widgets/Systems/InventorySystem/WheelMenu/WBP_WheelMenu.WBP_WheelMenu_C" _returnvalue))
  (bind _output_get (set `self.UIWheelMenu` _returnvalue_3))
  (`self.AddMenu` _output_get)
  (bind _returnvalue_4 (`|GenericCreateObject` "/Game/ProjectAI/Core/Game/Features/UI/Widgets/Menus/GameplayMenu/WBP_GameplayMenu.WBP_GameplayMenu_C" _returnvalue _returnvalue_2))
  (bind _output_get_2 (set `self.UIGameMenu` _returnvalue_4))
  (`self.AddMenu` _output_get_2)
  (bind _returnvalue_5 (`|GenericCreateObject` "/Game/ProjectAI/Core/Game/Features/UI/Widgets/Menus/PauseMenu/WBP_PauseMenu.WBP_PauseMenu_C"))
  (bind _output_get_3 (set `self.UIPauseMenu` _returnvalue_5))
  (`self.AddMenu` _output_get_3 11)
  (add `/Game/ProjectAI/Core/Game/Features/UI/Widgets/Menus/PauseMenu/WBP_PauseMenu.OnResume` _output_get_3 (`|CreateDelegate` :!event `OnResume_Event`)))

(event `EnhancedInput|/Game/ProjectAI/Core/Game/Inputs/Actions/GameplayToUI/IA_ToggleGameMenu`
  (params (ActionValue :type Boolean) (ElapsedSeconds :type "Float (double-precision)") (TriggeredSeconds :type "Float (double-precision)") (InputAction :type "InputAction Object Reference" :default "/Game/ProjectAI/Core/Game/Inputs/Actions/GameplayToUI/IA_ToggleGameMenu.IA_ToggleGameMenu"))
  ;[1 0 0] Game Menu Inputs
  (:`Triggered`
    (`self.ToggleUIMenu` (`self.UIGameMenu`))))

(event `EnhancedInput|/Game/ProjectAI/Core/Game/Inputs/UIActions/IA_NextMenuPage`
  (params (ActionValue :type Boolean) (ElapsedSeconds :type "Float (double-precision)") (TriggeredSeconds :type "Float (double-precision)") (InputAction :type "InputAction Object Reference" :default "/Game/ProjectAI/Core/Game/Inputs/UIActions/IA_NextMenuPage.IA_NextMenuPage"))
  ;[1 0 0] Game Menu Inputs
  (:`Triggered`
    (`/Game/ProjectAI/Core/Game/Features/UI/Widgets/Menus/GameplayMenu/WBP_GameplayMenu.NextMenuPage` (`self.UIGameMenu`))))

(event `EnhancedInput|/Game/ProjectAI/Core/Game/Inputs/UIActions/IA_PreviousMenuPage`
  (params (ActionValue :type Boolean) (ElapsedSeconds :type "Float (double-precision)") (TriggeredSeconds :type "Float (double-precision)") (InputAction :type "InputAction Object Reference" :default "/Game/ProjectAI/Core/Game/Inputs/UIActions/IA_PreviousMenuPage.IA_PreviousMenuPage"))
  ;[1 0 0] Game Menu Inputs
  (:`Triggered`
    (`/Game/ProjectAI/Core/Game/Features/UI/Widgets/Menus/GameplayMenu/WBP_GameplayMenu.PreviousMenuPage` (`self.UIGameMenu`))))

(event `EnhancedInput|/Game/ProjectAI/Core/Game/Inputs/Actions/GameplayToUI/IA_TogglePauseMenu`
  (params (ActionValue :type Boolean) (ElapsedSeconds :type "Float (double-precision)") (TriggeredSeconds :type "Float (double-precision)") (InputAction :type "InputAction Object Reference" :default "/Game/ProjectAI/Core/Game/Inputs/Actions/GameplayToUI/IA_TogglePauseMenu.IA_TogglePauseMenu"))
  ;[1 0 0] Game Menu Inputs
  (:`Triggered`
    (`self.ToggleUIMenu` (`self.UIPauseMenu`))))

(event `OnResume_Event`
  ;[1 0 0] Game Menu Inputs
  (`self.CloseUIMenu` (`self.UIPauseMenu`)))

(event `UIControllerTick`
  (params (`Delta Seconds` :type "Float (double-precision)"))
  ;[1 0 0] Wheel Menu Inputs
  (if (not (`self.bIsUsingGamepad`))
    (`/Game/ProjectAI/Core/Game/Features/UI/Widgets/Systems/InventorySystem/WheelMenu/WBP_WheelMenu.SetCursorTargetAngleByAxis` (`self.UIWheelMenu`) (`self.GetNormalizedMousePosition`))))

(event `EnhancedInput|/Game/ProjectAI/Core/Game/Inputs/Actions/GameplayToUI/IA_ToggleWheelMenu`
  (params (ActionValue :type Boolean) (ElapsedSeconds :type "Float (double-precision)") (TriggeredSeconds :type "Float (double-precision)") (InputAction :type "InputAction Object Reference" :default "/Game/ProjectAI/Core/Game/Inputs/Actions/GameplayToUI/IA_ToggleWheelMenu.IA_ToggleWheelMenu"))
  ;[1 0 0] Wheel Menu Inputs
  (:`Triggered`
    (`self.ToggleUIMenu` (`self.UIWheelMenu`))))

(event `EnhancedInput|/Game/ProjectAI/Core/Game/Inputs/UIActions/IA_WheelCursor`
  (params (ActionValue :type "Vector2D Structure") (ElapsedSeconds :type "Float (double-precision)") (TriggeredSeconds :type "Float (double-precision)") (InputAction :type "InputAction Object Reference" :default "/Game/ProjectAI/Core/Game/Inputs/UIActions/IA_WheelCursor.IA_WheelCursor"))
  ;[1 0 0] Wheel Menu Inputs
  (:`Triggered`
    (`/Game/ProjectAI/Core/Game/Features/UI/Widgets/Systems/InventorySystem/WheelMenu/WBP_WheelMenu.SetCursorTargetAngleByAxis` (`self.UIWheelMenu`) ActionValue)))

(fn `AddMenu`
  (params (Menu :type "/Game/ProjectAI/Core/Game/Features/UI/Widgets/Menus/Base/WBP_UIMenuBase Object Reference") (ZOrder :type Integer))
  (`UserWidget.AddToViewport` Menu ZOrder)
  (`Widget.SetVisibility` Menu "Collapsed")
  (`KismetArrayLibrary.Array_Add` (`self.MenuList`) Menu))

(fn `CloseUIMenu`
  (params (UIMenu :type "/Game/ProjectAI/Core/Game/Features/UI/Widgets/Menus/Base/WBP_UIMenuBase Object Reference"))
  (`/Game/ProjectAI/Core/Game/Features/UI/Widgets/Menus/Base/WBP_UIMenuBase.Close` UIMenu)
  (`self.Switch Mapping Context` "/Game/ProjectAI/Core/Game/Inputs/IMC_MenuInputs.IMC_MenuInputs" "/Game/ProjectAI/Core/Game/Inputs/IMC_GameplayInputs.IMC_GameplayInputs")
  (`WidgetBlueprintLibrary.SetInputMode_GameOnly` self true)
  (set `self.bShowMouseCursor` false)
  (`self.OnCloseUIMenu` UIMenu))

(fn `GetDataLog`
  (returns (ReturnValue :type "InventorySystem Object Reference"))
  (bind _returnvalue (`|GetDataTableRow` "/Game/ProjectAI/Core/Game/ProjectConfig/DT_ProjectTags.DT_ProjectTags" "DataLogInventory")
    (:`then`
      (return (`self.FindComponentByTag` (`GameplayStatics.GetGameMode`) "/Script/ProjectAI.InventorySystem" (break `/Game/ProjectAI/Core/Game/ProjectConfig/Structs/S_TagValue` _returnvalue))))))

(fn `GetPlayerInventory`
  (returns (ReturnValue :type "/Game/ProjectAI/Core/Game/Features/Gameplay/InventorySystem/Components/AC_PAIINventorySystem Object Reference"))
  (bind _returnvalue (`|GetDataTableRow` "/Game/ProjectAI/Core/Game/ProjectConfig/DT_ProjectTags.DT_ProjectTags" "PlayerInventory")
    (:`then`
      (return (`self.FindComponentByTag` (`GameplayStatics.GetGameMode`) "/Game/ProjectAI/Core/Game/Features/Gameplay/InventorySystem/Components/AC_PAIINventorySystem.AC_PAIINventorySystem_C" (break `/Game/ProjectAI/Core/Game/ProjectConfig/Structs/S_TagValue` _returnvalue))))))

(fn `OpenUIMenu`
  (params (UIMenu :type "/Game/ProjectAI/Core/Game/Features/UI/Widgets/Menus/Base/WBP_UIMenuBase Object Reference"))
  (`/Game/ProjectAI/Core/Game/Features/UI/Widgets/Menus/Base/WBP_UIMenuBase.Open` UIMenu)
  (`self.Switch Mapping Context` "/Game/ProjectAI/Core/Game/Inputs/IMC_GameplayInputs.IMC_GameplayInputs" "/Game/ProjectAI/Core/Game/Inputs/IMC_MenuInputs.IMC_MenuInputs")
  (`WidgetBlueprintLibrary.SetInputMode_GameAndUIEx` self UIMenu "LockInFullscreen")
  (set `self.bShowMouseCursor` true)
  (`self.OnOpenUIMenu` UIMenu))

(fn `Switch Mapping Context`
  (params (From :type "InputMappingContext Object Reference") (To :type "InputMappingContext Object Reference"))
  (bind _returnvalue (subsystem `EnhancedInputLocalPlayerSubsystem`))
  (`EnhancedInputSubsystemInterface.RemoveMappingContext` _returnvalue From (struct))
  (`EnhancedInputSubsystemInterface.AddMappingContext` _returnvalue To 0 (struct)))

(fn `ToggleUIMenu`
  (params (UIMenu :type "/Game/ProjectAI/Core/Game/Features/UI/Widgets/Menus/Base/WBP_UIMenuBase Object Reference"))
  (`self.IsAnyMenuOpen` UIMenu
    (:`False`
      (if (`Widget.IsVisible` UIMenu)
        (`self.CloseUIMenu` UIMenu)
        (else
          (`self.OpenUIMenu` UIMenu))))))

(fn `UserConstructionScript`)