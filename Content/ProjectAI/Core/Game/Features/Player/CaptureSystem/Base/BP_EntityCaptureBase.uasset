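; Base entity that the player can capture by interacting, then control and leave.
; On possession, the main entity's mesh attaches to a merge point and its actor to an exit point; both detach when possession ends.
; Leaving requires not falling and a clear line trace to the exit.
; While possessed, damage passes to the main entity, and respawning attempts release before respawning both; grabbing toggles gravity.
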(event `/Game/ProjectAI/Core/Game/Features/Gameplay/HookSystem/Interfaces/BPI_Grabbable.Grab`
  (bind _charactermovement (`self.CharacterMovement`))
  ;[0 0 0] Interfaces
  (set `CharacterMovementComponent.GravityScale` 0.0 _charactermovement)
  (`CharacterMovementComponent.SetMovementMode` _charactermovement "MOVE_Falling" 0))

(event `self.ReceiveBeginPlay`
  ;[0 0 0] Unreal Events
  (`parent.ReceiveBeginPlay`)
  (`self.SetMergePoint`)
  (`self.SetActorTickEnabled` false)
  (`self.CacheMainEntity`))

(event `/Game/ProjectAI/Core/Game/Features/Gameplay/HookSystem/Interfaces/BPI_Grabbable.Ungrab`
  ;[0 0 0] Interfaces
  (set `CharacterMovementComponent.GravityScale` 1.0 (`self.CharacterMovement`)))

(event `self.PossessionStarted`
  (params (PreviousEntity :type "/Game/ProjectAI/Core/Game/Features/Player/Base/BP_EntityBase Object Reference"))
  ;[0 0 0] Custom Events Override
  (`parent.PossessionStarted` PreviousEntity)
  (bind _output_get (set `self.MainEntity` PreviousEntity))
  (bind _output_get_2 (set `self.MainEntityMesh` (`Character.Mesh` _output_get)))
  (`SceneComponent.K2_AttachToComponent` _output_get_2 (`self.MergePoint`) "None" "KeepRelative" "KeepRelative" "KeepRelative" true)
  (`self.K2_AttachToComponent` (`self.MainEntity`) (`self.ExitPoint`) "None" "SnapToTarget" "SnapToTarget" "KeepWorld" true))

(event `self.ReceiveAnyDamage`
  (params (Damage :type "Float (single-precision)") (DamageType :type "DamageType Object Reference") (InstigatedBy :type "Controller Object Reference") (DamageCauser :type "Actor Object Reference"))
  ;[0 0 0] Damage
  (`parent.ReceiveAnyDamage` Damage null null null)
  (if (`self.IsPossessed`)
    (`GameplayStatics.ApplyDamage` (`self.MainEntity`) Damage)))

(event `self.PossessionEnded`
  (params (`New Entity` :type "/Game/ProjectAI/Core/Game/Features/Player/Base/BP_EntityBase Object Reference"))
  ;[0 0 0] Custom Events Override
  (`parent.PossessionEnded` `New Entity`)
  (`SceneComponent.K2_AttachToComponent` (`self.MainEntityMesh`) (`Actor.RootComponent` (`self.MainEntity`)) "None" "KeepRelative" "KeepRelative" "KeepRelative" true)
  (`self.K2_DetachFromActor` (`self.MainEntity`) "KeepWorld" "KeepWorld" "KeepWorld"))

(event `EnhancedInput|/Game/ProjectAI/Core/Game/Inputs/Actions/IA_LeaveCapture`
  (params (ActionValue :type Boolean) (ElapsedSeconds :type "Float (double-precision)") (TriggeredSeconds :type "Float (double-precision)") (InputAction :type "InputAction Object Reference" :default "/Game/ProjectAI/Core/Game/Inputs/Actions/IA_LeaveCapture.IA_LeaveCapture"))
  ;[0 0 0] Input Action
  (:`Triggered`
    (`self.TryPossessNewEntity`)))

(event `EnhancedInput|/Game/ProjectAI/Core/Game/Inputs/Actions/IA_EnterCapture`
  (params (ActionValue :type Boolean) (ElapsedSeconds :type "Float (double-precision)") (TriggeredSeconds :type "Float (double-precision)") (InputAction :type "InputAction Object Reference" :default "/Game/ProjectAI/Core/Game/Inputs/Actions/IA_EnterCapture.IA_EnterCapture"))
  (bind _nearest (`self.GetNearestInteractable`))
  (bind _returnvalue (`KismetSystemLibrary.Conv_InterfaceToObject` _nearest))
  (bind _asactor (cast `Actor` _returnvalue :!pure true))
  ;[0 0 0] Input Action
  (:`Triggered`
    (`/Engine/EditorBlueprintResources/StandardMacros.IsValid` _returnvalue
      (:`Is Valid`
        (`self.CanBeInteractedWith` _asactor
          (:`true`
            (cast `/Game/ProjectAI/Core/Game/Features/Player/Base/BP_EntityBase` _asactor
              (:`CastFailed`
                (`/Game/ProjectAI/Core/Game/Features/Gameplay/InteractSystem/Interfaces/BPI_Interactable.EnableInteract` _nearest)))))))))

(event `self.TryPossessNewEntity`
  ;[0 0 0] Custom Events Override
  (`self.CanLeaveCapture`
    (:`True`
      (`self.PossessNewEntity` (`self.MainEntity`) self))))

(event `/Game/ProjectAI/Core/Game/Features/Gameplay/InteractSystem/Interfaces/BPI_Interactable.EnableInteract`
  ;[0 0 0] Interfaces
  (`self.PossessNewEntity` (`self.MainEntity`) self (`self.MainEntity`)))

(event `self.Respawn`
  (params (RespawnTransform :type "Transform Structure"))
  ;[0 0 0] Custom Events Override
  (`self.TryPossessNewEntity`)
  (`parent.Respawn` RespawnTransform)
  (`self.Respawn` (`self.MainEntity`) RespawnTransform))

(fn `CacheMainEntity`
  (bind _asbp_entity_base (cast `/Game/ProjectAI/Core/Game/Features/Player/Base/BP_EntityBase` (`GameplayStatics.GetPlayerPawn` 0)))
  (set `self.MainEntity` _asbp_entity_base))

(fn `CanBeInteracted`
  (returns (Return :type Boolean))
  (bind _mainentity (`self.MainEntity`)
    (:`then`
      (return (`/Game/ProjectAI/Core/Game/Features/Player/Base/BP_EntityBase.IsPossessed` _mainentity)))
    (:`else`
      (return false))))

(fn `CanSensePlayer`
  (returns (bCanSense :type Boolean))
  (return false))

(fn `GetCanBeGrabbed`
  (returns (bCanBeGrabbed :type Boolean))
  (return (`self.bIsEntityGrabbable`)))

(fn `GetHUDInteractionInfo`
  (returns (Location :type "Vector Structure") (Text :type Text) (InputAction :type "InputAction Object Reference"))
  (return (`SceneComponent.K2_GetComponentLocation` (`self.HUDInteractionPoint`)) "Enter" "/Game/ProjectAI/Core/Game/Inputs/Actions/IA_EnterCapture.IA_EnterCapture"))

(fn `SetHealthVFX`
  (params (Health :type "Float (double-precision)"))
  (if (`self.IsPossessed`)
    (if (< Health (`/Game/ProjectAI/Core/Game/Features/Gameplay/HealthSystem/Components/AC_HealthManager.GetCurrentHealth` (`/Game/ProjectAI/Core/Game/Features/Player/Base/BP_EntityBase.AC_HealthManager` (`self.MainEntity`))))
      (`parent.SetHealthVFX` Health))))

(fn `SetMergePoint`)

(fn `UserConstructionScript`
  (`parent.UserConstructionScript`))