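; BP_RoboticArm is a player-controlled robotic arm in the capture system that grabs and releases with a child-actor BP_Hook.
; Move input shifts the Control Rig "arm_ctrl" control along clamped X and yaws the actor, while Look input steps its clamped Z.
; The spring arm's height follows the control every tick, and the two ability inputs call the hook's grab and ungrab.
; SetMergePoint snaps the merge point to a mesh socket.
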(event `self.ControlRig.OnPreInitializeDelegate`
  (params (Component :type "ControlRigComponent Object Reference"))
  ;[0 0 0] Control Rig Events
  (`ControlRigComponent.AddMappedCompleteSkeletalMesh` Component (`self.Mesh`)))

(event `self.ReceiveBeginPlay`
  ;[0 0 0] Unreal Events
  (`parent.ReceiveBeginPlay`)
  (bind _asbp_hook (cast `/Game/ProjectAI/Core/Game/Features/Gameplay/HookSystem/BP_Hook` (`ChildActorComponent.ChildActor` (`self.ChildActor`))))
  (set `self.Hook` _asbp_hook))

(event `self.ReceiveTick`
  (params (DeltaSeconds :type "Float (single-precision)"))
  ;[0 0 0] Unreal Events
  (`parent.ReceiveTick` DeltaSeconds)
  (`self.UpdateCameraHeight`))

(event `EnhancedInput|/Game/ProjectAI/Core/Game/Inputs/Actions/IA_EntityAbility_0`
  (params (ActionValue :type Boolean) (ElapsedSeconds :type "Float (double-precision)") (TriggeredSeconds :type "Float (double-precision)") (InputAction :type "InputAction Object Reference" :default "/Game/ProjectAI/Core/Game/Inputs/Actions/IA_EntityAbility_0.IA_EntityAbility_0"))
  ;[0 0 0] Grab Ability
  (:`Triggered`
    (`/Game/ProjectAI/Core/Game/Features/Gameplay/HookSystem/BP_Hook.TryGrab` (`self.Hook`))))

(event `EnhancedInput|/Game/ProjectAI/Core/Game/Inputs/Actions/IA_EntityAbility_1`
  (params (ActionValue :type Boolean) (ElapsedSeconds :type "Float (double-precision)") (TriggeredSeconds :type "Float (double-precision)") (InputAction :type "InputAction Object Reference" :default "/Game/ProjectAI/Core/Game/Inputs/Actions/IA_EntityAbility_1.IA_EntityAbility_1"))
  ;[0 0 0] Grab Ability
  (:`Triggered`
    (`/Game/ProjectAI/Core/Game/Features/Gameplay/HookSystem/BP_Hook.TryUngrab` (`self.Hook`))))

(fn `Look`
  (params (LookInput :type "Vector2D Structure"))
  (bind (_returnvalue_x _returnvalue_y) (`KismetMathLibrary.BreakVector` (`ControlRigComponent.GetControlPosition` (`self.ControlRig`) "arm_ctrl" "LocalSpace")))
  (set `self.PosZ` (`KismetMathLibrary.FClamp` (+ (`self.PosZ`) (* (`KismetMathLibrary.SignOfFloat` (* LookInput_Y -1.0)) (`GameplayStatics.GetWorldDeltaSeconds`) (`self.SpeedZ`))) -130.0 283.0))
  (`ControlRigComponent.SetControlPosition` (`self.ControlRig`) "arm_ctrl" (`KismetMathLibrary.MakeVector` _returnvalue_x _returnvalue_y (`self.PosZ`)) "LocalSpace"))

(fn `Move`
  (params (MoveInput :type "Vector Structure"))
  (bind (_returnvalue_x _returnvalue_y _returnvalue_z) (`KismetMathLibrary.BreakVector` (`ControlRigComponent.GetControlPosition` (`self.ControlRig`) "arm_ctrl" "LocalSpace")))
  (bind _output_get (set `self.PosX` (`KismetMathLibrary.FClamp` (+ (`self.PosX`) (* MoveInput_X (`GameplayStatics.GetWorldDeltaSeconds`) (`self.SpeedX`))) -17.0 176.0)))
  (`ControlRigComponent.SetControlPosition` (`self.ControlRig`) "arm_ctrl" (`KismetMathLibrary.MakeVector` _output_get _returnvalue_y _returnvalue_z) "LocalSpace")
  (`self.K2_AddActorWorldRotation` (`KismetMathLibrary.MakeRotator` 0.0 0.0 (* (`GameplayStatics.GetWorldDeltaSeconds`) (`self.AngularSpeed`) MoveInput_Y))))

(fn `SetMergePoint`
  (`SceneComponent.K2_AttachToComponent` (`self.MergePoint`) (`self.Mesh`) (`self.MergePointSocket`) "SnapToTarget" "SnapToTarget" "KeepWorld" true))

(fn `UpdateCameraHeight`
  (bind _springarm (`self.SpringArm`))
  (bind (_returnvalue_x _returnvalue_y _returnvalue_z) (`KismetMathLibrary.BreakVector` (`ControlRigComponent.GetControlPosition` (`self.ControlRig`) "arm_ctrl" "ActorSpace")))
  (bind (_returnvalue_x_2 _returnvalue_y_2) (`KismetMathLibrary.BreakVector` (`SceneComponent.K2_GetComponentLocation` _springarm)))
  (`SceneComponent.K2_SetWorldLocation` _springarm (`KismetMathLibrary.MakeVector` _returnvalue_x_2 _returnvalue_y_2 (+ _returnvalue_z (`self.CamHeightOffset`))) false false))

(fn `UserConstructionScript`
  (`parent.UserConstructionScript`))