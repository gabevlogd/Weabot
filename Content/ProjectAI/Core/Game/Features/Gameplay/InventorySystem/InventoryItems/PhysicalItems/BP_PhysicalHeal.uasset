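; BP_PhysicalHeal is a physical inventory item that applies area healing when it hits something, then destroys itself.
; Its hit event calls the parent handler, then sphere-traces at the impact point using HealRadiusSize and a single object type.
; Each BP_EntityBase found gains GainedHealth through its health manager and plays healing effects.
; The trace leaves persistent debug drawing enabled.
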(event `self.HitActorEvent`
  (params (OtherActor :type "Actor Object Reference") (Hit :type "HitResult Structure"))
  (bind (_bblockinghit _binitialoverlap _time _distance _location) (`GameplayStatics.BreakHitResult` Hit))
  (`parent.HitActorEvent` OtherActor Hit)
  (bind _outhits (`KismetSystemLibrary.SphereTraceMultiForObjects` :`Start` _location :`End` _location :`Radius` (`self.HealRadiusSize`) :`ObjectTypes` (`|MakeArray` "ObjectTypeQuery7" :!type "EObjectTypeQuery Enum") :`DrawDebugType` "Persistent"))
  (for _array_element _outhits
    (bind _asbp_entity_base (cast `/Game/ProjectAI/Core/Game/Features/Player/Base/BP_EntityBase` (`.HitActor` (`GameplayStatics.BreakHitResult` _array_element))))
    (`/Game/ProjectAI/Core/Game/Features/Gameplay/HealthSystem/Components/AC_HealthManager.AddHealth` (`/Game/ProjectAI/Core/Game/Features/Player/Base/BP_EntityBase.AC_HealthManager` _asbp_entity_base) (`self.GainedHealth`))
    (`/Game/ProjectAI/Core/Game/Features/Player/Base/BP_EntityBase.PlayHealingEffects` _asbp_entity_base))
  (`self.K2_DestroyActor`))

(fn `UserConstructionScript`
  (`parent.UserConstructionScript`))