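; Gameplay game mode for ProjectAI that hosts the game-over, quest, player inventory, checkpoint and data-log managers.
; On BeginPlay it tags both inventories from a data table, loads saved state, respawns the player pawn and starts a config-timed camera fade.
; Player death triggers game over through the game-over manager.
; Save prep writes the level name and each manager's data into BP_PAISaveGame; load events push that data back.
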(event `self.ReceiveBeginPlay`
  (add `/Game/ProjectAI/Core/Game/Managers/Events/Components/AC_GameEvents.OnPlayerDeath` (`self.AC_GameEvents`) (`|CreateDelegate` :!event `OnPlayerDeath_Event`))
  (`self.InitTagsGraph`)
  (`self.InitSaveGraph`)
  (`self.OnLevelLoaded`))

(event `OnPlayerDeath_Event`
  ;[1 0 0] Events
  (`/Game/ProjectAI/Core/Game/Managers/Gameover/Components/AC_GameoverManager.TriggerGameover` (`self.AC_GameoverManager`)))

(event `OnLevelLoaded`
  ;[1 0 0] Events
  (`/Game/ProjectAI/Core/Game/Managers/Gameover/Components/AC_GameoverManager.RespawnControllerPawn` (`self.AC_GameoverManager`))
  (`self.FadeOut`))

(event `FadeOut`
  ;[1 0 0] Camera Fade Out
  (bind _returnvalue (`|GetDataTableRow` "/Game/ProjectAI/Core/Game/ProjectConfig/DT_ProjectConfigs.DT_ProjectConfigs" "CameraFadeFadeDuration")
    (:`then`
      (`/Game/ProjectAI/Core/Game/Features/UI/Utility/CameraFadeSystem/Components/AC_CameraFadeManager.StartFade` (`self.AC_CameraFadeManager`) false 0.25 1.0 0.0 (`.FloatValue_6_D6B628494000F149351A3B8B736089B6` (break `/Game/ProjectAI/Core/Game/ProjectConfig/Structs/S_ConfigValue` _returnvalue)) (struct :`A` 1.0) false))))

(event `InitSaveGraph`
  (add `SaveManager.OnLoadGame` (`SSUtility.GetSaveManager`) (`|CreateDelegate` :!event `OnLoadGame_Event`))
  (`self.SetAllLoadedData`))

(event `OnLoadGame_Event`
  (params (SlotName :type String) (UserIndex :type Integer) (SaveGameData :type "DefaultSaveGame Object Reference") (Instigator :type "Object Object Reference"))
  (`self.SetAllLoadedData`))

(event `SetAllLoadedData`
  ;[1 0 0 1 42] Load
  (bind _asbp_paisave_game (cast `/Game/ProjectAI/Core/Game/Data/SaveSystemData/BP_PAISaveGame` (`SSUtility.GetSaveGame`)))
  (`QuestManager.LoadSaveData` (`self.QuestManager`) (`/Game/ProjectAI/Core/Game/Data/SaveSystemData/BP_PAISaveGame.QuestLogSaveData` _asbp_paisave_game))
  (`InventorySystem.LoadSaveData` (`self.PlayerInventorySystem`) (`/Game/ProjectAI/Core/Game/Data/SaveSystemData/BP_PAISaveGame.PlayerInventory` _asbp_paisave_game))
  (`CheckpointsManager.LoadSaveData` (`self.CheckpointsManager`) (`/Game/ProjectAI/Core/Game/Data/SaveSystemData/BP_PAISaveGame.CheckpointsSaveData` _asbp_paisave_game))
  (`InventorySystem.LoadSaveData` (`self.DataLogInventory`) (`/Game/ProjectAI/Core/Game/Data/SaveSystemData/BP_PAISaveGame.DataLogInventory` _asbp_paisave_game)))

(event `self.Saver.OnPrepSave`
  (params (SaveGameData :type "DefaultSaveGame Object Reference") (SlotInfoItem :type "SlotInfoItem Object Reference") (Istigator :type "Object Object Reference"))
  ;[1 0 0 1 42] Save
  (bind _asbp_paisave_game (cast `/Game/ProjectAI/Core/Game/Data/SaveSystemData/BP_PAISaveGame` SaveGameData))
  (bind _returnvalue (`GameplayStatics.GetCurrentLevelName` true))
  (set `/Game/ProjectAI/Core/Game/Data/SaveSystemData/BP_PAISaveGame.LevelName` _returnvalue _asbp_paisave_game)
  (set `/Game/ProjectAI/Core/Game/Data/SaveSystemData/BP_PAISaveGame.QuestLogSaveData` (`QuestManager.CreateSaveData` (`self.QuestManager`)) _asbp_paisave_game)
  (set `/Game/ProjectAI/Core/Game/Data/SaveSystemData/BP_PAISaveGame.PlayerInventory` (`InventorySystem.CreateSaveData` (`self.PlayerInventorySystem`)) _asbp_paisave_game)
  (set `/Game/ProjectAI/Core/Game/Data/SaveSystemData/BP_PAISaveGame.CheckpointsSaveData` (`CheckpointsManager.CreateSaveData` (`self.CheckpointsManager`)) _asbp_paisave_game)
  (set `/Game/ProjectAI/Core/Game/Data/SaveSystemData/BP_PAISaveGame.DataLogInventory` (`InventorySystem.CreateSaveData` (`self.DataLogInventory`)) _asbp_paisave_game))

(event `InitTagsGraph`
  (bind _returnvalue (`|GetDataTableRow` "/Game/ProjectAI/Core/Game/ProjectConfig/DT_ProjectTags.DT_ProjectTags" "PlayerInventory")
    (:`then`
      (set `ActorComponent.ComponentTags` (`|MakeArray` (break `/Game/ProjectAI/Core/Game/ProjectConfig/Structs/S_TagValue` _returnvalue)) (`self.PlayerInventorySystem`))
      (bind _returnvalue_2 (`|GetDataTableRow` "/Game/ProjectAI/Core/Game/ProjectConfig/DT_ProjectTags.DT_ProjectTags" "DataLogInventory")
        (:`then`
          (set `ActorComponent.ComponentTags` (`|MakeArray` (break `/Game/ProjectAI/Core/Game/ProjectConfig/Structs/S_TagValue` _returnvalue_2)) (`self.DataLogInventory`)))))))

(fn `UserConstructionScript`)