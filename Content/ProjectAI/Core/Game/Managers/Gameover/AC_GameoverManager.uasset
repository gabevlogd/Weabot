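; Gameover manager component that handles game over and respawning of the player.
; TriggerGameover calls ReloadLevel, which opens the LV_LoadGameLoadingScreen level instead of reopening the current one directly.
; A separate RespawnControllerPawn function looks up the current level's checkpoint, respawns the player's BP_EntityBase pawn at its transform and fires OnRespawn.
; Respawn does nothing without a checkpoint, and the game over event does not call it.
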(event `TriggerGameover`
  (`self.ReloadLevel`))

(fn `ReloadLevel`
  (`GameplayStatics.OpenLevelBySoftObjectPtr` "/Game/ProjectAI/Maps/Menus/LoadingScreens/LV_LoadGameLoadingScreen.LV_LoadGameLoadingScreen"))

(fn `RespawnControllerPawn`
  (bind (_outcheckpointtransform _returnvalue) (`CSUtility.TryGetCheckpoint` (`/Game/ProjectAI/Core/Game/Utility/BFL_PAILevelsUtility.GetCurrentLevelLoaded`)))
  (if _returnvalue
    (bind _asbp_entity_base (cast `/Game/ProjectAI/Core/Game/Features/Player/Base/BP_EntityBase` (`GameplayStatics.GetPlayerPawn` 0)))
    (`/Game/ProjectAI/Core/Game/Features/Player/Base/BP_EntityBase.Respawn` _asbp_entity_base _outcheckpointtransform)
    (`self.OnRespawn`)))