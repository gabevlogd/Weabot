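; BP_Entity is a bobbing, limited-lifespan player pawn that can possess other entities and emerge from them.
; TryChangeEntity picks the nearest detected entity; a timeline then moves and scales the pawn into its MergePoint while extending the spring arm, before possession and self-destruction.
; Exiting animates it out from a given MergePoint to a point ahead, with camera collision off.
; Both transitions disable player input, and a random phase offsets each instance's sine bob.
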(event `self.ReceiveBeginPlay`
  (`parent.ReceiveBeginPlay`)
  (`self.SetLifeSpan` (`self.LifeSpan`))
  (set `self.RandomPhase` (`KismetMathLibrary.RandomFloatInRange` 0.0 10.0)))

(event `self.ReceiveTick`
  (params (DeltaSeconds :type "Float (single-precision)"))
  (`self.AddBobbingMotion` (`self.Mesh`) 0.5 (`self.RandomPhase`) 3.0))

(event `self.PossessNewEntity`
  (params (NewEntity :type "Pawn Object Reference"))
  (bind _returnvalue (`GameplayStatics.GetPlayerController` 0))
  (`self.DisableInput` _returnvalue)
  (bind _asbp_entity_base (cast `/Game/ProjectAI/Core/Characters/Player/BP_EntityBase` NewEntity))
  (bind _output_get (set `self.StartTransform` (`self.GetTransform`)))
  (bind (_direction _alpha) (`Timeline|Timeline`)
    (:`Update`
      (bind (_returnvalue_location _returnvalue_rotation _returnvalue_scale) (`KismetMathLibrary.BreakTransform` (`SceneComponent.K2_GetComponentToWorld` (`/Game/ProjectAI/Core/Characters/Player/BP_EntityBase.MergePoint` _asbp_entity_base))))
      (`self.K2_SetActorTransform` (`KismetMathLibrary.TLerp` (`self.StartTransform`) (`KismetMathLibrary.MakeTransform` _returnvalue_location (.rotation _output_get) _returnvalue_scale) _alpha))
      (set `SpringArmComponent.TargetArmLength` (`KismetMathLibrary.Lerp` 300.0 600.0 _alpha) (`self.SpringArm`)))
    (:`Finished`
      (`parent.PossessNewEntity` _asbp_entity_base)
      (`self.EnableInput` _returnvalue)
      (`self.Destroy Entity`))))

(event `self.ExitFromEntity`
  (params (MergePoint :type "Transform Structure"))
  (bind _returnvalue (`GameplayStatics.GetPlayerController` 0))
  (`self.DisableInput` _returnvalue)
  (set `SpringArmComponent.bDoCollisionTest` false (`self.SpringArm`))
  (bind (_direction _alpha) (`Timeline|Timeline_0`)
    (:`Update`
      (`self.K2_SetActorTransform` (`KismetMathLibrary.TLerp` (`KismetMathLibrary.MakeTransform` MergePoint_Location (struct) MergePoint_Scale) (`KismetMathLibrary.MakeTransform` (+ MergePoint_Location (* (`KismetMathLibrary.GetForwardVector` MergePoint_Rotation) 200.0))) _alpha)))
    (:`Finished`
      (set `SpringArmComponent.bDoCollisionTest` true (`self.SpringArm`))
      (`self.EnableInput` _returnvalue))))

(fn `AddBobbingMotion`
  (params (Target :type "SceneComponent Object Reference") (BobbingAmplitude :type "Float (double-precision)") (BobbingPhase :type "Float (double-precision)") (BobbingSpeed :type "Float (double-precision)"))
  (`SceneComponent.K2_AddRelativeLocation` Target (`KismetMathLibrary.MakeVector` 0.0 0.0 (* (`KismetMathLibrary.Sin` (+ (* BobbingSpeed (`self.GetGameTimeSinceCreation`)) BobbingPhase)) BobbingAmplitude)) false false))

(fn `TryChangeEntity`
  (if (> (`KismetArrayLibrary.Array_Length` (`self.DetectedEntities`)) 0)
    (bind _pawn (`/Game/ProjectAI/Core/Characters/Interfaces/BPI_Entity.GetPawn` (`self.GetNearestEntity` (`self.DetectedEntities`))))
    (`self.PossessNewEntity` _pawn)
    (`KismetSystemLibrary.PrintString` "Hello")))

(fn `UserConstructionScript`
  (`parent.UserConstructionScript`))