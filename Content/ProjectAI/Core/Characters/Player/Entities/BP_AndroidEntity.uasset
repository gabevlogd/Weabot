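; Player-possessable android entity that can lock onto and operate an AndroidInteractable.
; Ability 0 freezes movement, enables the interactable and runs a timeline lerp aligning the actor to its trigger hitbox, keeping height.
; Ability 1 restores walking and disables it, with input gated until alignment finishes.
; Interaction blocks grabbing and keeps movement disabled on possession; the merge point attaches to a mesh socket.
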(event `/Game/ProjectAI/Core/Characters/Player/BP_EntityBase.PossessionStarted`
  (params (PreviousEntity :type "/Game/ProjectAI/Core/Characters/Player/BP_EntityBase Object Reference"))
  ;[0 0 0] Custom Events Override
  (`parent.PossessionStarted` PreviousEntity)
  (if (`self.IsInteracting`)
    (`CharacterMovementComponent.DisableMovement` (`self.CharacterMovement`))))

(event `EnhancedInput|/Game/ProjectAI/Core/Inputs/Actions/IA_EntityAbility_0`
  (params (ActionValue :type Boolean) (ElapsedSeconds :type "Float (double-precision)") (TriggeredSeconds :type "Float (double-precision)") (InputAction :type "InputAction Object Reference" :default "/Game/ProjectAI/Core/Inputs/Actions/IA_EntityAbility_0.IA_EntityAbility_0"))
  (bind _returnvalue (`self.GetTransform`))
  (bind _returnvalue_2 (`SceneComponent.K2_GetComponentToWorld` (`/Game/ProjectAI/Core/Props/BP_AndroidInteractable.TriggerHitBox` (`self.AndroidInteractable`))))
  ;[0 0 0] Entity Abilities
  (:`Triggered`
    (if (`self.CanInteract`)
      (if (not (`self.IsInteracting`))
        (set `self.CanInteract` false)
        (`CharacterMovementComponent.DisableMovement` (`self.CharacterMovement`))
        (set `self.IsInteracting` true)
        (`/Game/ProjectAI/Core/Props/BP_AndroidInteractable.Enable` (`self.AndroidInteractable`))
        (bind (_direction _alpha) (`Timeline|Timeline` :!via `PlayFromStart`)
          (:`Update`
            (`self.K2_SetActorTransform` (`KismetMathLibrary.TLerp` (`KismetMathLibrary.MakeTransform` (`KismetMathLibrary.MakeVector` (.x (.location _returnvalue)) (.y (.location _returnvalue)) (.z (.location _returnvalue))) (.rotation _returnvalue)) (`KismetMathLibrary.MakeTransform` (`KismetMathLibrary.MakeVector` (.x (.location _returnvalue_2)) (.y (.location _returnvalue_2)) (.z (.location _returnvalue))) (.rotation _returnvalue_2)) _alpha)))
          (:`Finished`
            (set `self.CanInteract` true)))))))

(event `EnhancedInput|/Game/ProjectAI/Core/Inputs/Actions/IA_EntityAbility_1`
  (params (ActionValue :type Boolean) (ElapsedSeconds :type "Float (double-precision)") (TriggeredSeconds :type "Float (double-precision)") (InputAction :type "InputAction Object Reference" :default "/Game/ProjectAI/Core/Inputs/Actions/IA_EntityAbility_1.IA_EntityAbility_1"))
  ;[0 0 0] Entity Abilities
  (:`Triggered`
    (if (`self.CanInteract`)
      (if (`self.IsInteracting`)
        (`CharacterMovementComponent.SetMovementMode` (`self.CharacterMovement`) "MOVE_Walking" 0)
        (set `self.IsInteracting` false)
        (`/Game/ProjectAI/Core/Props/BP_AndroidInteractable.Disable` (`self.AndroidInteractable`))))))

(fn `GetCanBeGrabbed`
  (returns (bCanBeGrabbed :type Boolean))
  (return (and (not (`self.IsInteracting`)) (`self.bIsEntityGrabbable`))))

(fn `SetMergePoint`
  (`SceneComponent.K2_AttachToComponent` (`self.MergePoint`) (`self.Mesh`) (`self.MergePointSocket`) "SnapToTarget" "SnapToTarget" "KeepWorld" true))

(fn `UserConstructionScript`
  (`parent.UserConstructionScript`))