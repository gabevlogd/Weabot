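; Interactable prop that a BP_Android can use, switching a group of activables on or off through its Enable and Disable events.
; Its trigger box registers it as the overlapping android's AndroidInteractable and shows a HUD "Interact" prompt, clearing both on exit.
; Enable and Disable set IsActive and drive ACGroupTriggerActivable.
; It supports custom-depth highlighting, while CanBeInteracted always returns false.
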(event `Enable`
  (set `self.IsActive` true)
  (`/Game/ProjectAI/Core/Game/Features/Gameplay/InteractSystem/Components/AC_GroupTriggerActivable.ActivateAll` (`self.AC_GroupTriggerActivable`)))

(event `Disable`
  (set `self.IsActive` false)
  (`/Game/ProjectAI/Core/Game/Features/Gameplay/InteractSystem/Components/AC_GroupTriggerActivable.DeactivateAll` (`self.AC_GroupTriggerActivable`)))

(event `self.TriggerHitBox.OnComponentBeginOverlap`
  (params (OverlappedComponent :type "PrimitiveComponent Object Reference") (OtherActor :type "Actor Object Reference") (OtherComp :type "PrimitiveComponent Object Reference") (OtherBodyIndex :type Integer) (bFromSweep :type Boolean) (SweepResult :type "HitResult Structure (by ref)"))
  (bind _asbp_android (cast `/Game/ProjectAI/Core/Game/Features/Player/CaptureSystem/Captures/BP_Android` OtherActor))
  (set `/Game/ProjectAI/Core/Game/Features/Player/CaptureSystem/Captures/BP_Android.AndroidInteractable` self _asbp_android)
  (`/Game/ProjectAI/Core/Game/UGameFramework/HUD/BP_PAIGameplayHUD.ShowInteraction` (cast `/Game/ProjectAI/Core/Game/UGameFramework/HUD/BP_PAIGameplayHUD` (`PlayerController.GetHUD` (`GameplayStatics.GetPlayerController` 0)) :!pure true) (`SceneComponent.K2_GetComponentLocation` (`self.HUDInteractionPoint`)) "Interact" "/Game/ProjectAI/Core/Game/Inputs/Actions/IA_EntityAbility_0.IA_EntityAbility_0"))

(event `self.TriggerHitBox.OnComponentEndOverlap`
  (params (OverlappedComponent :type "PrimitiveComponent Object Reference") (OtherActor :type "Actor Object Reference") (OtherComp :type "PrimitiveComponent Object Reference") (OtherBodyIndex :type Integer))
  (bind _asbp_android (cast `/Game/ProjectAI/Core/Game/Features/Player/CaptureSystem/Captures/BP_Android` OtherActor))
  (set `/Game/ProjectAI/Core/Game/Features/Player/CaptureSystem/Captures/BP_Android.AndroidInteractable` (`self.Null`) _asbp_android)
  (`/Game/ProjectAI/Core/Game/UGameFramework/HUD/BP_PAIGameplayHUD.HideInteraction` (cast `/Game/ProjectAI/Core/Game/UGameFramework/HUD/BP_PAIGameplayHUD` (`PlayerController.GetHUD` (`GameplayStatics.GetPlayerController` 0)) :!pure true)))

(event `/Game/ProjectAI/Core/Game/Features/Gameplay/HighlightingSystem/BPI_Highlightable.StartHighlight`
  (`PrimitiveComponent.SetRenderCustomDepth` (`self.StaticMesh`) true))

(event `/Game/ProjectAI/Core/Game/Features/Gameplay/HighlightingSystem/BPI_Highlightable.StopHighlight`
  (`PrimitiveComponent.SetRenderCustomDepth` (`self.StaticMesh`) false))

(fn `CanBeHighlighted`
  (returns (Result :type Boolean))
  (return true))

(fn `CanBeInteracted`
  (returns (Return :type Boolean))
  (return false))

(fn `UserConstructionScript`)