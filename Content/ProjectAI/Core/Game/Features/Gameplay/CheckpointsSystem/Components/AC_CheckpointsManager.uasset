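; AC_CheckpointsManager is a component that stores the current checkpoint for the checkpoints system.
; SetCheckpoint validates the given checkpoint, composes its CheckpointTransform with its actor transform, saves the result with a HasCheckpoint flag, and prints its name.
; GetCheckpoint returns that flag and transform from CurrentCheckpointData, so only the latest transform is kept, with no reference to the checkpoint actor.
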(fn `GetCheckpoint`
  (returns (bHasCheckpoint :type Boolean) (Transform :type "Transform Structure"))
  (bind _currentcheckpointdata (`self.CurrentCheckpointData`))
  (return (`/Game/ProjectAI/Core/Game/Features/Gameplay/CheckpointsSystem/Data/BP_CheckpointData.bHasCheckpoint` _currentcheckpointdata) (`/Game/ProjectAI/Core/Game/Features/Gameplay/CheckpointsSystem/Data/BP_CheckpointData.Checkpoint` _currentcheckpointdata)))

(fn `SetCheckpoint`
  (params (Checkpoint :type "/Game/ProjectAI/Core/Game/Features/Gameplay/CheckpointsSystem/BP_Checkpoint Object Reference"))
  (bind _currentcheckpointdata (`self.CurrentCheckpointData`))
  (`/Engine/EditorBlueprintResources/StandardMacros.IsValid` Checkpoint
    (:`Is Valid`
      (set `/Game/ProjectAI/Core/Game/Features/Gameplay/CheckpointsSystem/Data/BP_CheckpointData.Checkpoint` (`KismetMathLibrary.ComposeTransforms` (`/Game/ProjectAI/Core/Game/Features/Gameplay/CheckpointsSystem/BP_Checkpoint.CheckpointTransform` Checkpoint) (`Actor.GetTransform` Checkpoint)) _currentcheckpointdata)
      (set `/Game/ProjectAI/Core/Game/Features/Gameplay/CheckpointsSystem/Data/BP_CheckpointData.bHasCheckpoint` true _currentcheckpointdata)
      (`KismetSystemLibrary.PrintString` (`KismetSystemLibrary.GetDisplayName` Checkpoint)))))