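; BP_ActorBlockerTrigger is a world trigger that controls a blocking static mesh, opening it on entry and restoring it on exit.
; EnterTrigger hides the mesh, disables its collision and prints a debug "Hello".
; ExitTrigger makes it visible again with query and physics collision.
; The construction script only calls its parent.
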(event `self.EnterTrigger`
  (`KismetSystemLibrary.PrintString` "Hello")
  (`SceneComponent.SetVisibility` (`self.StaticMesh`) false false)
  (`PrimitiveComponent.SetCollisionEnabled` (`self.StaticMesh`) "NoCollision"))

(event `self.ExitTrigger`
  (`SceneComponent.SetVisibility` (`self.StaticMesh`) true false)
  (`PrimitiveComponent.SetCollisionEnabled` (`self.StaticMesh`) "QueryAndPhysics"))

(fn `UserConstructionScript`
  (`parent.UserConstructionScript`))