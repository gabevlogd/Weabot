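; BP_Exoskeleton is a player exoskeleton that hands control over to a separate BP_Entity when changing entity.
; TryChangeEntity always spawns a BP_Entity at the MergePoint's location and scale.
; A DoOnce after the spawn lets only the first call run ExitFromEntity with the MergePoint transform and possess the new entity.
; The construction script only calls its parent.
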(fn `TryChangeEntity`
  (bind (_returnvalue_location _returnvalue_rotation _returnvalue_scale) (`KismetMathLibrary.BreakTransform` (`SceneComponent.K2_GetComponentToWorld` (`self.MergePoint`))))
  (bind _returnvalue (`|SpawnActorFromClass` "/Game/ProjectAI/Core/Characters/Player/BP_Entity.BP_Entity_C" (`KismetMathLibrary.MakeTransform` _returnvalue_location (struct) _returnvalue_scale) "AlwaysSpawn" "MultiplyWithRoot" null null))
  (`/Engine/EditorBlueprintResources/StandardMacros.DoOnce` false
    (:`Completed`
      (`KismetSystemLibrary.PrintString` "exit")
      (`self.ExitFromEntity` _returnvalue (`SceneComponent.K2_GetComponentToWorld` (`self.MergePoint`)))
      (`self.PossessNewEntity` _returnvalue))))

(fn `UserConstructionScript`
  (`parent.UserConstructionScript`))