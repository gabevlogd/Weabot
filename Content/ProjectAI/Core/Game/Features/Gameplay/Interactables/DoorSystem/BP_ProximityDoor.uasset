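; Proximity door that, while active, opens when a possessed BP_EntityBase enters its trigger and closes when one leaves.
; A signed play rate runs a single skeletal animation either way, reversing from the current position if mid-play, with 2D open/close sounds.
; On each toggle, actors of MustBeMoved classes tracked by the Collider are pushed out along the forward axis toward their side.
; Activate and Deactivate turn a dynamic feedback material green or red.
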(event `self.ReceiveBeginPlay`
  (bind _activationfeedback (`self.ActivationFeedback`))
  (bind _returnvalue (`PrimitiveComponent.CreateDynamicMaterialInstance` _activationfeedback 0 (`PrimitiveComponent.GetMaterial` _activationfeedback 0) "None"))
  (set `self.ActivationFeedbackMaterial` _returnvalue)
  (`parent.ReceiveBeginPlay`))

(event `self.DoorTrigger.OnComponentBeginOverlap`
  (params (OverlappedComponent :type "PrimitiveComponent Object Reference") (OtherActor :type "Actor Object Reference") (OtherComp :type "PrimitiveComponent Object Reference") (OtherBodyIndex :type Integer) (bFromSweep :type Boolean) (SweepResult :type "HitResult Structure (by ref)"))
  ;[0 0 0] Door Trigger
  (if (`self.GetIsActive`)
    (if (`self.IsClose`)
      (bind _asbp_entity_base (cast `/Game/ProjectAI/Core/Game/Features/Player/Base/BP_EntityBase` OtherActor))
      (if (`/Game/ProjectAI/Core/Game/Features/Player/Base/BP_EntityBase.IsPossessed` _asbp_entity_base)
        (`self.TriggerAnimation` false)
        (set `self.IsClose` false)))))

(event `self.DoorTrigger.OnComponentEndOverlap`
  (params (OverlappedComponent :type "PrimitiveComponent Object Reference") (OtherActor :type "Actor Object Reference") (OtherComp :type "PrimitiveComponent Object Reference") (OtherBodyIndex :type Integer))
  ;[0 0 0] Door Trigger
  (if (`self.GetIsActive`)
    (if (not (`self.IsClose`))
      (bind _asbp_entity_base (cast `/Game/ProjectAI/Core/Game/Features/Player/Base/BP_EntityBase` OtherActor))
      (if (`/Game/ProjectAI/Core/Game/Features/Player/Base/BP_EntityBase.IsPossessed` _asbp_entity_base)
        (`self.TriggerAnimation` true)
        (set `self.IsClose` true)))))

(event `self.Collider.OnComponentBeginOverlap`
  (params (OverlappedComponent :type "PrimitiveComponent Object Reference") (OtherActor :type "Actor Object Reference") (OtherComp :type "PrimitiveComponent Object Reference") (OtherBodyIndex :type Integer) (bFromSweep :type Boolean) (SweepResult :type "HitResult Structure (by ref)"))
  ;[0 0 0] Checks actors in between door
  (if (`KismetArrayLibrary.Array_Contains` (`self.MustBeMoved`) (`GameplayStatics.GetObjectClass` OtherActor))
    (`KismetArrayLibrary.Array_Add` (`self.ActorsToMove`) OtherActor)))

(event `self.Collider.OnComponentEndOverlap`
  (params (OverlappedComponent :type "PrimitiveComponent Object Reference") (OtherActor :type "Actor Object Reference") (OtherComp :type "PrimitiveComponent Object Reference") (OtherBodyIndex :type Integer))
  ;[0 0 0] Checks actors in between door
  (if (`KismetArrayLibrary.Array_Contains` (`self.MustBeMoved`) (`GameplayStatics.GetObjectClass` OtherActor))
    (`KismetArrayLibrary.Array_RemoveItem` (`self.ActorsToMove`) OtherActor)))

(event `/Game/ProjectAI/Core/Game/Features/Gameplay/InteractSystem/Interfaces/BPI_Activable.Activate`
  (`parent.Activate`)
  (`MaterialInstanceDynamic.SetVectorParameterValue` (`self.ActivationFeedbackMaterial`) "EmissiveColor" (struct :`G` 1.0 :`A` 1.0)))

(event `/Game/ProjectAI/Core/Game/Features/Gameplay/InteractSystem/Interfaces/BPI_Activable.Deactivate`
  (`parent.Deactivate`)
  (`MaterialInstanceDynamic.SetVectorParameterValue` (`self.ActivationFeedbackMaterial`) "EmissiveColor" (struct :`R` 1.0 :`A` 1.0)))

(fn `MoveActorsInBetween`
  (for _array_element (`self.ActorsToMove`)
    (bind _returnvalue_x (`KismetMathLibrary.BreakVector` (`KismetMathLibrary.InverseTransformLocation` (`self.GetTransform`) (`self.K2_GetActorLocation` _array_element))))
    (`self.K2_AddActorWorldOffset` _array_element (* (`self.GetActorForwardVector`) 100.0 (`KismetMathLibrary.SignOfFloat` _returnvalue_x)) false false))
  (return))

(fn `TriggerAnimation`
  (params (Close :type Boolean))
  (locals (DoorDirection :type "Float (double-precision)") (Sound :type "SoundBase Object Reference"))
  (bind _mesh_door_01_b_open (`self.Mesh_Door_01_b_Open`))
  (if Close
    (set `local.DoorDirection` (* (`self.Speed`) -1.0))
    (else
      (set `local.DoorDirection` (`self.Speed`))))
  (`self.MoveActorsInBetween`)
  (`SkeletalMeshComponent.SetPlayRate` (`self.Mesh_Door_01_b_Open`) (`local.DoorDirection`))
  (`|ExecutionSequence`
    (:`then_0`
      (if (`SkeletalMeshComponent.IsPlaying` (`self.Mesh_Door_01_b_Open`))
        (`SkeletalMeshComponent.SetPosition` (`self.Mesh_Door_01_b_Open`) (`SkeletalMeshComponent.GetPosition` (`self.Mesh_Door_01_b_Open`)) true)
        (elif (> (`local.DoorDirection`) 0.0)
          (`SkeletalMeshComponent.SetPosition` (`self.Mesh_Door_01_b_Open`) 0.0 true)
          (else
            (`SkeletalMeshComponent.SetPosition` (`self.Mesh_Door_01_b_Open`) (`AnimSequenceBase.SequenceLength` (`self.DoorAnimationSequence`)) true)))))
    (:`then_1`
      (`SkeletalMeshComponent.Play` _mesh_door_01_b_open false)
      (if (> (`SkeletalMeshComponent.GetPlayRate` _mesh_door_01_b_open) 0.0)
        (set `local.Sound` (`self.OpenSound`))
        (else
          (set `local.Sound` (`self.CloseSound`))))
      (`GameplayStatics.PlaySound2D` (`local.Sound`) 1.0 1.0 0.0 null null))))

(fn `UserConstructionScript`)