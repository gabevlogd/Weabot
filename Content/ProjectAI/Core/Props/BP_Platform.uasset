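; Moving platform that starts at point A and travels to point B once enough triggers are active.
; Primary and secondary interact events raise and lower a clamped counter: reaching the maximum sends it to B, and dropping to one below sends it back to A.
; Each move lerps on Tick from the current location, with duration derived from distance and speed.
; Actors overlapping the collision trigger are attached to ride along.
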(event `self.ReceiveBeginPlay`
  ;[0 0 0] Unreal Events
  ;;[0.1059 0.1059 0.1059] Set start platform location
  (`self.K2_SetActorLocation` (`SceneComponent.K2_GetComponentLocation` (`self.PointA`)) false true))

(event `self.CollisionTrigger.OnComponentBeginOverlap`
  (params (OverlappedComponent :type "PrimitiveComponent Object Reference") (OtherActor :type "Actor Object Reference") (OtherComp :type "PrimitiveComponent Object Reference") (OtherBodyIndex :type Integer) (bFromSweep :type Boolean) (SweepResult :type "HitResult Structure (by ref)"))
  ;[0 0 0] Unreal Events
  ;;[0.1059 0.1059 0.1059] Parenting
  (`self.K2_AttachToActor` OtherActor self "None" "KeepWorld" "KeepWorld" "KeepWorld" true))

(event `self.CollisionTrigger.OnComponentEndOverlap`
  (params (OverlappedComponent :type "PrimitiveComponent Object Reference") (OtherActor :type "Actor Object Reference") (OtherComp :type "PrimitiveComponent Object Reference") (OtherBodyIndex :type Integer))
  ;[0 0 0] Unreal Events
  ;;[0.1059 0.1059 0.1059] Parenting
  (`self.K2_DetachFromActor` OtherActor "KeepWorld" "KeepWorld" "KeepWorld"))

(event `self.ReceiveTick`
  (params (DeltaSeconds :type "Float (single-precision)"))
  ;[0 0 0] Unreal Events
  ;;[0.1059 0.1059 0.1059] Location Lerping
  (`self.LocationLerpCompleted`
    (:`false`
      (`self.PerformLocationLerp`))))

(event `/Game/ProjectAI/Core/Interactables/Interfaces/BPI_Interactable.PrimaryInteract`
  ;[0 0 0] Platform Trigger
  (bind _triggerplatformmovement (`self.IncrementTriggerCounter` 1 (`self.MaxTriggerCount`)))
  (if _triggerplatformmovement
    (`self.CalculateLerp Data` (`SceneComponent.K2_GetComponentLocation` (`self.PointB`)))))

(event `/Game/ProjectAI/Core/Interactables/Interfaces/BPI_Interactable.SecondaryInteract`
  ;[0 0 0] Platform Trigger
  (bind _triggerplatformmovement (`self.IncrementTriggerCounter` -1 (- (`self.MaxTriggerCount`) 1)))
  (if _triggerplatformmovement
    (`self.CalculateLerp Data` (`SceneComponent.K2_GetComponentLocation` (`self.PointA`)))))

(fn `CalculateLerp Data`
  (params (EndLocation :type "Vector Structure"))
  ;[0 0 0] Set Locations
  (set `self.StartLocation` (`self.K2_GetActorLocation`))
  (set `self.EndLocation` EndLocation)
  ;[0 0 0] Reset Timer
  (set `self.ElapsedTime` 0.0)
  ;[0 0 0] Set Lerp Duration
  (set `self.LerpDuration` (/ (`KismetMathLibrary.Vector_Distance` (`self.StartLocation`) (`self.EndLocation`)) (`self.Speed`))))

(fn `IncrementTriggerCounter`
  (params (CounterIncrement :type Integer) (TriggerValue :type Integer))
  (returns (TriggerPlatformMovement :type Boolean))
  (bind _output_get (set `self.CurrentTriggerCount` (`KismetMathLibrary.Clamp` (+ (`self.CurrentTriggerCount`) CounterIncrement) 0 (`self.MaxTriggerCount`))))
  (return (== _output_get TriggerValue)))

(fn `PerformLocationLerp`
  ;[0 0 0] Setting New Location
  (`self.K2_SetActorLocation` (`KismetMathLibrary.VLerp` (`self.StartLocation`) (`self.EndLocation`) (/ (`self.ElapsedTime`) (`self.LerpDuration`))))
  ;[0 0 0] Update Elapsed Time
  (set `self.ElapsedTime` (+ (`self.ElapsedTime`) (`GameplayStatics.GetWorldDeltaSeconds`))))

(fn `UserConstructionScript`
  (`parent.UserConstructionScript`))