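; AI turret that switches between alert and passive states as its AI controller reports targets entering or leaving.
; An ACLaser component, initialized with the fire point, fires cycles on Shoot and is disabled on target loss.
; AimAtTarget and ResetLookRotation use a shared frame-time-scaled lerp to rotate the pivot and fire point toward the target or back to relative rest, passing axis constraints for the pivot only.
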(event `self.ReceiveBeginPlay`
  (`parent.ReceiveBeginPlay`)
  (`|ExecutionSequence`
    (:`then_0`
      (`self.Init`))
    (:`then_1`
      ;[1 0 0] Events
      (add `/Game/ProjectAI/Core/Game/Features/AI/Behaviours/Base/Behaviour/AIC_EntityController.OnTargetEnter` (`self.AIController`) (delegate `OnTargetEnter_Event`))
      (add `/Game/ProjectAI/Core/Game/Features/AI/Behaviours/Base/Behaviour/AIC_EntityController.OnTargetExit` (`self.AIController`) (delegate `OnTargetLost_Event`)))))

(event `Init`
  ;[1 0 0] Initialization
  (`/Game/ProjectAI/Core/Game/Features/Gameplay/WeaponSystem/Laser/Components/AC_Laser.Init` (`self.AC_Laser`) null (`|MakeArray` (`self.FirePoint`))))

(event `OnTargetEnter_Event`
  (params (TargetEntity :type "/Game/ProjectAI/Core/Game/Features/Player/Base/BP_EntityBase Object Reference"))
  ;[1 0 0] Events
  (`self.ChangeToAlert`))

(event `OnTargetLost_Event`
  (params (TargetEntity :type "/Game/ProjectAI/Core/Game/Features/Player/Base/BP_EntityBase Object Reference"))
  ;[1 0 0] Events
  (`self.ChangeToPassive`)
  (`/Game/ProjectAI/Core/Game/Features/Gameplay/WeaponSystem/Laser/Components/AC_Laser.DisableLaser` (`self.AC_Laser`)))

(event `Shoot`
  (`/Game/ProjectAI/Core/Game/Features/Gameplay/WeaponSystem/Laser/Components/AC_Laser.ShootLaserCycle` (`self.AC_Laser`)))

(event `self.OnStunnedState`)

(fn `AimAtTarget`
  (bind _targetactor (`self.GetTargetActor`))
  (bind _returnvalue (`KismetMathLibrary.FindLookAtRotation` (`SceneComponent.K2_GetComponentLocation` (`self.Pivot`)) (`self.K2_GetActorLocation` _targetactor)))
  (`self.LerpRotate` (`self.Pivot`) _returnvalue (`self.LookAtConstraints`) false (`self.LookSpeed`))
  (`self.LerpRotate` (`self.FirePoint`) _returnvalue (struct) false (`self.LookSpeed`)))

(fn `LerpRotate`
  (params (TargetComponent :type "SceneComponent Object Reference") (TargetRotation :type "Rotator Structure") (Costraints :type "/Game/ProjectAI/Core/Game/Utility/Data/Structs/S_XYZConstraints Structure") (bIsRelative :type Boolean) (Speed :type "Float (double-precision)"))
  (locals (bIsCurrRelative :type Boolean) (LookTargetComponent :type "SceneComponent Object Reference") (CurrConstraints :type "/Game/ProjectAI/Core/Game/Utility/Data/Structs/S_XYZConstraints Structure") (CurrTargetRotation :type "Rotator Structure") (RotateSpeed :type "Float (double-precision)"))
  (set `local.RotateSpeed` Speed)
  (set `local.CurrConstraints` Costraints)
  (set `local.LookTargetComponent` TargetComponent)
  (set `local.bIsCurrRelative` bIsRelative)
  (set `local.CurrTargetRotation` TargetRotation)
  (if (`local.bIsCurrRelative`)
    ;[1 1 1] Relative
    (`SceneComponent.K2_SetRelativeRotation` (`local.LookTargetComponent`) (`self.ApplyConstraints` (`KismetMathLibrary.RLerp` (`SceneComponent.RelativeRotation` (`local.LookTargetComponent`)) (`local.CurrTargetRotation`) (* (`local.RotateSpeed`) (`GameplayStatics.GetWorldDeltaSeconds`)) true) (`local.CurrConstraints`)) false false)
    (else
      ;[1 1 1] World
      (`SceneComponent.K2_SetWorldRotation` (`local.LookTargetComponent`) (`self.ApplyConstraints` (`KismetMathLibrary.RLerp` (`SceneComponent.K2_GetComponentRotation` (`local.LookTargetComponent`)) (`local.CurrTargetRotation`) (* (`local.RotateSpeed`) (`GameplayStatics.GetWorldDeltaSeconds`)) true) (`local.CurrConstraints`)) false false))))

(fn `ResetLookRotation`
  (`self.LerpRotate` (`self.Pivot`) (struct) (`self.LookAtConstraints`) true (`self.LookSpeed`))
  (`self.LerpRotate` (`self.FirePoint`) (struct) (struct) true (`self.LookSpeed`)))

(fn `UserConstructionScript`
  (`parent.UserConstructionScript`))