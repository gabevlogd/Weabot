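; Base world trigger that fires empty EnterTrigger and ExitTrigger events after configurable delays on overlap begin and end.
; IsTriggeringActor accepts actors that implement a chosen interface or exactly match a chosen class.
; Each side has a DoOnce gate with optional destroy or retrigger after firing.
; The gates precede the actor check, so a rejected overlap also closes them without a reset.
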(event `EnterTrigger`)

(event `ExitTrigger`)

(event `self.Trigger.OnComponentBeginOverlap`
  (params (OverlappedComponent :type "PrimitiveComponent Object Reference") (OtherActor :type "Actor Object Reference") (OtherComp :type "PrimitiveComponent Object Reference") (OtherBodyIndex :type Integer) (bFromSweep :type Boolean) (SweepResult :type "HitResult Structure (by ref)"))
  (`/Engine/EditorBlueprintResources/StandardMacros.DoOnce` false :!label _label
    (:`Completed`
      (`self.IsTriggeringActor` OtherActor
        (:`True`
          (`KismetSystemLibrary.Delay` (`self.EnterTriggerDelay`))
          (`self.EnterTrigger`)
          (if (`self.DestroyAfterEnter`)
            (`self.K2_DestroyActor`)
            (elif (`self.EnterRetriggerable`)
              (goto _label :!via `Reset`))))))))

(event `self.Trigger.OnComponentEndOverlap`
  (params (OverlappedComponent :type "PrimitiveComponent Object Reference") (OtherActor :type "Actor Object Reference") (OtherComp :type "PrimitiveComponent Object Reference") (OtherBodyIndex :type Integer))
  (`/Engine/EditorBlueprintResources/StandardMacros.DoOnce` false :!label _label_2
    (:`Completed`
      (`self.IsTriggeringActor` OtherActor
        (:`True`
          (`KismetSystemLibrary.Delay` (`self.ExitTriggerDelay`))
          (`self.ExitTrigger`)
          (if (`self.DestroyAfterExit`)
            (`self.K2_DestroyActor`)
            (elif (`self.ExitRetriggerable`)
              (goto _label_2 :!via `Reset`))))))))

(fn `UserConstructionScript`)