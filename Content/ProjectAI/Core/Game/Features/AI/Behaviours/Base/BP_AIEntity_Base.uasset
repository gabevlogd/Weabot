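; Base Blueprint for AI entities, managing passive, alert and stunned states and exposing empty per-state events as hooks.
; On BeginPlay it initializes its AIC_EntityController with a Behaviour, then binds to the game event for player invisibility ending to trigger retargeting.
; State changes go through the controller and skip repeats.
; A timed stun blocks alert and passive changes, then returns to passive and finds a new target.
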(event `self.ReceiveBeginPlay`
  (bind _asaic_entity_controller (cast `/Game/ProjectAI/Core/Game/Features/AI/Behaviours/Base/Behaviour/AIC_EntityController` (`AIBlueprintHelperLibrary.GetAIController` self)))
  (bind _output_get (set `self.AIController` _asaic_entity_controller))
  (`/Game/ProjectAI/Core/Game/Features/AI/Behaviours/Base/Behaviour/AIC_EntityController.Init` _output_get (`self.Behaviour`))
  (bind (_bsuccess _gameevents) (`/Game/ProjectAI/Core/Game/Managers/Events/Utility/BFL_GameEventsUtility.TryGetGameEvents`))
  (if _bsuccess
    (bind _output_get_2 (set `self.Game Events` _gameevents))
    (add `/Game/ProjectAI/Core/Game/Managers/Events/Components/AC_GameEvents.OnPlayerEndInvisibility` _output_get_2 (`|CreateDelegate` :!event `OnPlayerEndInvisibility_Event`))))

(event `OnAlertState`)

(event `OnPassiveState`)

(event `OnStunnedState`)

(event `StunRoutine`
  (params (Duration :type "Float (single-precision)"))
  (set `self.bIsStunned` true)
  (`KismetSystemLibrary.Delay` Duration)
  (set `self.bIsStunned` false)
  (`self.ChangeToPassive`)
  (`/Game/ProjectAI/Core/Game/Features/AI/Behaviours/Base/Behaviour/AIC_EntityController.FindNewTarget` (`self.AIController`)))

(event `OnPlayerEndInvisibility_Event`
  (`/Game/ProjectAI/Core/Game/Features/AI/Behaviours/Base/Behaviour/AIC_EntityController.FindNewTarget` (`self.AIController`)))

(fn `ChangeToAlert`
  (if (not (`self.bIsStunned`))
    (bind _bisstate (`/Game/ProjectAI/Core/Game/Features/AI/Behaviours/Base/Behaviour/AIC_EntityController.IsState` (`self.AIController`) "NewEnumerator1"))
    (if (not _bisstate)
      (`/Game/ProjectAI/Core/Game/Features/AI/Behaviours/Base/Behaviour/AIC_EntityController.SetState` (`self.AIController`) "NewEnumerator1")
      (`self.OnAlertState`))))

(fn `ChangeToPassive`
  (if (not (`self.bIsStunned`))
    (bind _bisstate (`/Game/ProjectAI/Core/Game/Features/AI/Behaviours/Base/Behaviour/AIC_EntityController.IsState` (`self.AIController`) "NewEnumerator0"))
    (if (not _bisstate)
      (`/Game/ProjectAI/Core/Game/Features/AI/Behaviours/Base/Behaviour/AIC_EntityController.SetState` (`self.AIController`) "NewEnumerator0")
      (`self.OnPassiveState`))))

(fn `ChangeToStunned`
  (params (Duration :type "Float (single-precision)"))
  (bind _bisstate (`/Game/ProjectAI/Core/Game/Features/AI/Behaviours/Base/Behaviour/AIC_EntityController.IsState` (`self.AIController`) "NewEnumerator2"))
  (if (not _bisstate)
    (`/Game/ProjectAI/Core/Game/Features/AI/Behaviours/Base/Behaviour/AIC_EntityController.SetState` (`self.AIController`) "NewEnumerator2")
    (`self.OnStunnedState`)
    (`self.StunRoutine` Duration)))

(fn `GetTargetActor`
  (returns (TargetActor :type "Actor Object Reference"))
  (return (`/Game/ProjectAI/Core/Game/Features/AI/Behaviours/Base/Behaviour/AIC_EntityController.TargetActor` (`self.AIController`))))

(fn `UserConstructionScript`)