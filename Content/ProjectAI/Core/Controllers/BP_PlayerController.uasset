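; Player controller Blueprint that sets up input and the on-screen HUD for the player.
; On BeginPlay it adds the player input mapping context, creates the entity base HUD widget in the viewport, and enables ticking on the player pawn.
; HideHUD and ShowHUD events toggle the widget's visibility, with showing delayed by a short pause.
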(event `self.ReceiveBeginPlay`
  (`EnhancedInputSubsystemInterface.AddMappingContext` (subsystem `EnhancedInputLocalPlayerSubsystem`) "/Game/ProjectAI/Core/Inputs/IMC_PlayerInput.IMC_PlayerInput" 0 (struct))
  (`self.AddHUD`)
  (`self.SetActorTickEnabled` (`GameplayStatics.GetPlayerPawn` 0) true))

(event `HideHUD`
  (`Widget.SetVisibility` (`self.WidgetHUD`) "Hidden"))

(event `ShowHUD`
  (`KismetSystemLibrary.Delay` 0.5)
  (`Widget.SetVisibility` (`self.WidgetHUD`) "Visible"))

(fn `AddHUD`
  (bind _returnvalue (`|CreateWidget` "/Game/ProjectAI/Core/UI/WBP_EntityBaseHUD.WBP_EntityBaseHUD_C"))
  (bind _output_get (set `self.WidgetHUD` _returnvalue))
  (`UserWidget.AddToViewport` _output_get 0))

(fn `UserConstructionScript`)