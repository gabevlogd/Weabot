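; Possessable, stationary turret entity that the player aims and fires to break Geometry Collection destructibles.
; Possession toggles an aim pointer widget and camera pitch limits, and leaving eases the gun's yaw back to rest.
; Each tick the poseable mesh's gun bone follows control rotation.
; Cooldown-gated shots play effects, then sphere trace and spawn a directional force field actor at impacts on Geometry Collections.
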(event `self.ReceiveBeginPlay`
  ;[0 0 0] Unreal Events Override
  (`parent.ReceiveBeginPlay`)
  (bind _returnvalue (`|CreateWidget` "/Game/ProjectAI/Core/UI/WBP_TurretPointer.WBP_TurretPointer_C"))
  (bind _output_get (set `self.TurretPointerWidget` _returnvalue))
  (`UserWidget.AddToViewport` _output_get 0)
  (`Widget.SetVisibility` _output_get "Hidden"))

(event `self.ReceiveTick`
  (params (DeltaSeconds :type "Float (single-precision)"))
  ;[0 0 0] Unreal Events Override
  (`parent.ReceiveTick` DeltaSeconds)
  (`self.Aim`))

(event `EnhancedInput|/Game/ProjectAI/Core/Inputs/Actions/IA_EntityAbility_0`
  (params (ActionValue :type Boolean) (ElapsedSeconds :type "Float (double-precision)") (TriggeredSeconds :type "Float (double-precision)") (InputAction :type "InputAction Object Reference" :default "/Game/ProjectAI/Core/Inputs/Actions/IA_EntityAbility_0.IA_EntityAbility_0"))
  ;[0 0 0] Shoot
  (:`Triggered`
    (`/Engine/EditorBlueprintResources/StandardMacros.DoOnce` false :!label _label
      (:`Completed`
        (bind _returnvalue (`self.PlayShootFX`))
        (`KismetSystemLibrary.Delay` 0.1)
        (`ActorComponent.K2_DestroyComponent` _returnvalue)
        (`self.Shoot`)
        (`KismetSystemLibrary.Delay` (`self.ShootCooldown`))
        (goto _label :!via `Reset`)))))

(event `/Game/ProjectAI/Core/Characters/Player/BP_EntityBase.PossessionStarted`
  (params (PreviousEntity :type "/Game/ProjectAI/Core/Characters/Player/BP_EntityBase Object Reference"))
  ;[0 0 0] Custom Events Override
  (`parent.PossessionStarted` PreviousEntity)
  (`self.SetPitchAngleLimit` (`self.MinAimPitch`) (`self.MaxAimPitch`))
  (`Widget.SetVisibility` (`self.TurretPointerWidget`) "Visible"))

(event `/Game/ProjectAI/Core/Characters/Player/BP_EntityBase.PossessionEnded`
  (params (`New Entity` :type "/Game/ProjectAI/Core/Characters/Player/BP_EntityBase Object Reference"))
  ;[0 0 0] Custom Events Override
  (`parent.PossessionEnded` `New Entity`)
  (`self.SetPitchAngleLimit` -90.0 90.0)
  (`Widget.SetVisibility` (`self.TurretPointerWidget`) "Hidden")
  (bind _returnvalue (`PoseableMeshComponent.GetBoneRotationByName` (`self.PoseableMesh`) "gun" "ComponentSpace"))
  (bind (_direction _alpha) (`Timeline|Timeline` :!via `PlayFromStart`)
    (:`Update`
      (`PoseableMeshComponent.SetBoneRotationByName` (`self.PoseableMesh`) "gun" (`KismetMathLibrary.MakeRotator` 0.0 0.0 (`KismetMathLibrary.Lerp` (.yaw _returnvalue) 0.0 _alpha)) "ComponentSpace"))))

(fn `Aim`
  (bind (_returnvalue_roll _returnvalue_pitch _returnvalue_yaw) (`KismetMathLibrary.BreakRotator` (`self.GetControlRotation`)))
  (`PoseableMeshComponent.SetBoneRotationByName` (`self.PoseableMesh`) "gun" (`KismetMathLibrary.MakeRotator` (* _returnvalue_pitch -1.0) 0.0 (+ _returnvalue_yaw -90.0)) "WorldSpace"))

(fn `Move`
  (params (MoveInput :type "Vector Structure")))

(fn `PlayShootFX`
  (returns (ReturnValue :type "ParticleSystemComponent Object Reference"))
  (bind _firepoint (`self.FirePoint`))
  (bind (_returnvalue_roll _returnvalue_pitch _returnvalue_yaw) (`KismetMathLibrary.BreakRotator` (`SceneComponent.K2_GetComponentRotation` _firepoint)))
  (bind _returnvalue (`GameplayStatics.SpawnEmitterAtLocation` "/Engine/Tutorial/SubEditors/TutorialAssets/TutorialParticleSystem.TutorialParticleSystem" (`SceneComponent.K2_GetComponentLocation` _firepoint) (`KismetMathLibrary.MakeRotator` _returnvalue_roll (+ _returnvalue_pitch 270.0) _returnvalue_yaw) (0.7 0.7 0.7) false))
  (`GameplayStatics.PlaySound2D` "/Game/ProjectAI/Audio/Shoot_Sound.Shoot_Sound" 1.0 (`KismetMathLibrary.RandomFloatInRange` 1.0 1.3) 0.0 null null)
  (`CameraShakeSourceComponent.StartCameraShake` :`self` (`self.ShootShakeSource`) :`InCameraShake` "/Game/ProjectAI/Core/Characters/Player/Entities/TurretEntity/BP_TurretCameraShake.BP_TurretCameraShake_C")
  (return _returnvalue))

(fn `SetMergePoint`
  (`SceneComponent.K2_AttachToComponent` (`self.MergePoint`) (`self.PoseableMesh`) (`self.MergePointSocket`) "SnapToTarget" "SnapToTarget" "KeepWorld" true))

(fn `SetPitchAngleLimit`
  (params (`View Pitch Min` :type "Float (single-precision)") (`View Pitch Max` :type "Float (single-precision)"))
  (bind _returnvalue (`GameplayStatics.GetPlayerCameraManager` 0))
  (set `PlayerCameraManager.ViewPitchMin` `View Pitch Min` _returnvalue)
  (set `PlayerCameraManager.ViewPitchMax` `View Pitch Max` _returnvalue))

(fn `Shoot`
  (bind _returnvalue (`SceneComponent.K2_GetComponentLocation` (`self.FirePoint`)))
  (bind _outhit (`KismetSystemLibrary.SphereTraceSingle` :`Start` _returnvalue :`End` (+ _returnvalue (* (`KismetMathLibrary.GetForwardVector` (`self.GetControlRotation`)) (`self.MaxShootDistance`))) :`Radius` 5.0 :`TraceChannel` "TraceTypeQuery2" :`DrawDebugType` "ForDuration"))
  (cast `GeometryCollectionComponent` (`.HitComponent` (`GameplayStatics.BreakHitResult` _outhit)))
  (bind _returnvalue_2 (`|SpawnActorFromClass` (`self.ForceFieldType`) (`KismetMathLibrary.MakeTransform` (`.ImpactPoint` (`GameplayStatics.BreakHitResult` _outhit)) (`KismetMathLibrary.MakeRotFromZ` (* (`.ImpactNormal` (`GameplayStatics.BreakHitResult` _outhit)) -1.0))) "Undefined" "MultiplyWithRoot" null null))
  (set `/Engine/EditorResources/FieldNodes/FS_MasterField.DirectionalMagnitude` (`self.ForceMagnitude`) _returnvalue_2)
  (`/Engine/EditorResources/FieldNodes/FS_MasterField.CE_Trigger` _returnvalue_2))

(fn `UserConstructionScript`
  (`parent.UserConstructionScript`))