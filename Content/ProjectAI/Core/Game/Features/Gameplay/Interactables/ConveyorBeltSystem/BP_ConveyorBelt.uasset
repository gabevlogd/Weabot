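; Spline-based conveyor belt that pushes overlapping actors along the spline, skipping ignored classes.
; The construction script lays visual spline meshes and raised collider copies, either stretched between spline points or tiled by mesh length.
; Tick offsets each actor once along the nearest spline direction, while a material parameter scrolls the surface.
; Belts run constantly or, if triggerable, for a timed duration, with counted Activate/Deactivate calls flipping direction and mirroring elapsed time when reversed mid-run.
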(event `self.ReceiveBeginPlay`
  ;[0 0 0] Unreal Events
  (`self.InitializeBelt`))

(event `self.ReceiveTick`
  (params (DeltaSeconds :type "Float (single-precision)"))
  ;[0 0 0] Unreal Events
  (`self.ActiveMovement`
    (:`true`
      (`self.PerformMovement`))))

(event `/Game/ProjectAI/Core/Game/Features/Gameplay/InteractSystem/Interfaces/BPI_Activable.Activate`
  ;[0 0 0] Belt Trigger
  (`self.IsTriggerable`
    (:`true`
      (bind _triggerbeltmovement (`self.IncrementTriggerCounter` 1 (`self.MaxTriggerCount`)))
      (if _triggerbeltmovement
        (`self.InitializeBeltMovement`)))))

(event `/Game/ProjectAI/Core/Game/Features/Gameplay/InteractSystem/Interfaces/BPI_Activable.Deactivate`
  ;[0 0 0] Belt Trigger
  (`self.IsTriggerable`
    (:`true`
      (bind _triggerbeltmovement (`self.IncrementTriggerCounter` -1 (- (`self.MaxTriggerCount`) 1)))
      (if _triggerbeltmovement
        (`self.InitializeBeltMovement`)))))

(fn `GetLastIndex`
  (returns (ReturnValue :type Integer))
  (bind _returnvalue_x (`KismetMathLibrary.BreakVector` (`self.GetMeshExtent`)))
  (if (`self.StretchMeshLenght`)
    (return (- (`SplineComponent.GetNumberOfSplinePoints` (`self.Spline`)) 2))
    (else
      (return (`KismetMathLibrary.FTrunc` (/ (`SplineComponent.GetSplineLength` (`self.Spline`)) _returnvalue_x))))))

(fn `GetMeshExtent`
  (returns (ReturnValue :type "Vector Structure"))
  (bind (_returnvalue_min _returnvalue_max) (break `Box` (`StaticMesh.GetBoundingBox` (`self.Mesh`))))
  (return (+ (`KismetMathLibrary.Vector_GetAbs` _returnvalue_min) (`KismetMathLibrary.Vector_GetAbs` _returnvalue_max))))

(fn `GetStartAndEnd`
  (params (PointIndex :type Integer))
  (returns (`Start Location` :type "Vector Structure") (`Start Tangent` :type "Vector Structure") (EndLocation :type "Vector Structure") (EndTangent :type "Vector Structure"))
  (bind _returnvalue_x (`KismetMathLibrary.BreakVector` (`self.GetMeshExtent`)))
  (bind _spline (`self.Spline`))
  (bind _spline_2 (`self.Spline`))
  (bind _spline_3 (`self.Spline`))
  (bind (_location _tangent) (`SplineComponent.GetLocationAndTangentAtSplinePoint` _spline_2 (+ PointIndex 1) "Local"))
  (bind (_location_2 _tangent_2) (`SplineComponent.GetLocationAndTangentAtSplinePoint` _spline_2 PointIndex "Local"))
  (bind _returnvalue (* PointIndex _returnvalue_x))
  (bind _returnvalue_2 (+ _returnvalue _returnvalue_x))
  (if (`self.StretchMeshLenght`)
    (return _location_2 _tangent_2 _location _tangent)
    (else
      (return (`SplineComponent.GetLocationAtDistanceAlongSpline` _spline_3 _returnvalue "Local") (`KismetMathLibrary.ClampVectorSize` (`SplineComponent.GetTangentAtDistanceAlongSpline` _spline_3 _returnvalue "Local") 0.0 _returnvalue_x) (`SplineComponent.GetLocationAtDistanceAlongSpline` _spline _returnvalue_2 "Local") (`KismetMathLibrary.ClampVectorSize` (`SplineComponent.GetTangentAtDistanceAlongSpline` _spline _returnvalue_2 "Local") 0.0 _returnvalue_x)))))

(fn `IncrementTriggerCounter`
  (params (CounterIncrement :type Integer) (TriggerValue :type Integer))
  (returns (TriggerBeltMovement :type Boolean))
  (bind _output_get (set `self.CurrentTriggerCount` (`KismetMathLibrary.Clamp` (+ (`self.CurrentTriggerCount`) CounterIncrement) 0 (`self.MaxTriggerCount`))))
  (return (== _output_get TriggerValue)))

(fn `InitializeBelt`
  (`self.IsTriggerable`
    (:`true`
      (if (`self.bIsActiveOnBegin`)
        (set `self.ElapsedTime` 0.0)
        (set `self.Direction` "NewEnumerator0")
        (`self.SetMaterialSpeed` (`self.PositiveSpeed`))
        (else
          (set `self.ElapsedTime` (`self.Duration`))
          (set `self.Direction` "NewEnumerator1")
          (`self.SetMaterialSpeed` 0.0))))
    (:`false`
      (bind _output_get (set `self.CurrentSpeed` (`self.PositiveSpeed`)))
      (`self.SetMaterialSpeed` _output_get))))

(fn `InitializeBeltMovement`
  (`self.ResetTimer`)
  (if (`|EnumEquality` (`self.Direction`) "NewEnumerator0")
    (set `self.Direction` "NewEnumerator1")
    (`self.SetMaterialSpeed` (`self.NegativeSpeed`))
    (else
      (set `self.Direction` "NewEnumerator0")
      (`self.SetMaterialSpeed` (`self.PositiveSpeed`)))))

(fn `PerformMovement`
  (for _array_element (`self.OverlapComponents`)
    (for _array_element_2 (`PrimitiveComponent.GetOverlappingActors` _array_element null)
      (if (not (`KismetArrayLibrary.Array_Contains` (`self.MovedActor`) _array_element_2))
        (`self.CanBeMoved` _array_element_2
          (:`true`
            (`KismetArrayLibrary.Array_Add` (`self.MovedActor`) _array_element_2)
            (`self.K2_AddActorWorldOffset` _array_element_2 (* (`SplineComponent.FindDirectionClosestToWorldLocation` (`self.Spline`) (`self.K2_GetActorLocation` _array_element_2) "World") (* (`self.CurrentSpeed`) (`GameplayStatics.GetWorldDeltaSeconds`))) (`self.SweepMovement`) false))))))
  (`KismetArrayLibrary.Array_Clear` (`self.MovedActor`)))

(fn `ResetTimer`
  (if (>= (`self.ElapsedTime`) (`self.Duration`))
    (set `self.ElapsedTime` 0.0)
    (else
      (set `self.ElapsedTime` (- (`self.Duration`) (`self.ElapsedTime`))))))

(fn `SetMaterialSpeed`
  (params (Speed :type "Float (double-precision)"))
  (locals (MaterialSpeed :type "Float (double-precision)"))
  (for _array_element (`self.SplineMeshes`)
    (`MeshComponent.SetScalarParameterValueOnMaterials` _array_element "Speed Y" (* Speed 0.01))))

(fn `UpdateDirection`
  (if (`|EnumEquality` (`self.Direction`) "NewEnumerator0")
    (set `self.CurrentSpeed` (`self.PositiveSpeed`))
    (else
      (set `self.CurrentSpeed` (`self.NegativeSpeed`)))))

(fn `UpdateTimer`
  (set `self.ElapsedTime` (+ (`self.ElapsedTime`) (`GameplayStatics.GetWorldDeltaSeconds`))))

(fn `UserConstructionScript`
  (bind (_returnvalue_x _returnvalue_y _returnvalue_z) (`KismetMathLibrary.BreakVector` (`self.GetMeshExtent`)))
  (bind _spline (`self.Spline`))
  (`parent.UserConstructionScript`)
  ;[0 0 0] Set up spline
  (for _index (range (+ (`self.GetLastIndex`) 1))
    ;;[0.1804 0.1804 0.1804] Spline Mesh
    (bind _returnvalue (`AddComponent|NODE_AddSplineMeshComponent-3`))
    (`SceneComponent.SetVisibility` _returnvalue (`self.MeshVisibility`) false)
    (`KismetArrayLibrary.Array_Add` (`self.SplineMeshes`) _returnvalue)
    (`StaticMeshComponent.SetStaticMesh` _returnvalue (`self.Mesh`))
    (bind (_start_location _start_tangent _endlocation _endtangent) (`self.GetStartAndEnd` _index))
    (`SplineMeshComponent.SetStartAndEnd` _returnvalue _start_location _start_tangent _endlocation _endtangent true)
    (if (`self.StretchMeshLenght`)
      (`MeshComponent.SetScalarParameterValueOnMaterials` _returnvalue "Texture Size Y" (/ (- (`SplineComponent.GetDistanceAlongSplineAtSplinePoint` _spline _index) (`SplineComponent.GetDistanceAlongSplineAtSplinePoint` _spline (+ _index 1))) 100.0)))
    ;;[0.1804 0.1804 0.1804] Collider
    (bind _returnvalue_2 (`AddComponent|NODE_AddSplineMeshComponent-4`))
    (`SceneComponent.K2_AddRelativeLocation` _returnvalue_2 (`KismetMathLibrary.MakeVector` 0.0 0.0 _returnvalue_z) false false)
    (`StaticMeshComponent.SetStaticMesh` _returnvalue_2 (`self.Mesh`))
    (`SplineMeshComponent.SetStartAndEnd` _returnvalue_2 _start_location _start_tangent _endlocation _endtangent true)
    (`KismetArrayLibrary.Array_Add` (`self.OverlapComponents`) _returnvalue_2)))