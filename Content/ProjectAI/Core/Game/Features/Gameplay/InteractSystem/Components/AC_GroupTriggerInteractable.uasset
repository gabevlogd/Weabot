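; AC_GroupTriggerInteractable is a component in the interact system that triggers a group of interactables at once.
; It exposes four events for primary interact, secondary interact, enable interact and disable interact.
; Each event loops over the Interactables array and forwards the matching call to every element, with no filtering or state of its own.
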(event `PrimaryInteractAll`
  (for _array_element (`self.Interactables`)
    (`/Game/ProjectAI/Core/Game/Features/Gameplay/InteractSystem/Interfaces/BPI_Interactable.PrimaryInteract` _array_element)))

(event `SecondaryInteractAll`
  (for _array_element (`self.Interactables`)
    (`/Game/ProjectAI/Core/Game/Features/Gameplay/InteractSystem/Interfaces/BPI_Interactable.SecondaryInteract` _array_element)))

(event `EnableInteractAll`
  (for _array_element (`self.Interactables`)
    (`/Game/ProjectAI/Core/Game/Features/Gameplay/InteractSystem/Interfaces/BPI_Interactable.EnableInteract` _array_element)))

(event `DisableInteractAll`
  (for _array_element (`self.Interactables`)
    (`/Game/ProjectAI/Core/Game/Features/Gameplay/InteractSystem/Interfaces/BPI_Interactable.DisableInteract` _array_element)))