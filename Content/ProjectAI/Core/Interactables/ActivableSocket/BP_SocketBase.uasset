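; BP_SocketBase is a base Blueprint for a grabbable physics object that can be placed in and removed from a socket.
; Grab and Ungrab events toggle a flag, exposed through CanBePlaced, so the object is placeable only while not held.
; PlaceSocket turns off physics simulation on the mesh and RemoveSocket turns it back on, with attachment and positioning left outside these graphs.
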(event `/Game/ProjectAI/Core/Interactables/GrabSystem/Interfaces/BPI_Grabbable.Grab`
  (set `self.bCanBePlaced` false))

(event `/Game/ProjectAI/Core/Interactables/GrabSystem/Interfaces/BPI_Grabbable.Ungrab`
  (set `self.bCanBePlaced` true))

(event `/Game/ProjectAI/Core/Interactables/ActivableSocket/Interfaces/BPI_Socket.PlaceSocket`
  (`PrimitiveComponent.SetSimulatePhysics` (`self.Mesh`) false))

(event `/Game/ProjectAI/Core/Interactables/ActivableSocket/Interfaces/BPI_Socket.RemoveSocket`
  (`PrimitiveComponent.SetSimulatePhysics` (`self.Mesh`) true))

(fn `CanBePlaced`
  (returns (bCanBePlaced :type Boolean))
  (return (`self.bCanBePlaced`)))

(fn `UserConstructionScript`)