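; BP_PhysicalShock is a physical inventory item that releases an area electric shock to stun AI when it hits an actor.
; On the hit event it runs the parent logic, then spawns a Niagara electricity effect scaled to the shock radius and a positional sound.
; A multi-sphere trace at the impact point stuns AI entities for the shock duration, then the item destroys itself.
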(event `self.HitActorEvent`
  (params (OtherActor :type "Actor Object Reference") (Hit :type "HitResult Structure"))
  (bind (_bblockinghit _binitialoverlap _time _distance _location) (`GameplayStatics.BreakHitResult` Hit))
  (`parent.HitActorEvent` OtherActor Hit)
  (bind _returnvalue (`NiagaraFunctionLibrary.SpawnSystemAtLocation` "/Game/ProjectAI/MaterialLibrary/Elettricity/NS_Elettricity.NS_Elettricity" (`.Location` (`GameplayStatics.BreakHitResult` Hit)) (struct) (1.0 1.0 1.0) true true "AutoRelease"))
  (`NiagaraComponent.SetVariableFloat` _returnvalue "User.Size" (* (`self.ShokRadiusSize`) 2.0))
  (`GameplayStatics.SpawnSoundAtLocation` "/Game/ProjectAI/Audio/Sounds/Effects/SW_Shock.SW_Shock" (`.Location` (`GameplayStatics.BreakHitResult` Hit)) (struct) 1.0 1.0 0.2 "/Game/ProjectAI/Audio/Attenuations/SA_Elettricity.SA_Elettricity" null)
  (bind _outhits (`KismetSystemLibrary.SphereTraceMulti` _location _location (`self.ShokRadiusSize`) "TraceTypeQuery3"))
  (for _array_element _outhits
    (bind _asbp_aientity_base (cast `/Game/ProjectAI/Core/Game/Features/AI/Behaviours/Base/BP_AIEntity_Base` (`.HitActor` (`GameplayStatics.BreakHitResult` _array_element))))
    (`/Game/ProjectAI/Core/Game/Features/AI/Behaviours/Base/BP_AIEntity_Base.Stun` _asbp_aientity_base (`self.ShockDuration`)))
  (`self.K2_DestroyActor`))

(fn `UserConstructionScript`
  (`parent.UserConstructionScript`))