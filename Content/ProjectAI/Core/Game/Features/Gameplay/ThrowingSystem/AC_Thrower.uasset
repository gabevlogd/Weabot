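; Actor component that lets its owner aim and throw a configurable actor class, with a trajectory preview and cooldown.
; While aiming, a next-tick loop predicts the projectile path and draws it through a spawned BP_AimPreviewSpline.
; Launch velocity follows control rotation plus pitch offset, gaining capped speed when looking up and optionally inheriting owner velocity.
; Throwing spawns the item at the predicted start and applies that velocity to its physics mesh.
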(event `self.ReceiveBeginPlay`
  (`self.Initialize`))

(event `OnThrow`
  (`/Engine/EditorBlueprintResources/StandardMacros.DoOnce` false :!label _label
    (:`Completed`
      (if (`self.bIsAiming`)
        (`self.StopAiming`)
        (`self.Throw`)
        (`GameplayStatics.PlaySound2D` "/Game/ProjectAI/Audio/Sounds/Effects/SW_Throwing.SW_Throwing" 1.0 1.0 0.0 null null)
        (`KismetSystemLibrary.Delay` (`self.ThrowAbilityCooldown`))
        (goto _label :!via `Reset`)
        (else
          (goto _label :!via `Reset`))))))

(event `OnAim`
  (params (IsAiming :type Boolean))
  (if (and IsAiming (`KismetSystemLibrary.IsValidClass` (`self.ItemToThrow`)))
    (`self.StartAiming`)
    (else
      (`self.StopAiming`))))

(event `AimingEvent`
  (if (`self.bIsAiming`)
    (`/Game/ProjectAI/Core/Game/Features/Gameplay/ThrowingSystem/BP_AimPreviewSpline.ClearSpline` (`self.AimPreviewSpline`))
    (bind _output_get (set `self.ThrowVelocity` (`self.GetThorwVelocity`)))
    (bind _output_get_2 (set `self.StartLocation` (`self.GetStartLocation`)))
    (bind _predictresult (`GameplayStatics.Blueprint_PredictProjectilePath_Advanced` (make `PredictProjectilePathParams` _output_get_2 _output_get true (`self.ProjectileRadius`) (`self.PredictTrajectoryTime`) true "ECC_WorldStatic" _ _ 12.0)))
    (`self.ShowAimPreview` _predictresult)
    (`KismetSystemLibrary.DelayUntilNextTick`)
    (`self.AimingEvent`)))

(fn `GetStartLocation`
  (returns (ReturnValue :type "Vector Structure"))
  (return (+ (`Actor.K2_GetActorLocation` (`self.GetOwner`)) (* (`KismetMathLibrary.GetForwardVector` (`Controller.GetControlRotation` (`GameplayStatics.GetPlayerController` 0))) (`self.SpawnPointOffset`)))))

(fn `GetThorwVelocity`
  (returns (ReturnValue :type "Vector Structure"))
  (bind _returnvalue (* (`KismetMathLibrary.GetForwardVector` (`KismetMathLibrary.MakeRotator` (.roll (`Controller.GetControlRotation` (`GameplayStatics.GetPlayerController` 0))) (+ (.pitch (`Controller.GetControlRotation` (`GameplayStatics.GetPlayerController` 0))) (`self.AimPitchOffset`)) (.yaw (`Controller.GetControlRotation` (`GameplayStatics.GetPlayerController` 0))))) (`self.GetThrowingSpeed`)))
  (if (`self.bManteinOwnerInertia`)
    (return (+ _returnvalue (`Actor.GetVelocity` (`self.GetOwner`))))
    (else
      (return _returnvalue))))

(fn `GetThrowingSpeed`
  (returns (ThrowingSpeed :type "Float (double-precision)"))
  (bind (_returnvalue_roll _returnvalue_pitch) (`KismetMathLibrary.BreakRotator` (`Controller.GetControlRotation` (`GameplayStatics.GetPlayerController` 0))))
  (if (and (>= _returnvalue_pitch 0.0) (<= _returnvalue_pitch 90.0))
    (if (<= _returnvalue_pitch (`self.MaxSpeedIncrementerPitchAngle`))
      (return (+ (`self.ThrowingSpeed`) (* _returnvalue_pitch (`self.SpeedIncrementMultiplier`))))
      (else
        (return (+ (`self.ThrowingSpeed`) (* (`self.MaxSpeedIncrementerPitchAngle`) (`self.SpeedIncrementMultiplier`))))))
    (else
      (return (`self.ThrowingSpeed`)))))

(fn `Initialize`
  (bind _returnvalue (`|SpawnActorFromClass` "/Game/ProjectAI/Core/Game/Features/Gameplay/ThrowingSystem/BP_AimPreviewSpline.BP_AimPreviewSpline_C" (`KismetMathLibrary.MakeTransform` (`self.GetStartLocation`)) "Undefined" "MultiplyWithRoot" null null))
  (bind _output_get (set `self.AimPreviewSpline` _returnvalue))
  (`/Game/ProjectAI/Core/Game/Features/Gameplay/ThrowingSystem/BP_AimPreviewSpline.ClearSpline` _output_get))

(fn `SetActorToThrow`
  (params (ActorToThrow :type "/Game/ProjectAI/Core/Game/Features/Gameplay/InventorySystem/InventoryItems/PhysicalItems/Base/BP_PhysicalItemBase Class Reference"))
  (set `self.ItemToThrow` ActorToThrow))

(fn `ShowAimPreview`
  (params (PredictProjectilePathResult :type "PredictProjectilePathResult Structure (by ref)"))
  (for _array_element (`.PathData` (break `PredictProjectilePathResult` PredictProjectilePathResult))
    (`/Game/ProjectAI/Core/Game/Features/Gameplay/ThrowingSystem/BP_AimPreviewSpline.AddPoint` (`self.AimPreviewSpline`) (break `PredictProjectilePathPointData` _array_element) (`.Velocity` (break `PredictProjectilePathPointData` _array_element))))
  (`/Game/ProjectAI/Core/Game/Features/Gameplay/ThrowingSystem/BP_AimPreviewSpline.ShowSpline` (`self.AimPreviewSpline`)))

(fn `StartAiming`
  (set `self.bIsAiming` true)
  (`self.AimingEvent`))

(fn `StopAiming`
  (set `self.bIsAiming` false)
  (`/Game/ProjectAI/Core/Game/Features/Gameplay/ThrowingSystem/BP_AimPreviewSpline.ClearSpline` (`self.AimPreviewSpline`)))

(fn `Throw`
  (if (`KismetSystemLibrary.IsValidClass` (`self.ItemToThrow`))
    (bind _returnvalue (`|SpawnActorFromClass` (`self.ItemToThrow`) (`KismetMathLibrary.MakeTransform` (`self.StartLocation`)) "AdjustIfPossibleButAlwaysSpawn" "MultiplyWithRoot" null null))
    (`PrimitiveComponent.SetPhysicsLinearVelocity` (`/Game/ProjectAI/Core/Game/Features/Gameplay/InventorySystem/InventoryItems/PhysicalItems/Base/BP_PhysicalItemBase.StaticMesh` _returnvalue) (`self.ThrowVelocity`) false "None")
    (`self.OnItemThrowed`)
    (else
      (return))))