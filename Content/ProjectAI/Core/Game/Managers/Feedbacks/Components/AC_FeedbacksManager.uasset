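; AC_FeedbacksManager is an actor component that plays controller vibration for player combat events.
; On BeginPlay it casts the game mode to GM_PAIGameplay and binds to its ACGameEvents damage and shoot dispatchers.
; Each handler plays a dedicated force feedback effect on player controller 0, ignoring the damage amount.
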(event `self.ReceiveBeginPlay`
  (bind _asgm_paigameplay (cast `/Game/ProjectAI/Core/Game/UGameFramework/GameModes/GM_PAIGameplay` (`GameplayStatics.GetGameMode`)))
  (bind _ac_gameevents (`/Game/ProjectAI/Core/Game/UGameFramework/GameModes/GM_PAIGameplay.AC_GameEvents` _asgm_paigameplay))
  (add `/Game/ProjectAI/Core/Game/Managers/Events/Components/AC_GameEvents.OnPlayerTakeDamage` _ac_gameevents (`|CreateDelegate` :!event `OnPlayerTakeDamage_Event`))
  (add `/Game/ProjectAI/Core/Game/Managers/Events/Components/AC_GameEvents.OnPlayerShoot` _ac_gameevents (`|CreateDelegate` :!event `OnPlayerShoot_Event`)))

(event `OnPlayerTakeDamage_Event`
  (params (DamageTaken :type "Float (double-precision)"))
  (`PlayerController.K2_ClientPlayForceFeedback` (`GameplayStatics.GetPlayerController` 0) "/Game/ProjectAI/Core/Game/Data/ForceFeedbackEffects/FFE_PlayerDamageVibration.FFE_PlayerDamageVibration" "None" false false false))

(event `OnPlayerShoot_Event`
  (`PlayerController.K2_ClientPlayForceFeedback` (`GameplayStatics.GetPlayerController` 0) "/Game/ProjectAI/Core/Game/Data/ForceFeedbackEffects/FFE_PlayerShootVibration.FFE_PlayerShootVibration" "None" false false false))